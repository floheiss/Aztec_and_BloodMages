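; BP_DistressManger tracks a combat unit's distress (DisgustData) and handles disfigurement of that unit, its Holder.
; ManagDisfigure reports the Holder's disfigurement to its CombatManager; the debuff function it calls is an empty stub.
; ManageDisfigureDistress picks distress by victim (self, ally or enemy) and body part, scaled through a multiplier map in GainDistress.
; Reaching the maximum calls AddNegativeModifier, which currently only subtracts that maximum.
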(fn `AddNegativeModifier`
  (bind (_currentdis _maxdis) (break `/Game/Chars/Distressmanager/UnitDisgustData` (`self.DisgustData`)))
  (setmembers `/Game/Chars/Distressmanager/UnitDisgustData` :`StructRef` (`self.DisgustData`) :`CurrentDis` (- _currentdis _maxdis)))

(fn `ApplyDisfigureDebuff`
  (params (Disfigure :type "/Game/Chars/Attacks/Enums/DisfigureOptions Enum" :default "NewEnumerator0")))

(fn `GainDistress`
  (params (Amount :type Integer) (MultiplayerToUse :type "/Game/Chars/Distressmanager/DisgustModifayerList Enum" :default "NewEnumerator0"))
  (locals (LocModi :type "Float (double-precision)"))
  (bind (_currentdis _maxdis) (break `/Game/Chars/Distressmanager/UnitDisgustData` (`self.DisgustData`)))
  (bind (_value _returnvalue) (`BlueprintMapLibrary.Map_Find` (`.Multiplayer_19_0B7DA30B4D058A579E924D97B2CFF891` (break `/Game/Chars/Distressmanager/UnitDisgustData` (`self.DisgustData`))) (`local.MultiplayerToUse`)))
  (if _returnvalue
    (set `local.LocModi` _value)
    (else
      (set `local.LocModi` 1.0)))
  (setmembers `/Game/Chars/Distressmanager/UnitDisgustData` :`StructRef` (`self.DisgustData`) :`CurrentDis` (+ (`.CurrentDis_4_41A9B4434BF10558B23762968DEFE87B` (break `/Game/Chars/Distressmanager/UnitDisgustData` (`self.DisgustData`))) (* (`local.Amount`) (`local.LocModi`))))
  (if (>= _currentdis _maxdis)
    (`self.AddNegativeModifier`)))

(fn `GetInfoForTransfer`
  (returns (DisgustData :type "/Game/Chars/Distressmanager/UnitDisgustData Structure"))
  (return (`self.DisgustData`)))

(fn `ManagDisfigure`
  (params (Disfigure :type "/Game/Chars/Attacks/Enums/DisfigureOptions Enum" :default "NewEnumerator0"))
  (`self.ApplyDisfigureDebuff` Disfigure)
  (`/Game/Combat/CombatManager.UnitDisfigured` (`/Game/Chars/PZD_Unit.Combat Manager` (`self.Holder`)) (`local.Disfigure`) (`self.Holder`)))

(fn `ManageDisfigureDistress`
  (params (Disfigure :type "/Game/Chars/Attacks/Enums/DisfigureOptions Enum" :default "NewEnumerator0") (UnitEffekted :type "/Game/Chars/PZD_Unit Object Reference"))
  (locals (LocMultiToUse :type "/Game/Chars/Distressmanager/DisgustModifayerList Enum" :default "NewEnumerator0") (LocAmountGained :type Integer :default 0))
  (set `local.LocMultiToUse` (select `/Game/Chars/Attacks/Enums/DisfigureOptions` (`local.Disfigure`) :`NewEnumerator0` "NewEnumerator2" :`NewEnumerator1` "NewEnumerator3" :`NewEnumerator2` "NewEnumerator4" :!type "/Game/Chars/Distressmanager/DisgustModifayerList Enum"))
  (`|ExecutionSequence`
    (:`then_0`
      (if (!= (`self.Holder`) (`local.UnitEffekted`))
        (set `local.LocAmountGained` (`KismetMathLibrary.SelectInt` 10 40 (!= (`/Game/Chars/PZD_Unit.Team` (`local.UnitEffekted`)) (`/Game/Chars/PZD_Unit.Team` (`self.Holder`)))))
        (else
          (set `local.LocAmountGained` 20))))
    (:`then_1`
      (`self.GainDistress` (`local.LocAmountGained`) (`local.LocMultiToUse`)))))

(fn `ReInit`
  (params (DisgustData :type "/Game/Chars/Distressmanager/UnitDisgustData Structure") (Holder :type "/Game/Chars/PZD_Unit Object Reference"))
  (set `self.DisgustData` DisgustData)
  (set `self.Holder` Holder))