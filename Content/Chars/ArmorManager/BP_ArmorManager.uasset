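; Manages a unit's equipped armor and its durability, removing the armor when durability runs out.
; Equipping looks up item data, refuses heavy armor for units that cannot use it, and applies the armor's stat bonuses to the Holder.
; Related perks are applied or removed through briefly spawned perk actors, destroyed immediately after messaging.
; Dispatchers report armor changes, and state can be exported and re-initialized for transfer.
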(fn `EquipArmor`
  (params (Armor :type "/Game/InventorySystem/Utilities/ItemList Enum" :default "NewEnumerator0") (Durability :type Integer))
  (if (`|EnumInequality` (`local.Armor`) "NewEnumerator0")
    (`self.RemoveArmor`))
  (bind _itemdata (`/Game/Core/BFL_General.GetDataFormItem` (`local.Armor`)))
  (set `self.ItemData` _itemdata)
  (if (or (`.canUseHeavyArmor_75_81FAFD02413EA947714790872C8D4678` (break `/Game/Chars/Utilities/UnitStructs/Unit_Data` (`/Game/Chars/PZD_Unit.UnitData` (`self.Holder`)))) (not (`.isHeavy_5_05B6FE60443AB36A828A1A8AC240955D` (break `/Game/InventorySystem/Utilities/ArmorData` (`.armorStats_29_1AC204174A45D71322A59BB17D5B35DD` (break `/Game/InventorySystem/Utilities/ItemData` (`self.ItemData`)))))))
    (set `self.CurrentArmor` (`local.Armor`))
    (set `self.RemainingDurability` (`local.Durability`))
    (`self.NewArmorEquiped` (`self.CurrentArmor`) (`self.RemainingDurability`))
    (bind _perkdata (`/Game/Core/BFL_General.GetDataFormPerk` (`.RelatedPerk_28_CBC4626046DE1333F688AAAF029A0DC6` (break `/Game/InventorySystem/Utilities/ArmorData` (`.armorStats_29_1AC204174A45D71322A59BB17D5B35DD` (break `/Game/InventorySystem/Utilities/ItemData` (`self.ItemData`)))))))
    (bind _returnvalue (`|SpawnActorFromClass` (`.PerkClass_24_8A42A5014A4964BB2B23CF95EA7C84BA` (break `/Game/Chars/PerkSystem/PerkData` _perkdata)) (`KismetMathLibrary.MakeTransform` (-999.0 -999.0 -999.0)) "AlwaysSpawn" "MultiplyWithRoot" null null))
    (message `/Game/Chars/PerkSystem/PerkClasses/IN_Perk.ApplyPerk` _returnvalue (`self.Holder`))
    (`Actor.K2_DestroyActor` _returnvalue)
    (`/Game/Chars/PZD_Unit.SetMoreUnitStat` (`self.Holder`) false (`.ArmorStats_25_67386E5D4D745B5894636AB4A633F15D` (break `/Game/InventorySystem/Utilities/ArmorData` (`.armorStats_29_1AC204174A45D71322A59BB17D5B35DD` (break `/Game/InventorySystem/Utilities/ItemData` (`self.ItemData`))))))
    (else
      (`KismetSystemLibrary.PrintText` "ERROR cant use this armor (is heavy and you cant :( )" true true (struct :`R` 1.0 :`B` 0.059451 :`A` 1.0) 10.0))))

(fn `GainDurability`
  (params (GainDurability :type Integer))
  (bind ((`MaxAmoutMaxDurability_46_550060C34F79CCA0A5A31B9B726D0F9E` _maxamoutmaxdurability)) (break `/Game/InventorySystem/Utilities/ItemData` (`self.ItemData`)))
  (bind _output_get (set `self.RemainingDurability` (+ (`self.RemainingDurability`) (`local.GainDurability`))))
  (if (> _maxamoutmaxdurability _output_get)
    (set `self.RemainingDurability` _maxamoutmaxdurability)))

(fn `GetArmor`
  (returns (CurrentArmor :type "/Game/InventorySystem/Utilities/ItemList Enum") (RemainingDurability :type Integer))
  (return (`self.CurrentArmor`) (`self.RemainingDurability`)))

(fn `GetInfoForTransfer`
  (returns (CurrentArmor :type "/Game/InventorySystem/Utilities/ItemList Enum") (RemainingDurability :type Integer))
  (return (`self.CurrentArmor`) (`self.RemainingDurability`)))

(fn `ReduceDurability`
  (params (LostDurability :type Integer))
  (bind _output_get (set `self.RemainingDurability` (- (`self.RemainingDurability`) (`local.LostDurability`))))
  (if (<= _output_get 0)
    (`self.RemoveArmor`)
    (`self.ArmorTriggered` (`self.CurrentArmor`) (`self.RemainingDurability`))))

(fn `ReInit`
  (params (CurrentArmor :type "/Game/InventorySystem/Utilities/ItemList Enum" :default "NewEnumerator0") (RemainingDurability :type Integer) (Holder :type "/Game/Chars/PZD_Unit Object Reference"))
  (set `self.CurrentArmor` CurrentArmor)
  (set `self.RemainingDurability` RemainingDurability)
  (set `self.Holder` Holder)
  (bind _itemdata (`/Game/Core/BFL_General.GetDataFormItem` (`local.CurrentArmor`)))
  (set `self.ItemData` _itemdata))

(fn `RemoveArmor`
  (set `self.CurrentArmor` "NewEnumerator0")
  (set `self.RemainingDurability` 0)
  (bind _perkdata (`/Game/Core/BFL_General.GetDataFormPerk` (`.RelatedPerk_28_CBC4626046DE1333F688AAAF029A0DC6` (break `/Game/InventorySystem/Utilities/ArmorData` (`.armorStats_29_1AC204174A45D71322A59BB17D5B35DD` (break `/Game/InventorySystem/Utilities/ItemData` (`self.ItemData`)))))))
  (bind _returnvalue (`|SpawnActorFromClass` (`.PerkClass_24_8A42A5014A4964BB2B23CF95EA7C84BA` (break `/Game/Chars/PerkSystem/PerkData` _perkdata)) (`KismetMathLibrary.MakeTransform` (-999.0 -999.0 -999.0)) "AdjustIfPossibleButAlwaysSpawn" "MultiplyWithRoot" null null))
  (message `/Game/Chars/PerkSystem/PerkClasses/IN_Perk.RemovePerk` _returnvalue (`self.Holder`) 1)
  (`Actor.K2_DestroyActor` _returnvalue)
  (`/Game/Chars/PZD_Unit.SetMoreUnitStat` (`self.Holder`) true (`.ArmorStats_25_67386E5D4D745B5894636AB4A633F15D` (break `/Game/InventorySystem/Utilities/ArmorData` (`.armorStats_29_1AC204174A45D71322A59BB17D5B35DD` (break `/Game/InventorySystem/Utilities/ItemData` (`self.ItemData`))))))
  (`self.ArmorDestroyed`))