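; Per-unit distress manager that tracks a combat unit's distress meter and reacts to disfigurements.
; Gains and losses apply crit and keyed multipliers; gains wrap at the maximum into an overflow count, then notify the bar and Holder.
; Disfigurements broadcast through the CombatManager, and the distress response scales by body part and whether the victim is self, same team or opposing.
; Cap-trigger effects and disfigure debuffs are unfinished stubs.
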(fn GetInfoforTransfer
  (return (Variables|Default|GetDisstressData)))

(fn ReInit
  (params (DisgustData :type Unit%20Disgust%20Data%20Structure) (Holder :type PZD%20Unit%20Object%20Reference))
  (Variables|Default|SetDisstressData DisgustData)
  (Variables|Default|SetHolder Holder))

(fn GainDistress
  (params (Amount :type Integer) (MultiplayerToUse :type DisgustModifayerList%20Enum :default "NewEnumerator0") (IsCrit :type Boolean))
  (bind _disstressdata (Variables|Default|GetDisstressData))
  (bind _multiplayer (Utilities|Struct|BreakUnitDisgustData _disstressdata))
  (bind (_value _returnvalue) (Utilities|Map|Find _multiplayer MultiplayerToUse))
  (LocalVariables|SetLocModi (Math|Float|SelectFloat _value 1.0 _returnvalue))
  (LocalVariables|SetLocOld (Utilities|Struct|BreakUnitDisgustData (Variables|Default|GetDisstressData)))
  (LocalVariables|SetLocMax (Utilities|Struct|BreakUnitDisgustData (Variables|Default|GetDisstressData)))
  (LocalVariables|SetLocNew (Math|Float|Round (* (CallFunction|CalulateAmount Amount IsCrit false) (LocalVariables|GetLocModi))))
  (LocalVariables|SetLocOverflow (|(floor((({449C5CFF-4D76-4909-3D93-6393B375E278}+{6C9F3261-49DC-08F8-68DD-73A039F6C241})/{8083C52D-48FA-5E71-4A36-A8B4F19257AC})))))
  (Utilities|Struct|SetmembersinUnitDisgustData (Variables|Default|GetDisstressData) (|(({449C5CFF-4D76-4909-3D93-6393B375E278}+{6C9F3261-49DC-08F8-68DD-73A039F6C241})%{8083C52D-48FA-5E71-4A36-A8B4F19257AC})))
  (CallFunction|ManageDistressBar (LocalVariables|GetLocOverflow))
  (CallFunction|ManagDistressCap (LocalVariables|GetLocOverflow)))

(fn RemoveDistress
  (params (Amount :type Integer) (MultiplayerToUse :type DisgustModifayerList%20Enum :default "NewEnumerator0") (IsCirt :type Boolean))
  (bind _disstressdata (Variables|Default|GetDisstressData))
  (bind _multiplayer (Utilities|Struct|BreakUnitDisgustData _disstressdata))
  (bind (_value _returnvalue) (Utilities|Map|Find _multiplayer MultiplayerToUse))
  (LocalVariables|SetLocAmount (CallFunction|CalulateAmount Amount IsCirt true))
  (LocalVariables|SetLocModi (Math|Float|SelectFloat _value 1.0 _returnvalue))
  (Utilities|Struct|SetmembersinUnitDisgustData (Variables|Default|GetDisstressData) (Math|Integer|Clamp(Integer) (- (Utilities|Struct|BreakUnitDisgustData (Variables|Default|GetDisstressData)) (* Amount (LocalVariables|GetLocModi))) 0 (- (Utilities|Struct|BreakUnitDisgustData (Variables|Default|GetDisstressData)) (* Amount (LocalVariables|GetLocModi)))))
  (CallFunction|ManageDistressBar)
  ;[1 1 1] debug code
  (Development|PrintText (Utilities|Text|FormatText "i {c} have lost distress. I now have {d}" (Utilities|String|EnumtoString (Variables|/Game/Chars/PZD_Unit.PZD_Unit_C|GetClass (Variables|Default|GetHolder))) (Utilities|Struct|BreakUnitDisgustData (Variables|Default|GetDisstressData))) true true "(R=0.195535,G=1.000000,B=0.000000,A=1.000000)" 2e+01))

(fn ManagDistressCap
  (params (OverFlow :type Integer))
  (bind _disstressdata (Variables|Default|GetDisstressData))
  (bind (_timestriggered _maxtimestriggered) (Utilities|Struct|BreakUnitDisgustData _disstressdata))
  (for _index (range 0 (- OverFlow 1))
    (if (>= _timestriggered _maxtimestriggered)
      _)))

(fn ManagDisfigure
  (params (Disfigure :type DisfigureOptions%20Enum :default "NewEnumerator0"))
  (Disfigure|ApplyDisfigureDebuff Disfigure)
  (Default|CallUnitDisfigured (Variables|/Game/Chars/PZD_Unit.PZD_Unit_C|GetCombat%20Manager (Variables|Default|GetHolder)) Disfigure (Variables|Default|GetHolder)))

(fn ManageDisfigureDistress
  (params (Disfigure :type DisfigureOptions%20Enum :default "NewEnumerator0") (UnitEffekted :type PZD%20Unit%20Object%20Reference))
  (LocalVariables|SetLocMultiToUse (Utilities|Select :Index Disfigure :NewEnumerator0 "NewEnumerator2" :NewEnumerator1 "NewEnumerator3" :NewEnumerator2 "NewEnumerator4"))
  (Utilities|FlowControl|Sequence
    (:then_0
      (if (!= (Variables|Default|GetHolder) UnitEffekted)
        (LocalVariables|SetLocAmountGained (Math|Integer|SelectInt 10 40 (!= (Variables|/Game/Chars/PZD_Unit.PZD_Unit_C|GetTeam UnitEffekted) (Variables|/Game/Chars/PZD_Unit.PZD_Unit_C|GetTeam (Variables|Default|GetHolder)))))
        (else
          (LocalVariables|SetLocAmountGained 20))))
    (:then_1
      (CallFunction|GainDistress (LocalVariables|GetLocAmountGained) (LocalVariables|GetLocMultiToUse) false))))

(fn ApplyDisfigureDebuff
  (params (Disfigure :type DisfigureOptions%20Enum :default "NewEnumerator0")))

(fn CalulateAmount
  (params (Amount :type Integer) (IsCirt :type Boolean) (IsDistressLoss :type Boolean))
  (bind _disstressdata (Variables|Default|GetDisstressData))
  (bind (_critmultigain _critmultiloss) (Utilities|Struct|BreakUnitDisgustData _disstressdata))
  (return (Math|Integer|SelectInt (* Amount (Math|Float|SelectFloat _critmultiloss _critmultigain IsDistressLoss)) Amount IsCirt)))

(fn ManageDistressBar
  (params (Overflow :type Integer))
  (bind _disstressdata (Variables|Default|GetDisstressData))
  (bind (_currentdis _maxdis) (Utilities|Struct|BreakUnitDisgustData _disstressdata))
  (Default|CallDistressUpdate Overflow _currentdis _maxdis)
  (Default|CallUnitStatWasChanged (Variables|Default|GetHolder) "NewEnumerator22" _currentdis))