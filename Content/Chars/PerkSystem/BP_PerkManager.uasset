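; Perk manager that tracks a character's leveled perks and timed buffs/debuffs, and can be re-initialized with transferred state.
; Perk enums resolve to DT_PerkList rows, whose classes are spawned as throwaway actors to run apply, remove or damage-trigger logic.
; Buffs grant their related perk, refreshing duration on repeats; temporary ones expire by tick or at combat end, multi-combat ones count down per combat.
; Take-damage triggers chain each matching perk's modified damage values into the next.
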(fn `AddBuffDeBuff`
  (params (BuffToApply :type "/Game/Chars/PerkSystem/BuffDeBuffStruct Structure"))
  (locals (LocIndex :type Integer :default -1))
  (bind ((`isThisADeBuff_11_40C1736845F08045FE7818A663D6491F` _isthisadebuff) (`icMultiCombat_25_2CA5FEBB4362D2A084B67B8CA3269E41` _icmulticombat) (`RelatedPerk_29_EB2A1D12466FE881AC54E0B511937B78` _relatedperk)) (break `/Game/Chars/PerkSystem/BuffDeBuffStruct` (`local.BuffToApply`)))
  (`KismetSystemLibrary.PrintText` "Tryint to apply buff")
  (for (_array_element _array_index) (`self.ActiveBuffs`)
    (bind ((`isThisADeBuff_11_40C1736845F08045FE7818A663D6491F` _isthisadebuff_2) (`icMultiCombat_25_2CA5FEBB4362D2A084B67B8CA3269E41` _icmulticombat_2) (`RelatedPerk_29_EB2A1D12466FE881AC54E0B511937B78` _relatedperk_2)) (break `/Game/Chars/PerkSystem/BuffDeBuffStruct` _array_element))
    (if (and (== _isthisadebuff_2 _isthisadebuff) (== _icmulticombat_2 _icmulticombat) (`|EnumEquality` (`.PerkType_6_43273B054447BC528895A4AF321DFF41` (break `/Game/Chars/PerkSystem/PerkData` _relatedperk_2)) (`.PerkType_6_43273B054447BC528895A4AF321DFF41` (break `/Game/Chars/PerkSystem/PerkData` _relatedperk))))
      (set `local.LocIndex` _array_index)
      (`KismetSystemLibrary.PrintText` "Found existing buff ")
      (break)))
  (if (!= (`local.LocIndex`) -1)
    (setmembers `/Game/Chars/PerkSystem/BuffDeBuffStruct` :`StructRef` (`|GetArrayItem` (`self.ActiveBuffs`) (`local.LocIndex`)) :`Duration` (`.Duration_17_E34068944B451771C8EBD395BC744633` (break `/Game/Chars/PerkSystem/BuffDeBuffStruct` (`local.BuffToApply`))))
    (`KismetSystemLibrary.PrintText` "add duration to old ")
    (else
      (`KismetArrayLibrary.Array_Add` (`self.ActiveBuffs`) (`local.BuffToApply`))
      (`self.ApplyPerk` (`.PerkType_6_43273B054447BC528895A4AF321DFF41` (break `/Game/Chars/PerkSystem/PerkData` (`.RelatedPerk_29_EB2A1D12466FE881AC54E0B511937B78` (break `/Game/Chars/PerkSystem/BuffDeBuffStruct` (`local.BuffToApply`))))))
      (`KismetSystemLibrary.PrintText` "Applied new"))))

(fn `ApplyPerk`
  (params (NewPerk :type "/Game/Chars/PerkSystem/PerkTypes Enum" :default "NewEnumerator0"))
  (locals (LocPerkToApply :type "/Game/Chars/PerkSystem/PerkData Structure"))
  (bind (_value _returnvalue) (`BlueprintMapLibrary.Map_Find` (`self.PerkList`) (`local.NewPerk`)))
  (bind _perkdtrow (`self.ConvertPerkToDTRow` NewPerk))
  (set `local.LocPerkToApply` _perkdtrow)
  (`|ExecutionSequence`
    (:`then_0`
      (if _returnvalue
        (if (< _value (`.MaxLvL_10_6B8E9E5947F3F2DA4B750BA0A12E9B9D` (break `/Game/Chars/PerkSystem/PerkData` (`local.LocPerkToApply`))))
          (bind _result (`/Engine/EditorBlueprintResources/StandardMacros.IncrementInt` _value)
            (:`  `
              (`BlueprintMapLibrary.Map_Add` (`self.PerkList`) (`local.NewPerk`) (`KismetMathLibrary.Max` 1 _result) :!label _label))))
        (else
          (goto _label))))
    (:`then_1`
      (bind _returnvalue_2 (`|SpawnActorFromClass` (`.PerkClass_24_8A42A5014A4964BB2B23CF95EA7C84BA` (break `/Game/Chars/PerkSystem/PerkData` (`local.LocPerkToApply`))) (`KismetMathLibrary.MakeTransform` (-999.0 -999.0 -999.0)) "AlwaysSpawn" "MultiplyWithRoot" null null))
      (message `/Game/Chars/PerkSystem/PerkClasses/IN_Perk.ApplyPerk` _returnvalue_2 (`self.Holder`))
      (`Actor.K2_DestroyActor` _returnvalue_2))))

(fn `CheckBuffDeBuffDuration`
  (locals (LocBuffToRemove :type "/Game/Chars/PerkSystem/BuffDeBuffStruct Structure") (LocIndex :type Integer))
  (bind _locindex (`local.LocIndex`))
  (`KismetSystemLibrary.PrintText` "Check if any buffs need to be removed")
  (for (_array_element _array_index) (`self.ActiveBuffs`)
    (set `local.LocIndex` _array_index)
    (bind ((`Duration_17_E34068944B451771C8EBD395BC744633` _duration) (`icMultiCombat_25_2CA5FEBB4362D2A084B67B8CA3269E41` _icmulticombat)) (break `/Game/Chars/PerkSystem/BuffDeBuffStruct` _array_element))
    (if (not _icmulticombat)
      (bind _result (`/Engine/EditorBlueprintResources/StandardMacros.DecrementInt` _duration)
        (:`  `
          (`KismetSystemLibrary.PrintText` (`|FormatText` "Dur. was changed {dur++} real dur{rDur}" _result _duration))
          (if (<= _result 0)
            (set `local.LocBuffToRemove` (`|GetArrayItem` (`self.ActiveBuffs`) _locindex))
            (`KismetArrayLibrary.Array_Remove` (`self.ActiveBuffs`) _locindex)
            (`self.RemovePerk` (`.PerkType_6_43273B054447BC528895A4AF321DFF41` (break `/Game/Chars/PerkSystem/PerkData` (`.RelatedPerk_29_EB2A1D12466FE881AC54E0B511937B78` (break `/Game/Chars/PerkSystem/BuffDeBuffStruct` (`local.LocBuffToRemove`))))))
            (`KismetSystemLibrary.PrintText` "A Temp BUff was remvoed ")))))))

(fn `ConvertPerkToDTRow`
  (params (Perk :type "/Game/Chars/PerkSystem/PerkTypes Enum" :default "NewEnumerator0"))
  (returns (PerkDTRow :type "/Game/Chars/PerkSystem/PerkData Structure"))
  (bind _returnvalue (`|GetDataTableRow` "/Game/Chars/PerkSystem/DT_PerkList.DT_PerkList" (`KismetStringLibrary.Conv_StringToName` (`|GetEnumeratorNameAsString` Perk)))
    (:`then`
      (return _returnvalue))
    (:`RowNotFound`
      (`KismetSystemLibrary.PrintText` "ErrorNoPerkFoundGivenDefault")
      (bind _returnvalue_2 (`|GetDataTableRow` "/Game/Chars/PerkSystem/DT_PerkList.DT_PerkList" "TesterPerk1")
        (:`then`
          (return _returnvalue_2))))))

(fn `EndOfCombatBuffDeBuffHandle`
  (locals (LocIndex :type Integer) (LocBuffToRemove :type "/Game/Chars/PerkSystem/BuffDeBuffStruct Structure"))
  (for (_array_element _array_index) (`self.ActiveBuffs`)
    (set `local.LocIndex` _array_index)
    (bind ((`Duration_17_E34068944B451771C8EBD395BC744633` _duration) (`icMultiCombat_25_2CA5FEBB4362D2A084B67B8CA3269E41` _icmulticombat)) (break `/Game/Chars/PerkSystem/BuffDeBuffStruct` _array_element))
    (if _icmulticombat
      (bind _result (`/Engine/EditorBlueprintResources/StandardMacros.DecrementInt` _duration)
        (:`  `
          (if (<= _result 0)
            (`KismetSystemLibrary.PrintText` "A MC Buff was removed ")
            (set `local.LocBuffToRemove` (`|GetArrayItem` (`self.ActiveBuffs`) (`local.LocIndex`)) :!label _label)
            (`KismetArrayLibrary.Array_Remove` (`self.ActiveBuffs`) (`local.LocIndex`))
            (`self.RemovePerk` (`.PerkType_6_43273B054447BC528895A4AF321DFF41` (break `/Game/Chars/PerkSystem/PerkData` (`.RelatedPerk_29_EB2A1D12466FE881AC54E0B511937B78` (break `/Game/Chars/PerkSystem/BuffDeBuffStruct` (`local.LocBuffToRemove`)))))))))
      (else
        (`KismetSystemLibrary.PrintText` "A Temp buff was removed ")
        (goto _label)))))

(fn `GetInfoForTransfer`
  (returns (Perks :type "Map of /Game/Chars/PerkSystem/PerkTypes Enum to Integer") (ActiveBuffs :type "Array of /Game/Chars/PerkSystem/BuffDeBuffStruct Structure"))
  (return (`self.PerkList`) (`self.ActiveBuffs`)))

(fn `GetTriggersOnForGivenPerk`
  (params (PerrkToCheck :type "/Game/Chars/PerkSystem/PerkTypes Enum" :default "NewEnumerator0"))
  (returns (TriggersOn :type "Array of /Game/Chars/PerkSystem/TriggerTypes Enum"))
  (bind _perkdtrow (`self.ConvertPerkToDTRow` PerrkToCheck))
  (return (`.TriggerOn_15_9117973B45089E21EEDB49AD8E0340C3` (break `/Game/Chars/PerkSystem/PerkData` _perkdtrow))))

(fn `ReInit`
  (params (PerkList :type "Map of /Game/Chars/PerkSystem/PerkTypes Enum to Integer") (Holder :type "/Game/Chars/PZD_Unit Object Reference") (ActiveBuffs :type "Array of /Game/Chars/PerkSystem/BuffDeBuffStruct Structure"))
  (set `self.PerkList` PerkList)
  (set `self.Holder` Holder)
  (set `self.ActiveBuffs` ActiveBuffs))

(fn `RemovePerk`
  (params (PerkToRemove :type "/Game/Chars/PerkSystem/PerkTypes Enum" :default "NewEnumerator0"))
  (locals (LocPerkLvL :type Integer))
  (bind _value (`BlueprintMapLibrary.Map_Find` (`self.PerkList`) (`local.PerkToRemove`)))
  (if (`BlueprintMapLibrary.Map_Contains` (`self.PerkList`) (`local.PerkToRemove`))
    (`KismetSystemLibrary.PrintText` "perk will be removed i have his lvl")
    (bind _perkdtrow (`self.ConvertPerkToDTRow` (`local.PerkToRemove`)))
    (bind _returnvalue (`|SpawnActorFromClass` (`.PerkClass_24_8A42A5014A4964BB2B23CF95EA7C84BA` (break `/Game/Chars/PerkSystem/PerkData` _perkdtrow)) (`KismetMathLibrary.MakeTransform` (-999.0 -999.0 -999.0)) "AlwaysSpawn" "MultiplyWithRoot" null null))
    (message `/Game/Chars/PerkSystem/PerkClasses/IN_Perk.RemovePerk` _returnvalue (`self.Holder`) _value)
    (`Actor.K2_DestroyActor` _returnvalue)
    (`KismetSystemLibrary.PrintText` (`|FormatText` "perkwas removed lvl: {lvl}" _value))
    (`BlueprintMapLibrary.Map_Remove` (`self.PerkList`) (`local.PerkToRemove`))
    (`KismetSystemLibrary.PrintText` (`|FormatText` "perk is still in the list  {yn}" (`KismetTextLibrary.Conv_BoolToText` (`BlueprintMapLibrary.Map_Contains` (`self.PerkList`) (`local.PerkToRemove`)))))
    (else
      (`KismetSystemLibrary.PrintText` "ERROR removing perk that doesnt exist"))))

(fn `TriggerOnTakeDMG`
  (params (TriggeredWhen :type "/Game/Chars/PerkSystem/TriggerTypes Enum" :default "NewEnumerator0") (DmgDealt :type Integer) (DmgPen :type Integer) (DmgType :type "/Game/Chars/Attacks/Utilities/DmgTypes Enum" :default "NewEnumerator0") (DmgSituation :type "/Game/Chars/Attacks/Utilities/AttackSituations Enum" :default "NewEnumerator0"))
  (returns (NewDmgDealt :type Integer) (NewDmgPen :type Integer) (NewDmgType :type "/Game/Chars/Attacks/Utilities/DmgTypes Enum") (NewDmgSituation :type "/Game/Chars/Attacks/Utilities/AttackSituations Enum"))
  (locals (LocDmgDealt :type Integer) (LocDmgPen :type Integer) (LocDmgType :type "/Game/Chars/Attacks/Utilities/DmgTypes Enum" :default "NewEnumerator0") (LocDmgSituation :type "/Game/Chars/Attacks/Utilities/AttackSituations Enum" :default "NewEnumerator0") (LocPerksTriggered :type Integer))
  (set `local.LocDmgDealt` DmgDealt)
  (set `local.LocDmgPen` DmgPen)
  (set `local.LocDmgType` DmgType)
  (set `local.LocDmgSituation` DmgSituation)
  (bind _keys (`BlueprintMapLibrary.Map_Keys` (`self.PerkList`)))
  (for _array_element _keys
    (bind _triggerson (`self.GetTriggersOnForGivenPerk` _array_element))
    (if (`KismetArrayLibrary.Array_Contains` _triggerson (`local.TriggeredWhen`))
      (bind _perkdtrow (`self.ConvertPerkToDTRow` _array_element))
      (bind _returnvalue (`|SpawnActorFromClass` (`.PerkClass_24_8A42A5014A4964BB2B23CF95EA7C84BA` (break `/Game/Chars/PerkSystem/PerkData` _perkdtrow)) (`KismetMathLibrary.MakeTransform` (-999.0 -999.0 -999.0)) "AlwaysSpawn" "MultiplyWithRoot" null null))
      (bind (_perktriggerd _newdmgdealt _newdmgpen _newdmgtype _newdmgsituation) (message `/Game/Chars/PerkSystem/PerkClasses/IN_Perk.TriggerTakeDmg` _returnvalue (`local.TriggeredWhen`) (`local.LocDmgDealt`) (`local.LocDmgPen`) (`local.LocDmgType`) (`local.LocDmgSituation`) (`self.Holder`)))
      (if _perktriggerd
        (`/Engine/EditorBlueprintResources/StandardMacros.IncrementInt` (`local.LocPerksTriggered`)
          (:`  `
            (set `local.LocDmgDealt` _newdmgdealt)
            (set `local.LocDmgPen` _newdmgpen)
            (set `local.LocDmgType` _newdmgtype)
            (set `local.LocDmgSituation` _newdmgsituation))))
      (`Actor.K2_DestroyActor` _returnvalue)))
  (return (`local.LocDmgDealt`) (`local.LocDmgPen`) (`local.LocDmgType`) (`local.LocDmgSituation`)))