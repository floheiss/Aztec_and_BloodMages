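; BP_DotManager tracks bleed damage-over-time on its Holder unit in a turn-based system, with light, medium and heavy tiers.
; ApplyBleed clamps the rank and overwrites that tier's remaining duration.
; StartOFTurnDealBleedDMG sums fixed damage from active tiers, decrements their durations and calls DmgUnit on the Holder.
; IsAnyBleedActive repeats that tick, durations included, but returns an active flag and the damage total instead of dealing it.
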(fn `ApplyBleed`
  (params (BleedRank :type Integer) (Duration :type Integer))
  (switch `int` (`KismetMathLibrary.Clamp` BleedRank 0 2)
    (:`0`
      (set `self.LightBleed` (`local.Duration`)))
    (:`1`
      (set `self.MediumBleed` (`local.Duration`)))
    (:`2`
      (set `self.HeavyBleed` (`local.Duration`)))))

(fn `IsAnyBleedActive`
  (returns (AnyBleedActive :type Boolean) (DmgToDeal :type Integer))
  (locals (LocAmountBleeds :type Integer))
  (`|ExecutionSequence`
    (:`then_0`
      (if (> (`self.LightBleed`) 0)
        (set `local.LocAmountBleeds` (+ (`local.LocAmountBleeds`) 3))
        (`/Engine/EditorBlueprintResources/StandardMacros.DecrementInt` (`self.LightBleed`))))
    (:`then_1`
      (if (> (`self.MediumBleed`) 0)
        (set `local.LocAmountBleeds` (+ (`local.LocAmountBleeds`) 5))
        (`/Engine/EditorBlueprintResources/StandardMacros.DecrementInt` (`self.MediumBleed`))))
    (:`then_2`
      (if (> (`self.HeavyBleed`) 0)
        (set `local.LocAmountBleeds` (+ (`local.LocAmountBleeds`) 10))
        (`/Engine/EditorBlueprintResources/StandardMacros.DecrementInt` (`self.HeavyBleed`))))
    (:`then_3`
      (return (> (`local.LocAmountBleeds`) 0) (`local.LocAmountBleeds`)))))

(fn `StartOFTurnDealBleedDMG`
  (locals (LocAmountBleeds :type Integer))
  (`|ExecutionSequence`
    (:`then_0`
      (if (> (`self.LightBleed`) 0)
        (set `local.LocAmountBleeds` (+ (`local.LocAmountBleeds`) 3))
        (`/Engine/EditorBlueprintResources/StandardMacros.DecrementInt` (`self.LightBleed`))))
    (:`then_1`
      (if (> (`self.MediumBleed`) 0)
        (set `local.LocAmountBleeds` (+ (`local.LocAmountBleeds`) 5))
        (`/Engine/EditorBlueprintResources/StandardMacros.DecrementInt` (`self.MediumBleed`))))
    (:`then_2`
      (if (> (`self.HeavyBleed`) 0)
        (set `local.LocAmountBleeds` (+ (`local.LocAmountBleeds`) 10))
        (`/Engine/EditorBlueprintResources/StandardMacros.DecrementInt` (`self.HeavyBleed`))))
    (:`then_3`
      (`/Game/Chars/PZD_Unit.DmgUnit` (`self.Holder`) (`local.LocAmountBleeds`) 0 "NewEnumerator0" "NewEnumerator4"))))