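; Attack manager that tracks a character's available attacks, selected loadout, main attack and skill tree reference.
; Available attacks form a map of attack to upgraded flag, which gates upgrading, main-attack choice and additions to the size-capped selection.
; Selection edits swap the main attack into the first slot, and changes broadcast through event dispatchers.
; GetInfoForTransfer and ReInit export and restore the whole state for transfer between instances.
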(fn `AddAvaliableAttacks`
  (params (AttackToAdd :type "/Game/Chars/Attacks/Enums/AttackList Enum" :default "NewEnumerator1") (IsUpgraded :type Boolean) (IsMainAttack :type Boolean))
  (`BlueprintMapLibrary.Map_Add` (`self.AvaliableAttacks`) (`local.AttackToAdd`) (`local.IsUpgraded`))
  (`self.AvaliableAttacksChanged` (`self.AvaliableAttacks`))
  (if (`local.IsMainAttack`)
    (`self.SetMainAttack` (`local.AttackToAdd`))))

(fn `AddSelectedAttack`
  (params (AttackToAdd :type "/Game/Chars/Attacks/Enums/AttackList Enum" :default "NewEnumerator1"))
  (returns (Succ :type Boolean))
  (if (`.ReturnValue` (`BlueprintMapLibrary.Map_Find` (`self.AvaliableAttacks`) (`local.AttackToAdd`)))
    (if (< (`KismetArrayLibrary.Array_Length` (`self.SelectedAttacks`)) (`self.MaxNumberOfSelecedAttacks`))
      (`KismetArrayLibrary.Array_AddUnique` (`self.SelectedAttacks`) (`local.AttackToAdd`))
      (`self.SetMainAttackAsFirst`)
      (`self.AttackSelectionChanged` (`self.SelectedAttacks`))
      (return true)
      (else
        (return false)))
    (else
      (return false))))

(fn `ClearAvaliableAttck`
  (`BlueprintMapLibrary.Map_Clear` (`self.AvaliableAttacks`))
  (`self.AvaliableAttacksChanged` (`self.AvaliableAttacks`)))

(fn `ClearSelectedAttacks`
  (`KismetArrayLibrary.Array_Clear` (`self.SelectedAttacks`))
  (`self.AttackSelectionChanged` (`self.SelectedAttacks`)))

(fn `Get Upgraded Form Attack`
  (params (AttackToCheck :type "/Game/Chars/Attacks/Enums/AttackList Enum" :default "NewEnumerator1"))
  (returns (IsUpgaded :type Boolean))
  (return (`BlueprintMapLibrary.Map_Find` (`self.AvaliableAttacks`) (`local.AttackToCheck`))))

(fn `GetAllAvaliableAttacks`
  (returns (AvaliableAttacks :type "Map of /Game/Chars/Attacks/Enums/AttackList Enum to Boolean"))
  (return (`self.AvaliableAttacks`)))

(fn `GetAllSelecedAttacks`
  (returns (SelectedAttacks :type "Array of /Game/Chars/Attacks/Enums/AttackList Enum"))
  (`KismetArrayLibrary.Array_Swap` (`self.SelectedAttacks`) (`KismetArrayLibrary.Array_Find` (`self.SelectedAttacks`) (`self.MainAttack`)))
  (return (`self.SelectedAttacks`)))

(fn `GetInfoForTransfer`
  (returns (SelectedAttacks :type "Array of /Game/Chars/Attacks/Enums/AttackList Enum") (AvaliableAttacks :type "Map of /Game/Chars/Attacks/Enums/AttackList Enum to Boolean") (MainAttack :type "/Game/Chars/Attacks/Enums/AttackList Enum") (SkillTree :type "/Game/Core/GeneralEnums/SkillTreeList Enum"))
  (return (`self.SelectedAttacks`) (`self.AvaliableAttacks`) (`self.MainAttack`) (`self.SkillTree`)))

(fn `ReInit`
  (params (SelecedAttacks :type "Array of /Game/Chars/Attacks/Enums/AttackList Enum") (AvaliableAttacks :type "Map of /Game/Chars/Attacks/Enums/AttackList Enum to Boolean") (MainAttack :type "/Game/Chars/Attacks/Enums/AttackList Enum" :default "NewEnumerator1") (SkillTree :type "/Game/Core/GeneralEnums/SkillTreeList Enum" :default "NewEnumerator0"))
  (set `self.SelectedAttacks` SelecedAttacks)
  (set `self.AvaliableAttacks` AvaliableAttacks)
  (set `self.MainAttack` MainAttack)
  (set `self.SkillTree` SkillTree))

(fn `RemoveAvaliableAttack`
  (params (AttackToRemove :type "/Game/Chars/Attacks/Enums/AttackList Enum" :default "NewEnumerator1"))
  (`BlueprintMapLibrary.Map_Remove` (`self.AvaliableAttacks`) (`local.AttackToRemove`))
  (`self.AvaliableAttacksChanged` (`self.AvaliableAttacks`)))

(fn `ReMoveSelectedAttack`
  (params (AttackToRemove :type "/Game/Chars/Attacks/Enums/AttackList Enum" :default "NewEnumerator1"))
  (if (`|EnumInequality` (`local.AttackToRemove`) (`self.MainAttack`))
    (`KismetArrayLibrary.Array_RemoveItem` (`self.SelectedAttacks`) (`local.AttackToRemove`))
    (`self.SetMainAttackAsFirst`)
    (`self.AttackSelectionChanged` (`self.SelectedAttacks`))))

(fn `SetMainAttack`
  (params (Attack :type "/Game/Chars/Attacks/Enums/AttackList Enum" :default "NewEnumerator1"))
  (if (`.ReturnValue` (`BlueprintMapLibrary.Map_Find` (`self.AvaliableAttacks`) (`local.Attack`)))
    (set `self.MainAttack` (`local.Attack`))
    (`KismetArrayLibrary.Array_Add` (`self.SelectedAttacks`) (`self.MainAttack`))
    (`self.SetMainAttackAsFirst`)
    (`self.AttackSelectionChanged` (`self.SelectedAttacks`))))

(fn `SetMainAttackAsFirst`
  (`KismetArrayLibrary.Array_Swap` (`self.SelectedAttacks`) 0 (`KismetArrayLibrary.Array_Find` (`self.SelectedAttacks`) (`self.MainAttack`))))

(fn `UpgradeAttack`
  (params (AttackToUpgade :type "/Game/Chars/Attacks/Enums/AttackList Enum" :default "NewEnumerator1"))
  (returns (Succ :type Boolean))
  (bind (_value _returnvalue) (`BlueprintMapLibrary.Map_Find` (`self.AvaliableAttacks`) (`local.AttackToUpgade`)))
  (if _returnvalue
    (if (== _value false)
      (`BlueprintMapLibrary.Map_Add` (`self.AvaliableAttacks`) (`local.AttackToUpgade`) true)
      (`self.AttackUpgraded` (`self.AvaliableAttacks`))
      (return true)
      (else
        (`KismetSystemLibrary.PrintText` "ERROR tried upgrading an attack that was already upraded" true true (struct :`R` 1.0 :`B` 0.011716 :`A` 1.0) 10.0)
        (return false)))
    (else
      (`KismetSystemLibrary.PrintText` "ERROR tried upgrading an unavaliable attack" true true (struct :`R` 1.0 :`B` 0.011716 :`A` 1.0) 10.0)
      (return false))))