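; Assets manager for characters that sets up a holder's sprite to match its class and team.
; SetUp stores the Holder and its Sprite, then selects an image by class, with only BloodMage and Bandit assigned so far.
; It also sets the sprite's render transform angle, leaving team 0 unrotated and turning any other team half a turn.
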(event `SetUp`
  (params (Holder :type "/Game/Chars/PZD_Unit Object Reference"))
  (bind _output_get (set `self.Holder` Holder))
  (bind _output_get_2 (set `self.Sprite` (`/Game/Chars/PZD_Unit.Sprite` _output_get)))
  (`/Game/Chars/DeBug_Test/W_Test_Sprite.SetSrpite` _output_get_2 (select `/Game/Chars/Utilities/ClassList` (`/Game/Chars/PZD_Unit.Class` _output_get) :`NewEnumerator0` "/Game/Chars/SubClasses/BloodMages/Assets/Sprites/BloodMage_Attack_3/06813ee9-7230-40db-ae09-a75f4f7676d5.06813ee9-7230-40db-ae09-a75f4f7676d5" :`NewEnumerator11` "/Game/Chars/SubClasses/BloodMages/Assets/Sprites/BloodMage_Attack_3/71bd61bf-a84c-4bc7-ba86-1bbb4ce1d7a5.71bd61bf-a84c-4bc7-ba86-1bbb4ce1d7a5" :!type "Texture2D Object Reference"))
  (`Widget.SetRenderTransformAngle` (`self.Sprite`) (`KismetMathLibrary.SelectFloat` 0.0 180.0 (== (`/Game/Chars/PZD_Unit.Team` (`self.Holder`)) 0))))