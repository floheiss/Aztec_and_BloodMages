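; Per-unit level manager that tracks a mercenary's experience and level-ups, using the DT_UnitLvLStats row matching the holder's class.
; GainExp triggers LvLUp, which handles multi-level gains, scales the next threshold and adds HP and damage.
; Level-ups send PerkManager options, tiered stat points and level-gated stat choices to CallUnitLevelUp, boosting Epic/Legendary perk weights at five-level milestones.
; GetInfoForTransfer and ReInit carry state between instances.
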(event `self.ReceiveBeginPlay`)

(fn `FindPointsToSpend`
  (params (LvLToCheck :type Integer))
  (returns (PointsToSpend :type Integer))
  (locals (LocPoints :type Integer :default 0))
  (set `local.LocPoints` (select `/Game/Core/GeneralEnums/TierList` (`self.FindTierToCurrentLvL` (`local.LvLToCheck`)) :`NewEnumerator0` 1 :`NewEnumerator1` 2 :`NewEnumerator2` 3 :`NewEnumerator3` 4 :`NewEnumerator5` 4 :`NewEnumerator6` 6))
  (return (`local.LocPoints`)))

(fn `FindStatsToChange`
  (params (LvLToCheck :type Integer))
  (returns (StatsToChangeAndAmount :type "Map of /Game/Chars/Utilities/UnitStatToChange Enum to Integer"))
  (locals (LocStatMap :type "Map of /Game/Chars/Utilities/UnitStatToChange Enum to Integer"))
  (bind ((`PerLvLReRollCrit_32_960755B34FD7610033C815B82916200B` _perlvlrerollcrit) (`PerLvLReRollDoge_36_E9A1A4D643007A8D715B32AC16301F4A` _perlvlrerolldoge) (`PerLvLReRollAcc_34_4FAF0EF74D3E761D3A7D64AC4768DB61` _perlvlrerollacc)) (break `/Game/Chars/MercLvLManagment/UnitLvlData` (`self.UnitLvLData`)))
  (bind ((`PerLvLHp_11_5E6398B24A951D5311872AAEF84868DB` _perlvlhp) (`PerLvLDmg_28_D370B05542ADC504835AE3BDFFE21865` _perlvldmg) (`PerLvLCrit_54_0DCCF72542DEDBF3DB45EDB2185F7C82` _perlvlcrit) (`PerLvLMeleeArmor_13_DD4B40804972C729D02E4A87992E18D0` _perlvlmeleearmor) (`PerLvLRangedArmor_25_6A4D63F542443692A754F18B0479FC7D` _perlvlrangedarmor) (`PerLvLMagicArmor_18_13AD7BC749EC71D695889683A2DA3B5A` _perlvlmagicarmor)) (break `/Game/Chars/MercLvLManagment/UnitLvlData` (`self.UnitLvLData`)))
  (bind ((`PerLvLMeleePen_20_5D0E6DE84A024DC7CFA0F5ABFE2AF90E` _perlvlmeleepen) (`PerLvLRangedPen_23_E4FED9B1423F889BE05CF29DB078F650` _perlvlrangedpen) (`PerLvLMagicPen_24_F935E72F40B5E65D835B06A97906A207` _perlvlmagicpen) (`PerLvLDoge_29_C3DF64444E1C2B77C8D3FCAFC8DF5A91` _perlvldoge)) (break `/Game/Chars/MercLvLManagment/UnitLvlData` (`self.UnitLvLData`)))
  (`|ExecutionSequence`
    (:`then_0`
      ;[1 1 1] Base line can be gained very lvl
      (`BlueprintMapLibrary.Map_Add` (`local.LocStatMap`) "NewEnumerator0" _perlvlhp)
      (`BlueprintMapLibrary.Map_Add` (`local.LocStatMap`) "NewEnumerator9" _perlvldmg)
      (`BlueprintMapLibrary.Map_Add` (`local.LocStatMap`) "NewEnumerator18" _perlvlcrit)
      (`BlueprintMapLibrary.Map_Add` (`local.LocStatMap`) "NewEnumerator3" _perlvlmeleearmor)
      (`BlueprintMapLibrary.Map_Add` (`local.LocStatMap`) "NewEnumerator4" _perlvlrangedarmor)
      (`BlueprintMapLibrary.Map_Add` (`local.LocStatMap`) "NewEnumerator5" _perlvlmagicarmor))
    (:`then_1`
      (if (== (`KismetMathLibrary.FMod` (`KismetMathLibrary.Conv_IntToDouble` (`local.LvLToCheck`)) 5.0) 0.0)
        (`BlueprintMapLibrary.Map_Add` (`local.LocStatMap`) "NewEnumerator6" _perlvlmeleepen)
        (`BlueprintMapLibrary.Map_Add` (`local.LocStatMap`) "NewEnumerator7" _perlvlrangedpen)
        (`BlueprintMapLibrary.Map_Add` (`local.LocStatMap`) "NewEnumerator8" _perlvlmagicpen)
        (`BlueprintMapLibrary.Map_Add` (`local.LocStatMap`) "NewEnumerator10" _perlvldoge)))
    (:`then_2`
      (if (== (`KismetMathLibrary.FMod` (`KismetMathLibrary.Conv_IntToDouble` (`local.LvLToCheck`)) 10.0) 0.0)
        (`BlueprintMapLibrary.Map_Add` (`local.LocStatMap`) "NewEnumerator12" _perlvlrerollcrit)
        (`BlueprintMapLibrary.Map_Add` (`local.LocStatMap`) "NewEnumerator13" _perlvlrerolldoge)
        (`BlueprintMapLibrary.Map_Add` (`local.LocStatMap`) "NewEnumerator14" _perlvlrerollacc)))
    (:`then_3`
      ; checks so no values of <=0 are dispalyed
      (bind _keys (`BlueprintMapLibrary.Map_Keys` (`local.LocStatMap`)))
      (for _array_element _keys
        (if (<= (`BlueprintMapLibrary.Map_Find` (`local.LocStatMap`) _array_element) 0)
          (`BlueprintMapLibrary.Map_Remove` (`local.LocStatMap`) _array_element)))
      (return (`local.LocStatMap`)))))

(fn `FindTierToCurrentLvL`
  (params (CurrentLvL :type Integer))
  (returns (Tier :type "/Game/Core/GeneralEnums/TierList Enum"))
  (locals (LocTier :type "/Game/Core/GeneralEnums/TierList Enum" :default "NewEnumerator0"))
  (bind _returnvalue (cast `/Game/Core/GeneralEnums/TierList` (+ (`KismetSystemLibrary.MakeLiteralByte` (`local.LocTier`)) (`KismetMathLibrary.Conv_IntToByte` (`KismetMathLibrary.SelectInt` 1 0 (== (`KismetMathLibrary.FMod` (`KismetMathLibrary.Conv_IntToDouble` (`local.CurrentLvL`)) 5.0) 0.0))))))
  (`|ExecutionSequence`
    (:`then_0`
      (if (< (`local.CurrentLvL`) 5)
        (set `local.LocTier` "NewEnumerator0")
        (elif (< (`local.CurrentLvL`) 10)
          (set `local.LocTier` "NewEnumerator1")
          (elif (< (`local.CurrentLvL`) 10)
            (set `local.LocTier` "NewEnumerator2")
            (elif (< (`local.CurrentLvL`) 15)
              (set `local.LocTier` "NewEnumerator3")
              (elif (< (`local.CurrentLvL`) 20)
                (set `local.LocTier` "NewEnumerator5")))))))
    (:`then_1`
      (`KismetSystemLibrary.PrintText` (`|FormatText` "i will was selected for: {t} --> was upgrded to: {u}" (`|GetEnumeratorNameAsString` (stale _output_get)) (`|GetEnumeratorNameAsString` _returnvalue)))
      (bind _output_get (set `local.LocTier` _returnvalue))
      (return (`local.LocTier`)))))

(fn `GainExp`
  (params (ExpGained :type Integer))
  (bind _unitlvldata (`self.UnitLvLData`))
  (bind ((`CurrentExp_5_F750DCB74F9873F8005305B79826BFA1` _currentexp) (`NextLevelExp_7_0FC3BF0A4FB12C96A14874A47D29B174` _nextlevelexp)) (break `/Game/Chars/MercLvLManagment/UnitLvlData` (`self.UnitLvLData`)))
  (bind _structout (setmembers `/Game/Chars/MercLvLManagment/UnitLvlData` :`StructRef` _unitlvldata :`CurrentExp` (+ (`.CurrentExp_5_F750DCB74F9873F8005305B79826BFA1` (break `/Game/Chars/MercLvLManagment/UnitLvlData` _unitlvldata)) (`local.ExpGained`))))
  (if (>= _currentexp _nextlevelexp)
    (`self.LvLUp`)
    (else
      (bind ((`CurrentLevel_8_2439F2D94A72EA392640E2AC62DA3289` _currentlevel) (`CurrentExp_5_F750DCB74F9873F8005305B79826BFA1` _currentexp_2)) (break `/Game/Chars/MercLvLManagment/UnitLvlData` _structout))
      (`KismetSystemLibrary.PrintText` (`|FormatText` "I lvl up: {lvl} --> exp: {exp}" _currentlevel _currentexp_2)))))

(fn `Get Next Lv L Exp`
  (returns (NextLvLExp :type Integer))
  (locals (LocNextLvLBase :type Integer) (LocLvLMultiplayer :type "Float (double-precision)"))
  (set `local.LocNextLvLBase` (`.NextLevelExp_7_0FC3BF0A4FB12C96A14874A47D29B174` (break `/Game/Chars/MercLvLManagment/UnitLvlData` (`self.UnitLvLData`))))
  (bind _output_get (set `local.LocLvLMultiplayer` (select `int` (`.CurrentLevel_8_2439F2D94A72EA392640E2AC62DA3289` (break `/Game/Chars/MercLvLManagment/UnitLvlData` (`self.UnitLvLData`))) :`0` 0.0 :`1` 1.3 :`2` 1.3 :`3` 1.3 :`4` 1.3 :`5` 1.3 :`6` 1.2 :`7` 1.2 :`8` 1.2 :`9` 1.1 :`10` 1.1)))
  (return (* (`local.LocNextLvLBase`) _output_get)))

(fn `GetInfoForTransfer`
  (returns (UnitLvLData :type "/Game/Chars/MercLvLManagment/UnitLvlData Structure") (Last5xMultiApplied :type Integer) (NumberOfPerkSDisplayed :type Integer) (`Rarity Map` :type "Map of /Game/Core/GeneralEnums/TierList Enum to Float (double-precision)"))
  (return (`self.UnitLvLData`) (`self.Last5xMultiApplied`) (`self.NumberOfPerkSDisplayed`) (`self.Rarity Map`)))

(fn `GetRelatedRowFormDT`
  (returns (OutputPin :type "/Game/Chars/MercLvLManagment/UnitLvlData Structure"))
  (bind _outrownames (`DataTableFunctionLibrary.GetDataTableRowNames` "/Game/Chars/MercLvLManagment/DT_UnitLvLStats.DT_UnitLvLStats"))
  (for _array_element _outrownames
    (bind _returnvalue (`|GetDataTableRow` "/Game/Chars/MercLvLManagment/DT_UnitLvLStats.DT_UnitLvLStats" _array_element)
      (:`then`
        (if (`|EnumEquality` (`.RelatedClass_42_AC3336B94C41FBD132E70D9B88290488` (break `/Game/Chars/MercLvLManagment/UnitLvlData` _returnvalue)) (`/Game/Chars/PZD_Unit.Class` (`self.Holder`)))
          (return _returnvalue)))))
  (`KismetSystemLibrary.PrintText` "ERROR Sir we if fact did not fine a related class for lvl stats" true true (struct :`R` 1.0 :`B` 0.050762 :`A` 1.0) 5.0))

(fn `LvLUp`
  (locals (LocLvLGained :type Integer) (LocArrayDisplayedPerks :type "Array of /Game/Chars/PerkSystem/PerkTypes Enum") (LocRarityMap :type "Map of /Game/Core/GeneralEnums/TierList Enum to Float (double-precision)") (LocCurrentLvL :type Integer))
  (bind ((`PerLvLHp_11_5E6398B24A951D5311872AAEF84868DB` _perlvlhp) (`PerLvLDmg_28_D370B05542ADC504835AE3BDFFE21865` _perlvldmg)) (break `/Game/Chars/MercLvLManagment/UnitLvlData` (`self.UnitLvLData`)))
  (bind ((`CurrentLevel_8_2439F2D94A72EA392640E2AC62DA3289` _currentlevel)) (break `/Game/Chars/MercLvLManagment/UnitLvlData` (`self.UnitLvLData`)))
  (bind ((`CurrentExp_5_F750DCB74F9873F8005305B79826BFA1` _currentexp) (`NextLevelExp_7_0FC3BF0A4FB12C96A14874A47D29B174` _nextlevelexp)) (break `/Game/Chars/MercLvLManagment/UnitLvlData` (`self.UnitLvLData`)))
  (bind ((`CurrentExp_5_F750DCB74F9873F8005305B79826BFA1` _currentexp_2) (`NextLevelExp_7_0FC3BF0A4FB12C96A14874A47D29B174` _nextlevelexp_2)) (break `/Game/Chars/MercLvLManagment/UnitLvlData` (`self.UnitLvLData`)))
  (set `local.LocRarityMap` (`self.Rarity Map`))
  (`|ExecutionSequence`
    (:`then_0`
      (set `local.LocCurrentLvL` _currentlevel)
      (setmembers `/Game/Chars/MercLvLManagment/UnitLvlData` :`StructRef` (`self.UnitLvLData`) :`CurrentLevel` (+ _currentlevel 1) :`CurrentExp` (- _currentexp_2 _nextlevelexp_2) :!label _label)
      (bind _nextlvlexp (`self.Get Next Lv L Exp`))
      (setmembers `/Game/Chars/MercLvLManagment/UnitLvlData` :`StructRef` (`self.UnitLvLData`) :`NextLevelExp` _nextlvlexp)
      (if (>= _currentexp _nextlevelexp)
        (`/Engine/EditorBlueprintResources/StandardMacros.IncrementInt` (`local.LocLvLGained`)
          (:`  `
            (goto _label)))))
    (:`then_1`
      (for _ (range (+ (`local.LocLvLGained`) 1))
        ;[1 1 1] On lvl always + hp +dmg
        (`/Engine/EditorBlueprintResources/StandardMacros.IncrementInt` (`local.LocCurrentLvL`)
          (:`  `
            (`/Game/Chars/PZD_Unit.SetMoreUnitStat` (`self.Holder`) false (`|MakeMap` "NewEnumerator0" _perlvlhp "NewEnumerator9" _perlvldmg :!type "/Game/Chars/Utilities/UnitStatToChange Enum"))
            (`|ExecutionSequence`
              (:`then_0`
                ;[1 1 1] triggers every 5x lvl / is used to upgrade the rarity map
                (if (> (* (`.ReturnValue` (`KismetMathLibrary.FMod` (`KismetMathLibrary.Conv_IntToDouble` (`.CurrentLevel_8_2439F2D94A72EA392640E2AC62DA3289` (break `/Game/Chars/MercLvLManagment/UnitLvlData` (`self.UnitLvLData`)))) 5.0)) 5) (`self.Last5xMultiApplied`))
                  (set `self.Last5xMultiApplied` (* (`.ReturnValue` (`KismetMathLibrary.FMod` (`KismetMathLibrary.Conv_IntToDouble` (`.CurrentLevel_8_2439F2D94A72EA392640E2AC62DA3289` (break `/Game/Chars/MercLvLManagment/UnitLvlData` (`self.UnitLvLData`)))) 5.0)) 5))
                  (`BlueprintMapLibrary.Map_Add` (`local.LocRarityMap`) "NewEnumerator2" (+ (`BlueprintMapLibrary.Map_Find` (`local.LocRarityMap`) "NewEnumerator2") 0.2))
                  (`BlueprintMapLibrary.Map_Add` (`local.LocRarityMap`) "NewEnumerator3" (+ (`BlueprintMapLibrary.Map_Find` (`local.LocRarityMap`) "NewEnumerator3") 0.1))))
              (:`then_1`
                (bind _discoveredperk (`/Game/Chars/PerkSystem/BP_PerkManager.GenPerkOnLvLUp` (`/Game/Chars/PZD_Unit.PerkManager` (`self.Holder`)) (`self.NumberOfPerkSDisplayed`) (`local.LocRarityMap`)))
                (`self.UnitLevelUp` (make `/Game/Chars/MercLvLManagment/UnitLeveledDisplayUpData` (`self.Holder`) (`self.FindPointsToSpend` (`local.LocCurrentLvL`)) _discoveredperk (`self.FindStatsToChange` (`local.LocCurrentLvL`))))))))))))

(fn `ReInit`
  (params (Holder :type "/Game/Chars/PZD_Unit Object Reference") (UnitLvLData :type "/Game/Chars/MercLvLManagment/UnitLvlData Structure") (Last5xMultiApplied :type Integer) (NumberOfPerksDisplayed :type Integer) (RarityMap :type "Map of /Game/Core/GeneralEnums/TierList Enum to Float (double-precision)"))
  (set `self.Holder` Holder)
  (set `self.UnitLvLData` UnitLvLData)
  (set `self.Last5xMultiApplied` Last5xMultiApplied)
  (set `self.NumberOfPerkSDisplayed` NumberOfPerksDisplayed)
  (set `self.Rarity Map` RarityMap))

(fn `SetUp`
  (params (Holder :type "/Game/Chars/PZD_Unit Object Reference"))
  (set `self.Holder` Holder)
  (bind _outputpin (`self.GetRelatedRowFormDT`))
  (set `self.UnitLvLData` _outputpin)
  (set `self.NumberOfPerkSDisplayed` 3))