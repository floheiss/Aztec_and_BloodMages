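; Manages a unit's bonus ability stats, tracking gun ammunition and a blood resource in one UnitBonusStats struct.
; ReInit and GetInfoForTransfer set and return that struct for handover.
; Gun functions fire, reload and raise capacity, with firing and reloading calling dispatchers.
; Blood gains and max changes are clamped, while RemoveBlood subtracts only when the amount is at least current blood, otherwise showing "To little blood", and always returns false.
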(fn `ChangeMaxBlood`
  (params (Amount :type Integer) (Remove :type Boolean))
  (bind ((`CurrentBlood_15_C6C4EF7643F97017CEB4408207E565A5` _currentblood) (`MaxBlood_16_A036775948B87069DB12A3B67E0B41EA` _maxblood)) (break `/Game/Chars/UnitBonusInfoManager/Unit_BonusAbilityStruct` (`self.UnitBonusStats`)))
  (bind _returnvalue (`KismetMathLibrary.Max` (+ _maxblood (`KismetMathLibrary.SelectInt` (* Amount -1) (`local.Amount`) Remove))))
  (setmembers `/Game/Chars/UnitBonusInfoManager/Unit_BonusAbilityStruct` :`StructRef` (`self.UnitBonusStats`) :`CurrentBlood` (`KismetMathLibrary.Min` _returnvalue _currentblood) :`MaxBlood` _returnvalue))

(fn `Check Gun Shot Remaing`
  (returns (ReturnValue :type Boolean))
  (return (>= (`.GunLoadedShots_5_040A195641275EB51A1A1DB5022C0BCF` (break `/Game/Chars/UnitBonusInfoManager/Unit_BonusAbilityStruct` (`self.UnitBonusStats`))) 1)))

(fn `CheckBloodAmount`
  (params (AmountToCheck :type Integer))
  (returns (IsValid :type Boolean))
  (return (>= AmountToCheck (`.CurrentBlood_15_C6C4EF7643F97017CEB4408207E565A5` (break `/Game/Chars/UnitBonusInfoManager/Unit_BonusAbilityStruct` (`self.UnitBonusStats`))))))

(fn `GainBlood`
  (params (ToAdd :type Integer))
  (bind ((`CurrentBlood_15_C6C4EF7643F97017CEB4408207E565A5` _currentblood) (`MaxBlood_16_A036775948B87069DB12A3B67E0B41EA` _maxblood)) (break `/Game/Chars/UnitBonusInfoManager/Unit_BonusAbilityStruct` (`self.UnitBonusStats`)))
  (setmembers `/Game/Chars/UnitBonusInfoManager/Unit_BonusAbilityStruct` :`StructRef` (`self.UnitBonusStats`) :`CurrentBlood` (`KismetMathLibrary.Clamp` (+ _currentblood (`local.ToAdd`)) 0 _maxblood))
  (return))

(fn `GetInfoForTransfer`
  (returns (UnitBonusStats :type "/Game/Chars/UnitBonusInfoManager/Unit_BonusAbilityStruct Structure"))
  (return (`self.UnitBonusStats`)))

(fn `IncreaseGunMaxShots`
  (bind _unitbonusstats (`self.UnitBonusStats`))
  (bind ((`GunMaxAmunition_3_1F9B070C41AB8D314FC9378C0F00AED7` _gunmaxamunition) (`GunLoadedShots_5_040A195641275EB51A1A1DB5022C0BCF` _gunloadedshots)) (break `/Game/Chars/UnitBonusInfoManager/Unit_BonusAbilityStruct` _unitbonusstats))
  (setmembers `/Game/Chars/UnitBonusInfoManager/Unit_BonusAbilityStruct` :`StructRef` _unitbonusstats :`GunMaxAmunition` (+ _gunmaxamunition 1) :`GunLoadedShots` (+ _gunloadedshots 1)))

(fn `ReInit`
  (params (UnitBonusStats :type "/Game/Chars/UnitBonusInfoManager/Unit_BonusAbilityStruct Structure") (Holder :type "/Game/Chars/PZD_Unit Object Reference"))
  (set `self.UnitBonusStats` UnitBonusStats)
  (set `self.Holder` Holder))

(fn `ReLoadGun`
  (params (Amount :type Integer :default -1))
  (setmembers `/Game/Chars/UnitBonusInfoManager/Unit_BonusAbilityStruct` :`StructRef` (`self.UnitBonusStats`) :`GunLoadedShots` (select `bool` (!= Amount -1) :`false` (`.GunMaxAmunition_3_1F9B070C41AB8D314FC9378C0F00AED7` (break `/Game/Chars/UnitBonusInfoManager/Unit_BonusAbilityStruct` (`self.UnitBonusStats`))) :`true` (`local.Amount`)))
  (`self.GunLoaded` (`local.Amount`)))

(fn `RemoveBlood`
  (params (ToRemove :type Integer))
  (returns (IsValid :type Boolean))
  (bind _unitbonusstats (`self.UnitBonusStats`))
  (if (`self.CheckBloodAmount` (`local.ToRemove`))
    (setmembers `/Game/Chars/UnitBonusInfoManager/Unit_BonusAbilityStruct` :`StructRef` _unitbonusstats :`CurrentBlood` (- (`.CurrentBlood_15_C6C4EF7643F97017CEB4408207E565A5` (break `/Game/Chars/UnitBonusInfoManager/Unit_BonusAbilityStruct` _unitbonusstats)) (`local.ToRemove`)))
    (return false)
    (else
      (message `/Game/Core/IN_UniversalController.DisplayNotification` (`GameplayStatics.GetPlayerController` 0) "To little blood" 3.0)
      (return false))))

(fn `UseGun`
  (setmembers `/Game/Chars/UnitBonusInfoManager/Unit_BonusAbilityStruct` :`StructRef` (`self.UnitBonusStats`) :`GunLoadedShots` (- (`.GunLoadedShots_5_040A195641275EB51A1A1DB5022C0BCF` (break `/Game/Chars/UnitBonusInfoManager/Unit_BonusAbilityStruct` (`self.UnitBonusStats`))) 1))
  (`self.CallGunFired`))