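; Enemy combat AI manager that chooses an attack and its targets for the unit that holds it.
; AiAttack picks a seeded random attack from the holder's AttackManager, then draws unique random Team0 members from CombatManager to match its target count, within ten tries.
; Helpers select targets at random or by lowest stat via a bubble-style sort; several smarter attack-selection functions are stubs or unreachable.
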(fn `AiAttack`
  (returns (AttackToUse :type "/Game/Chars/Attacks/AttackData Structure") (SelectedTargets :type "Array of /Game/Chars/PZD_Unit Object Reference"))
  (locals (LocSelectedAttack :type "/Game/Chars/Attacks/Enums/AttackList Enum" :default "NewEnumerator1") (LocAttackData :type "/Game/Chars/Attacks/AttackData Structure") (Loctargets :type "Array of /Game/Chars/PZD_Unit Object Reference"))
  (bind _attacktouse (`self.GenerateAttack`))
  (bind _output_get (set `local.LocAttackData` _attacktouse))
  (bind _selectedtargets (`self.GenerateTargets` (`.targetNumber_15_1FF9936C4D7DA3AF4B7193B8A06134B1` (break `/Game/Chars/Attacks/AttackData` _output_get))))
  (set `local.Loctargets` _selectedtargets)
  (return (`local.LocAttackData`) (`local.Loctargets`)))

(fn `CheckIfKindExistsAndFindMostDmg`
  (params (AvaliableAttacks :type "Array of /Game/Chars/Attacks/Enums/AttackList Enum"))
  (returns (Attack :type "/Game/Chars/Attacks/Enums/AttackList Enum"))
  (return "NewEnumerator1"))

(fn `FindAttackWithMostTargets`
  (params (AvaliableAttacks :type "Array of /Game/Chars/Attacks/Enums/AttackList Enum"))
  (returns (AttackFound :type "/Game/Chars/Attacks/Enums/AttackList Enum"))
  (locals (LocTargetNumber :type Integer))
  (return (`KismetArrayLibrary.Array_RandomFromStream` AvaliableAttacks (`/Game/Core/GI_Persistence.CurrentSeed` (`/Game/Core/BFL_General.GetGameInst`)))))

(fn `FindBloodMage`
  (returns (BloodMage :type "Array of /Game/Chars/PZD_Unit Object Reference"))
  (return))

(fn `FindHeal`
  (params (AvaliableAttacks :type "Array of /Game/Chars/Attacks/Enums/AttackList Enum"))
  (returns (Attack :type "/Game/Chars/Attacks/Enums/AttackList Enum"))
  (locals (LocAttacks :type "Array of /Game/Chars/Attacks/Enums/AttackList Enum") (LocClass :type "/Game/Chars/Attacks/Enums/AttackList Enum") (LocHealFound :type Boolean)))

(fn `FindMostDmgAttack`
  (params (AvaliableAttacks :type "Array of /Game/Chars/Attacks/Enums/AttackList Enum"))
  (returns (Attack :type "/Game/Chars/Attacks/Enums/AttackList Enum"))
  (locals (LocAttacks :type "Array of /Game/Chars/Attacks/Enums/AttackList Enum") (LocMulti :type Integer) (LocClass :type "/Game/Chars/Attacks/Enums/AttackList Enum"))
  (return (`local.LocClass`)))

(fn `FindRandomTarget`
  (params (NumberToFind :type Integer) (PossibleTargets :type "/Game/Chars/Attacks/Enums/PossibleTargets Enum" :default "NewEnumerator1"))
  (returns (Targets :type "Array of /Game/Chars/PZD_Unit Object Reference"))
  (locals (LocTargets :type "Array of /Game/Chars/PZD_Unit Object Reference") (LocFoundTargets :type "Array of /Game/Chars/PZD_Unit Object Reference") (LocIndexI :type Integer) (LocIndexJ :type Integer) (LocArrayLen :type Integer :default 0))
  (bind _targets (`/Game/Combat/CombatManager.FindPossibleTargets` (`self.GetCombatManager`)))
  (bind _output_get (set `local.LocTargets` _targets))
  (`KismetArrayLibrary.Array_Shuffle` _output_get)
  (for _index (range (`local.NumberToFind`))
    (`KismetArrayLibrary.Array_Add` (`local.LocFoundTargets`) (`|GetArrayItem` (`local.LocTargets`) _index)))
  (return (`local.LocFoundTargets`)))

(fn `GenerateAttack`
  (returns (AttackToUse :type "/Game/Chars/Attacks/AttackData Structure"))
  (locals (LocAvaliableAttacks :type "Map of /Game/Chars/Attacks/Enums/AttackList Enum to Boolean") (LocAttackList :type "/Game/Chars/Attacks/Enums/AttackList Enum") (LocAvaliableKeys :type "Array of /Game/Chars/Attacks/Enums/AttackList Enum"))
  (bind _avaliableattacks (`/Game/Chars/AttackManager/BP_AttackManager.GetAllAvaliableAttacks` (`/Game/Chars/PZD_Unit.AttackManager` (`self.Holder`))))
  (bind _output_get (set `local.LocAvaliableAttacks` _avaliableattacks))
  (bind _keys (`BlueprintMapLibrary.Map_Keys` _output_get))
  (bind _attackdata (`/Game/Chars/Attacks/BFL_Attacks.getAttackDataFormAttack` (`KismetArrayLibrary.Array_RandomFromStream` _keys (`/Game/Core/BFL_General.GetCurrentSeed`))))
  (return _attackdata))

(fn `GenerateTargets`
  (params (NumberOfTargets :type Integer))
  (returns (SelectedTargets :type "Array of /Game/Chars/PZD_Unit Object Reference"))
  (locals (LocTargets :type "Array of /Game/Chars/PZD_Unit Object Reference") (LocTies :type Integer) (LocCombatManager :type "/Game/Combat/CombatManager Object Reference"))
  (bind _returnvalue (`GameplayStatics.GetActorOfClass` "/Game/Combat/CombatManager.CombatManager_C"))
  (set `local.LocCombatManager` _returnvalue)
  (while (and (< (`KismetArrayLibrary.Array_Length` (`local.LocTargets`)) (`local.NumberOfTargets`)) (< (`local.LocTies`) 10))
    (`/Engine/EditorBlueprintResources/StandardMacros.IncrementInt` (`local.LocTies`)
      (:`  `
        (`KismetArrayLibrary.Array_AddUnique` (`local.LocTargets`) (`KismetArrayLibrary.Array_Random` (`/Game/Combat/CombatManager.Team0` (`local.LocCombatManager`)))))))
  (if (not (== (`KismetArrayLibrary.Array_Length` (`local.LocTargets`)) (`local.NumberOfTargets`)))
    (`KismetSystemLibrary.PrintText` "PROBLEM to few targets found " true true (struct :`R` 1.0 :`B` 0.005072 :`A` 1.0) 20.0))
  (return (`local.LocTargets`)))

(fn `GetCombatManager`
  (returns (CombatManager :type "/Game/Combat/CombatManager Object Reference"))
  (bind _returnvalue (`GameplayStatics.GetActorOfClass` "/Game/Combat/CombatManager.CombatManager_C"))
  (return _returnvalue))

(fn `ReInit`
  (params (AIActive :type Boolean) (Holder :type "/Game/Chars/PZD_Unit Object Reference"))
  (set `self.AiActive` AIActive)
  (set `self.Holder` Holder))

(fn `SortLowestGivenStat`
  (params (NumberToFind :type Integer) (StatToCheckFor :type "/Game/Chars/Utilities/UnitStatToChange Enum" :default "NewEnumerator0"))
  (returns (Targets :type "Array of /Game/Chars/PZD_Unit Object Reference"))
  (locals (LocTargets :type "Array of /Game/Chars/PZD_Unit Object Reference") (LocFoundTargets :type "Array of /Game/Chars/PZD_Unit Object Reference") (LocIndexI :type Integer) (LocIndexJ :type Integer) (LocArrayLen :type Integer :default 0))
  (bind _targets (`/Game/Combat/CombatManager.FindPossibleTargets` (`self.GetCombatManager`)))
  (bind _output_get (set `local.LocTargets` _targets))
  (set `local.LocArrayLen` (`KismetArrayLibrary.Array_Length` _output_get))
  (if (> (`local.LocArrayLen`) 1)
    (for _index (range (`local.LocArrayLen`))
      (set `local.LocIndexI` _index)
      (for _index_2 (range (+ (- (`local.LocArrayLen`) (`local.LocIndexI`) 1) 1))
        (set `local.LocIndexJ` _index_2)
        (if (> (`/Game/Chars/PZD_Unit.GetUnitStat` (`|GetArrayItem` (`local.LocTargets`) (`local.LocIndexJ`)) (`local.StatToCheckFor`)) (`/Game/Chars/PZD_Unit.GetUnitStat` (`|GetArrayItem` (`local.LocTargets`) (+ (`local.LocIndexJ`) 1)) (`local.StatToCheckFor`)))
          (`KismetArrayLibrary.Array_Swap` (`local.LocTargets`) (`local.LocIndexJ`) (+ (`local.LocIndexJ`) 1))
          (break)))))
  (for _index_3 (range (`local.NumberToFind`))
    (`KismetArrayLibrary.Array_Add` (`local.LocFoundTargets`) (`|GetArrayItem` (`local.LocTargets`) _index_3)))
  (return (`local.LocFoundTargets`)))