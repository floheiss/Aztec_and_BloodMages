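; Bandit enemy AI persona that decides which attack to make and whom it hits in combat.
; GenerateAttack picks one of two attack types at even odds, using the game instance's seeded random stream, and fetches its attack data.
; AiMakeAttack has the CombatManager find possible targets for that attack, then returns it with randomly chosen targets matching its target count.
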(fn `AiMakeAttack`
  (returns (AttackData :type "/Game/Chars/Attacks/AttackData Structure") (Targets :type "Array of /Game/Chars/PZD_Unit Object Reference"))
  (bind _attackdata (`self.GenerateAttack`))
  (`/Game/Combat/BP_CombatManager.FindPossibleTargetsAi` (`self.CombatManager`) _attackdata)
  (bind _targets (`self.FindRandomTargets` (`.targetNumber_15_1FF9936C4D7DA3AF4B7193B8A06134B1` (break `/Game/Chars/Attacks/AttackData` _attackdata))))
  (return _attackdata _targets))

(fn `GenerateAttack`
  (returns (AttackData :type "/Game/Chars/Attacks/AttackData Structure"))
  (bind _attackdata (`/Game/Chars/Attacks/BFL_Attacks.getAttackDataFormAttack` (select `bool` (`KismetMathLibrary.RandomBoolWithWeightFromStream` (`/Game/Core/GI_Persistence.CurrentSeed` (`/Game/Core/BFL_General.GetGameInst`))) :`false` "NewEnumerator10" :`true` "NewEnumerator15" :!type "/Game/Chars/Attacks/Enums/AttackList Enum")))
  (return _attackdata))

(fn `UserConstructionScript`
  (`parent.UserConstructionScript`))