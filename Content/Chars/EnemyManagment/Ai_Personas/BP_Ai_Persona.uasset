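; BP_Ai_Persona is an enemy AI persona that chooses attacks and targets in combat, with GenerateAttack left empty.
; Setup applies its perks to the holder's PerkManager and caches the level's BP_CombatManager.
; Helpers pick targets randomly, by unit class, or by lowest stat via a bubble-style pass that stops after each first swap.
; AiMakeAttack pairs a fixed attack with random targets from the combat manager, bypassing the random-attack helper.
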(event `/Game/Chars/EnemyManagment/Ai_Personas/IN_Ai_Persona.AiSetUp`
  (params (Holder :type "/Game/Chars/PZD_Unit Object Reference"))
  (set `self.Holder` Holder)
  (for _array_element (`self.PerksToAdd`)
    (`/Game/Chars/PerkSystem/BP_PerkManager.ApplyPerk` (`/Game/Chars/PZD_Unit.PerkManager` (`self.Holder`)) _array_element)))

(event `/Game/Chars/EnemyManagment/Ai_Personas/IN_Ai_Persona.AiCombatSetUp`
  (bind _returnvalue (`GameplayStatics.GetActorOfClass` "/Game/Combat/BP_CombatManager.BP_CombatManager_C"))
  (set `self.CombatManager` _returnvalue))

(fn `AiMakeAttack`
  (returns (AttackData :type "/Game/Chars/Attacks/AttackData Structure") (Targets :type "Array of /Game/Chars/PZD_Unit Object Reference"))
  (bind _attackdata (`/Game/Chars/Attacks/BFL_Attacks.getAttackDataFormAttack` "NewEnumerator9"))
  (`/Game/Combat/BP_CombatManager.FindPossibleTargetsAi` (`self.CombatManager`) _attackdata)
  (bind _targets (`self.FindRandomTargets` (`.targetNumber_15_1FF9936C4D7DA3AF4B7193B8A06134B1` (break `/Game/Chars/Attacks/AttackData` _attackdata))))
  (return _attackdata _targets))

(fn `BasicGenRandomAttack`
  (returns (Attack :type "/Game/Chars/Attacks/Enums/AttackList Enum"))
  (return (`KismetArrayLibrary.Array_Random` (`self.AllPossibleAttack`))))

(fn `FindBloodMage`
  (returns (BloodMage :type "Array of /Game/Chars/PZD_Unit Object Reference"))
  (locals (LocTargets :type "Array of /Game/Chars/PZD_Unit Object Reference"))
  (bind _targets (`/Game/Combat/BP_CombatManager.FindPossibleTargets` (`self.CombatManager`)))
  (for _array_element _targets
    (if (`|EnumEquality` (`/Game/Chars/PZD_Unit.UnitClass` _array_element) "NewEnumerator0")
      (`KismetArrayLibrary.Array_Add` (`local.LocTargets`) _array_element)
      (break)))
  (return (`local.LocTargets`)))

(fn `FindRandomTargets`
  (params (NumberOfTargets :type Integer))
  (returns (Targets :type "Array of /Game/Chars/PZD_Unit Object Reference"))
  (locals (LocTargets :type "Array of /Game/Chars/PZD_Unit Object Reference") (LocFoundTargets :type "Array of /Game/Chars/PZD_Unit Object Reference"))
  (bind _output_get (set `local.LocTargets` (`/Game/Combat/BP_CombatManager.PossibleTargets` (`self.CombatManager`))))
  (`KismetArrayLibrary.Array_Shuffle` _output_get)
  (for _index (range (`local.NumberOfTargets`))
    (`KismetArrayLibrary.Array_Add` (`local.LocFoundTargets`) (`|GetArrayItem` (`local.LocTargets`) _index)))
  (return (`local.LocFoundTargets`)))

(fn `FindTargetOfLowestGivenStat`
  (params (NumberOfTargets :type Integer) (UnitStat :type "/Game/Chars/Utilities/UnitStatToChange Enum" :default "NewEnumerator0"))
  (returns (Targets :type "Array of /Game/Chars/PZD_Unit Object Reference"))
  (locals (LocTargets :type "Array of /Game/Chars/PZD_Unit Object Reference") (LocArrayLen :type Integer) (LocFoundTargets :type "Array of /Game/Chars/PZD_Unit Object Reference") (LocIndexI :type Integer) (LocIndexJ :type Integer))
  (bind _unitstat (`local.UnitStat`))
  (bind _targets (`/Game/Combat/BP_CombatManager.FindPossibleTargets` (`self.CombatManager`)))
  (bind _output_get (set `local.LocTargets` _targets))
  (set `local.LocArrayLen` (`KismetArrayLibrary.Array_Length` _output_get))
  (if (> (`local.LocArrayLen`) 1)
    (for _index (range (`local.LocArrayLen`))
      (set `local.LocIndexI` _index)
      (for _index_2 (range (+ (- (`local.LocArrayLen`) (`local.LocIndexI`) 1) 1))
        (set `local.LocIndexJ` _index_2)
        (if (> (`/Game/Chars/PZD_Unit.GetUnitStat` (`|GetArrayItem` (`local.LocTargets`) (`local.LocIndexJ`)) _unitstat) (`/Game/Chars/PZD_Unit.GetUnitStat` (`|GetArrayItem` (`local.LocTargets`) (+ (`local.LocIndexJ`) 1)) _unitstat))
          (`KismetArrayLibrary.Array_Swap` (`local.LocTargets`) (`local.LocIndexJ`) (+ (`local.LocIndexJ`) 1))
          (break)))))
  (for _index_3 (range (`local.NumberOfTargets`))
    (`KismetArrayLibrary.Array_Add` (`local.LocFoundTargets`) (`|GetArrayItem` (`local.LocTargets`) _index_3)))
  (return (`local.LocFoundTargets`)))

(fn `GenerateAttack`
  (returns (AttackData :type "/Game/Chars/Attacks/AttackData Structure"))
  (return))

(fn `UserConstructionScript`)