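; Town skill tree manager that opens the skill tree menu and handles buying attack tiers with party gold.
; DisplaySkillTree shows the W_SkillTrees widget on the player's HUD and sets the game instance's menu state.
; BuyAttack checks gold against the tier price, increments the tier in BloodMageUnlockedAttacks, deducts gold and calls BroughtAttack.
; The deducted price is looked up after the increment, so it uses the new tier's index.
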(event `DisplaySkillTree`
  (bind _returnvalue (`|CreateWidget` "/Game/Town/SkillTrees/HUD/W_SkillTrees.W_SkillTrees_C"))
  (message `/Game/Core/IN_UniversalController.SetDisplayedHUD` (`GameplayStatics.GetPlayerController` 0) _returnvalue)
  (`/Game/Core/GI_Persistence.SetMenu` (`/Game/Core/BFL_General.GetGameInst`) "NewEnumerator13"))

(fn `BuyAttack`
  (params (AttackToBuy :type "/Game/Chars/Attacks/Enums/AttackList Enum" :default "NewEnumerator1"))
  (returns (Succ :type Boolean))
  (locals (LocSkillTreeData :type "/Game/Chars/Attacks/AttackSkillTreeData Structure"))
  (bind _bloodmageunlockedattacks (`/Game/Core/GI_Persistence.BloodMageUnlockedAttacks` (`/Game/Core/BFL_General.GetGameInst`)))
  (bind (_value _returnvalue) (`BlueprintMapLibrary.Map_Find` (`/Game/Core/GI_Persistence.BloodMageUnlockedAttacks` (`/Game/Core/BFL_General.GetGameInst`)) (`local.AttackToBuy`)))
  (bind _relatedattackskilltree (`/Game/Chars/Attacks/BFL_Attacks.GetAttackSkillDataFromAttack` AttackToBuy))
  (bind _output_get (set `local.LocSkillTreeData` _relatedattackskilltree))
  (bind _output (`|GetArrayItem` (`.Price_22_0F67AF674B31102D8DDBD9A2DD8B7AF8` (break `/Game/Chars/Attacks/AttackSkillTreeData` _output_get)) (`KismetMathLibrary.SelectInt` _value 0 _returnvalue)))
  (if (>= (- (`/Game/Core/GI_Persistence.Gold` (`/Game/Core/BFL_General.GetGameInst`)) _output) 0)
    (`BlueprintMapLibrary.Map_Add` _bloodmageunlockedattacks (`local.AttackToBuy`) (+ (`BlueprintMapLibrary.Map_Find` _bloodmageunlockedattacks (`local.AttackToBuy`)) 1))
    (`/Game/Core/GI_Persistence.ManagePartyGold` (`/Game/Core/BFL_General.GetGameInst`) _output true)
    (`KismetSystemLibrary.PrintText` "We brought an attack :)")
    (`self.BroughtAttack` (`local.AttackToBuy`))
    (return true)
    (else
      (`KismetSystemLibrary.PrintText` "Sry we dont give credit " true true (struct :`R` 1.0 :`B` 0.059374 :`A` 1.0) 10.0)
      (return false))))

(fn `UserConstructionScript`)