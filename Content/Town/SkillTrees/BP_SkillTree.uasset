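; BP_SkillTree is a skill tree Blueprint in the Town area that resolves an attack into its full data set.
; ConvertSkillTreeToAttackData passes the requested attack to three lookups for attack data, related skill tree data and asset data.
; It stores each result in a local variable and returns all three together.
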(fn `Convert Skill Tree to Attack Data`
  (params (AttackToFind :type "/Game/Chars/Attacks/Enums/AttackList Enum" :default "NewEnumerator1"))
  (returns (AttackData :type "/Game/Chars/Attacks/AttackData Structure") (AttackSkillTreeData :type "/Game/Chars/Attacks/AttackSkillTreeData Structure") (AttackAssets :type "/Game/Chars/Attacks/AttackAssetsData Structure"))
  (locals (LocAttackData :type "/Game/Chars/Attacks/AttackData Structure") (LocAttackSkillData :type "/Game/Chars/Attacks/AttackSkillTreeData Structure") (LocAttackAssets :type "/Game/Chars/Attacks/AttackAssetsData Structure"))
  (bind _attackdata (`/Game/Chars/Attacks/BFL_Attacks.getAttackDataFormAttack` AttackToFind))
  (set `local.LocAttackData` _attackdata)
  (bind _relatedattackskilltree (`/Game/Chars/Attacks/BFL_Attacks.GetAttackSkillDataFromAttack` (`local.AttackToFind`)))
  (set `local.LocAttackSkillData` _relatedattackskilltree)
  (bind _attackassetdata (`/Game/Chars/Attacks/BFL_Attacks.GetAttackAssetDataFormAttack` (`local.AttackToFind`)))
  (set `local.LocAttackAssets` _attackassetdata)
  (return (`local.LocAttackData`) (`local.LocAttackSkillData`) (`local.LocAttackAssets`)))