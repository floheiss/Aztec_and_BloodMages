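; Town guild interactable that opens a contract selection menu while no contract is set.
; On interact it fills and shuffles a contract list, picking difficulty per slot from overall party strength, then passes it to W_Guild.
; Contracts get random rewards, map info and text from DataTables keyed by composed row names, with a debug fallback description.
; Type is currently fixed to Boss in Woods, and stored difficulty and reward tier to Common.
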(event `/Game/Core/IN_Interact.InteractWith`
  (if (and (`self.CheckIfMenuOpen`) (== (`/Game/Core/GI_Persistence.ContractSet` (`/Game/Core/BFL_General.GetGameInst`)) false))
    (if (not (>= (`KismetArrayLibrary.Array_Length` (`self.Contracts`)) (`self.MaxContractAmount`)))
      (for _index (range (+ (`self.MaxContractAmount`) 1))
        (bind _diff (`self.SelectDiffForContract` _index))
        (`KismetArrayLibrary.Array_Add` (`self.Contracts`) (`self.Create Contract` _diff)))
      (`KismetArrayLibrary.Array_Shuffle` (`self.Contracts`)))
    (bind _returnvalue (`|CreateWidget` "/Game/Town/Guild/Assests_Guild/HUD/W_Guild.W_Guild_C" null (`self.Contracts`)))
    (`Widget.SetFocus` _returnvalue)
    (`self.ChanceMenu` _returnvalue "NewEnumerator7")))

(fn `Create Contract`
  (params (Diff :type "/Game/Core/GeneralEnums/TierList Enum" :default "NewEnumerator0"))
  (returns (ExtContract :type "/Game/Town/Guild/Contract_Data Structure (by ref)"))
  (locals (NewContract :type "/Game/Town/Guild/Contract_Data Structure"))
  (bind (_contract_type _maptype _extrainfo) (`self.CreateContractType` (`local.Diff`)))
  (bind (_title _describtion) (`self.CreateContractText` (`local.Diff`) _contract_type _maptype))
  (setmembers `/Game/Town/Guild/Contract_Data` :`StructRef` (`local.NewContract`) :`difficulty` "NewEnumerator0")
  (setmembers `/Game/Town/Guild/Contract_Data` :`StructRef` (`local.NewContract`) :`Reward` (+ (`KismetMathLibrary.RandomIntegerInRange` 30 70) (select `/Game/Core/GeneralEnums/TierList` "NewEnumerator0" :`NewEnumerator0` 100 :`NewEnumerator1` 170 :`NewEnumerator2` 250 :`NewEnumerator3` 330 :`NewEnumerator4` 1000)))
  (setmembers `/Game/Town/Guild/Contract_Data` :`StructRef` (`local.NewContract`) :`MapType` _maptype :`ContractTypeExtraInfo` _extrainfo :`ContractType` _contract_type)
  (setmembers `/Game/Town/Guild/Contract_Data` :`StructRef` (`local.NewContract`) :`MapInfo` (`self.CreateMapInfo` (`local.Diff`) _contract_type))
  (bind _structout (setmembers `/Game/Town/Guild/Contract_Data` :`StructRef` (`local.NewContract`) :`DescriptionTitle` _title :`DescriptionMission` _describtion :`MapMaxLvL` 6))
  (return _structout))

(fn `CreateContractText`
  (params (Diff :type "/Game/Core/GeneralEnums/TierList Enum" :default "NewEnumerator0") (ContractType :type "/Game/Town/Guild/Contract_Types Enum" :default "NewEnumerator0") (MapType :type "/Game/Town/Guild/Contract_Map_Types Enum" :default "NewEnumerator0"))
  (returns (Title :type Text) (Describtion :type Text))
  (locals (LocTitle :type Text :default "NSLOCTEXT(\"\", \"AE12D00E4902E2F29B4C6B84FC053D71\", \"Filler Title\")") (LocDescrib :type Text :default "NSLOCTEXT(\"\", \"94C6770545E62C31A8A1BFBA691E2081\", \"Filler Describtion\")") (LocDataTableRow :type Text))
  (if (`|EnumInequality` Diff "NewEnumerator4")
    ;[1 1 1] Normal contract no story or ability
    (bind _output_get (set `local.LocDataTableRow` (`|FormatText` "{ContractType}{MapType}{Difficculty}" (select `/Game/Town/Guild/Contract_Types` (`local.ContractType`) :`NewEnumerator0` "1" :`NewEnumerator1` "2" :`NewEnumerator2` "3" :`NewEnumerator4` "4") (select `/Game/Town/Guild/Contract_Map_Types` (`local.MapType`) :`NewEnumerator0` "1") (select `/Game/Core/GeneralEnums/TierList` (`local.Diff`) :`NewEnumerator0` "1" :`NewEnumerator1` "1" :`NewEnumerator2` "2" :`NewEnumerator3` "3" :`NewEnumerator5` "4" :`NewEnumerator6` "5"))))
    (bind _returnvalue (`|GetDataTableRow` "/Game/Town/Guild/DT_ContractDescribtion.DT_ContractDescribtion" (`KismetStringLibrary.Conv_StringToName` (`KismetTextLibrary.Conv_TextToString` _output_get)))
      (:`then`
        (bind ((`titleContract_9_13E4538E4024CA7658E16991DE74D9F0` _titlecontract) (`describtionContract_10_BB11FB814AC16AA506C8D5908652A3F3` _describtioncontract)) (break `/Game/Town/Guild/ContractDescribtion_Data` _returnvalue))
        (set `local.LocTitle` _titlecontract)
        (set `local.LocDescrib` _describtioncontract))
      (:`RowNotFound`
        (bind _returnvalue_2 (`|GetDataTableRow` "/Game/Town/Guild/DT_ContractDescribtion.DT_ContractDescribtion" "000")
          (:`then`
            (set `local.LocTitle` (`.titleContract_9_13E4538E4024CA7658E16991DE74D9F0` (break `/Game/Town/Guild/ContractDescribtion_Data` _returnvalue_2)))
            (set `local.LocDescrib` (`|FormatText` "Diff: {Diff}, ContractType: {ContractType}, MapType: {MapType} -> {Line checked}" (`|GetEnumeratorNameAsString` (`local.Diff`)) (`|GetEnumeratorNameAsString` (`local.ContractType`)) (`|GetEnumeratorNameAsString` (`local.MapType`)) (`local.LocDataTableRow`)))))))
    (return (`local.LocTitle`) (`local.LocDescrib`))))

(fn `CreateContractType`
  (params (Diff :type "/Game/Core/GeneralEnums/TierList Enum" :default "NewEnumerator0"))
  (returns (`Contract Type` :type "/Game/Town/Guild/Contract_Types Enum") (MapType :type "/Game/Town/Guild/Contract_Map_Types Enum") (ExtraInfo :type Integer))
  (locals (locContractType :type "/Game/Town/Guild/Contract_Types Enum" :default "NewEnumerator0") (LocMapType :type "/Game/Town/Guild/Contract_Map_Types Enum" :default "NewEnumerator0") (LocExtraInfo :type Integer :default 0))
  ;[1 1 1] have to look at the other kinds of contract (for now only boss is done)(Diff is used later for extra info things)
  (set `local.locContractType` "NewEnumerator0")
  (switch `/Game/Town/Guild/Contract_Types` (`local.locContractType`)
    (:`NewEnumerator0`
      (set `local.LocMapType` "NewEnumerator0")
      (return (`local.locContractType`) (`local.LocMapType`) (`local.LocExtraInfo`)))))

(fn `CreateMapInfo`
  (params (Diff :type "/Game/Core/GeneralEnums/TierList Enum" :default "NewEnumerator0") (ContractType :type "/Game/Town/Guild/Contract_Types Enum" :default "NewEnumerator0"))
  (returns (MapInfo :type "/Game/Town/Guild/MapInfo_Data Structure"))
  (locals (LocMapInfo :type "/Game/Town/Guild/MapInfo_Data Structure") (NewLocalVar :type "/Game/Town/Guild/MapInfo_Data Structure"))
  (bind _result (`|FormatText` "{Difficulty}{ContractType}" (select `/Game/Core/GeneralEnums/TierList` (`local.Diff`) :`NewEnumerator0` "1" :`NewEnumerator1` "2" :`NewEnumerator2` "3" :`NewEnumerator3` "4") (select `/Game/Town/Guild/Contract_Types` (`local.ContractType`) :`NewEnumerator0` "1" :`NewEnumerator1` "2" :`NewEnumerator2` "3" :`NewEnumerator4` "4")))
  (if (`|EnumInequality` Diff "NewEnumerator4")
    ;[1 1 1] Pulls all the need data for a normal Contract Form DT (add random to Rows in Map)
    (bind _returnvalue (`|GetDataTableRow` "/Game/Town/Guild/DT_MapInfo.DT_MapInfo" (`KismetStringLibrary.Conv_StringToName` (`KismetTextLibrary.Conv_TextToString` _result)))
      (:`then`
        (bind _structout (setmembers `/Game/Town/Guild/MapInfo_Data` :`StructRef` _returnvalue :`PathsInMap` (+ (`.PathsInMap_39_BFC829DA406418556202E2BF692EDCE8` (break `/Game/Town/Guild/MapInfo_Data` _returnvalue)) (`KismetMathLibrary.RandomIntegerInRange` 0 1))))
        (return _structout))
      (:`RowNotFound`
        ;[1 1 1] DeBug
        (`KismetSystemLibrary.PrintString` (`KismetTextLibrary.Conv_TextToString` (`|FormatText` "Error cant find the line in DT (MapInfo + {Line})" _result)))))))

(fn `HoverOver`
  (returns (Message :type Text))
  (if (`self.CheckIfMenuOpen`)
    (if (== (`/Game/Core/GI_Persistence.ContractSet` (`/Game/Core/BFL_General.GetGameInst`)) false)
      (return (`self.MenuName`))
      (else
        (return "Contract is already selected ")))))

(fn `SelectDiffForContract`
  (params (Index :type Integer))
  (returns (Diff :type "/Game/Core/GeneralEnums/TierList Enum"))
  (locals (locDiff :type "/Game/Core/GeneralEnums/TierList Enum"))
  (bind _returnvalue (`KismetMathLibrary.Conv_ByteToInt` (`/Game/Core/GI_Persistence.PartyOverallStrength` (`/Game/Core/BFL_General.GetGameInst`))))
  (switch `/Game/Core/GeneralEnums/TierList` (`/Game/Core/GI_Persistence.PartyOverallStrength` (`/Game/Core/BFL_General.GetGameInst`))
    (:`NewEnumerator0`
      ;[1 1 1] Generates ontract >Diff for common - epic
      (switch `int` (`local.Index`) :!label _label
        (:`0`
          (set `local.locDiff` (`/Game/Core/GI_Persistence.PartyOverallStrength` (`/Game/Core/BFL_General.GetGameInst`)) :!label _label_2))
        (:`1`
          (goto _label_2))
        (:`2`
          (goto _label_2))
        (:`3`
          (goto _label_2))
        (:`4`
          (set `local.locDiff` "NewEnumerator0" :!label _label_3))
        (:`5`
          (if (`KismetMathLibrary.RandomBool`)
            (goto _label_3)
            (else
              (set `local.locDiff` (cast `/Game/Core/GeneralEnums/TierList` (+ (`/Game/Core/GI_Persistence.PartyOverallStrength` (`/Game/Core/BFL_General.GetGameInst`)) 1)) :!label _label_4))))
        (:`6`
          (goto _label_4))
        (:`7`
          (set `local.locDiff` (cast `/Game/Core/GeneralEnums/TierList` (`KismetMathLibrary.Conv_IntToByte` (`KismetMathLibrary.Clamp` _returnvalue 0 _returnvalue)))))))
    (:`NewEnumerator1`
      (goto _label))
    (:`NewEnumerator2`
      (goto _label))
    (:`NewEnumerator3`
      (switch `int` (`local.Index`)
        (:`0`
          (set `local.locDiff` "NewEnumerator2" :!label _label_5))
        (:`1`
          (goto _label_5))
        (:`2`
          (goto _label_5))
        (:`3`
          (goto _label_5))
        (:`4`
          (set `local.locDiff` "NewEnumerator3" :!label _label_6))
        (:`5`
          (goto _label_6))
        (:`6`
          (set `local.locDiff` "NewEnumerator5"))
        (:`7`
          (set `local.locDiff` "NewEnumerator4"))))
    (:`NewEnumerator5`
      (switch `int` (`local.Index`)
        (:`0`
          (set `local.locDiff` "NewEnumerator2" :!label _label_7))
        (:`1`
          (goto _label_7))
        (:`2`
          (set `local.locDiff` "NewEnumerator3" :!label _label_8))
        (:`3`
          (goto _label_8))
        (:`4`
          (set `local.locDiff` "NewEnumerator5" :!label _label_9))
        (:`5`
          (goto _label_9))
        (:`6`
          (set `local.locDiff` "NewEnumerator6"))
        (:`7`
          (set `local.locDiff` "NewEnumerator4"))))
    (:`NewEnumerator6`
      (switch `int` (`local.Index`)
        (:`0`
          (set `local.locDiff` "NewEnumerator3" :!label _label_10))
        (:`1`
          (goto _label_10))
        (:`2`
          (set `local.locDiff` "NewEnumerator5" :!label _label_11))
        (:`3`
          (goto _label_11))
        (:`4`
          (goto _label_11))
        (:`5`
          (set `local.locDiff` "NewEnumerator6" :!label _label_12))
        (:`6`
          (goto _label_12))
        (:`7`
          (set `local.locDiff` "NewEnumerator4")))))
  (return (`local.locDiff`)))

(fn `UserConstructionScript`
  (`parent.UserConstructionScript`))