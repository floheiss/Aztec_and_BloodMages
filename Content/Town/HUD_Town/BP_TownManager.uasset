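; BP_TownManager manages the town HUD, creating the W_Town widget and exposing control over it.
; DisplayTown creates and stores the widget, then passes it to player controller 0 through SetDisplayedHUDMessage.
; SetTownActiveWidget forwards an index to that widget to switch its active view.
; Simple getters and setters hold the CanSwapWidget and CantSwapText values for access by other code.
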(event `DisplayTown`
  (bind _returnvalue (`|CreateWidget` "/Game/Town/HUD_Town/W_Town.W_Town_C"))
  (set `self.TownWidget` _returnvalue)
  (message `/Game/Core/IN_UniversalController.SetDisplayedHUD` (`GameplayStatics.GetPlayerController` 0) (`self.TownWidget`)))

(fn `GetCanSwap`
  (returns (CanSwapWidget :type Boolean))
  (return (`self.CanSwapWidget`)))

(fn `GetCantSwapText`
  (returns (CantSwapText :type Text))
  (return (`self.CantSwapText`)))

(fn `SetCanSwap`
  (params (CanSwapWidget :type Boolean))
  (set `self.CanSwapWidget` CanSwapWidget))

(fn `SetCantSwapText`
  (params (CantSwapText :type Text))
  (set `self.CantSwapText` CantSwapText))

(fn `SetTownActiveWidget`
  (params (WidgeIndex :type Integer))
  (`/Game/Town/HUD_Town/W_Town.SetActiveWidget` (`self.TownWidget`) WidgeIndex))

(fn `UserConstructionScript`)