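; BP_StartContract is an interactable town actor that sends the player to the contract room once a contract is set.
; It begins with its model and sprite hidden and collision disabled.
; A game instance event, bound on BeginPlay, toggles visibility and collision with the contract state.
; Interacting rechecks that state, calls the game instance's teleport, then looks up BP_ContractManager without using the result.
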(event `self.ReceiveBeginPlay`
  (add `/Game/Core/GI_Persistence.ContractWasSet` (`/Game/Core/BFL_General.GetGameInst`) (delegate `SetVisibility`))
  (`SceneComponent.SetVisibility` (`self.3dModel`) false false)
  (`SceneComponent.SetVisibility` (`self.Sprite`) false false)
  (`PrimitiveComponent.SetCollisionEnabled` (`self.CollisionR`) "NoCollision"))

(event `SetVisibility`
  (params (ContractSet :type Boolean))
  (`SceneComponent.SetVisibility` (`self.3dModel`) ContractSet false)
  (`SceneComponent.SetVisibility` (`self.Sprite`) ContractSet false)
  (`SceneComponent.SetVisibility` (`self.CollisionR`) ContractSet false)
  (`PrimitiveComponent.SetCollisionEnabled` (`self.CollisionR`) (select `bool` ContractSet :`false` "NoCollision" :`true` "QueryAndPhysics" :!type "ECollisionEnabled Enum")))

(event `/Game/Core/IN_Interact.InteractWith`
  (if (`/Game/Core/GI_Persistence.ContractSet` (`/Game/Core/BFL_General.GetGameInst`))
    (`/Game/Core/GI_Persistence.Teleport To ContractRoom` (`/Game/Core/BFL_General.GetGameInst`))
    (`GameplayStatics.GetActorOfClass` "/Game/Contract/BP_ContractManager.BP_ContractManager_C")))

(fn `UserConstructionScript`
  (`parent.UserConstructionScript`))