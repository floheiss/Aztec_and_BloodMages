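; BP_MapEditor is a map editor Blueprint whose W_TABS_MapEditor HUD is meant to show only in debug mode.
; Its DeBugModeUpdate event removes the HUD from the viewport, then re-adds it if debug mode is active.
; The setup that creates the HUD and binds that event to the game instance is disconnected, and BeginPlay is empty, so the file never initializes the editor.
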(event `self.ReceiveBeginPlay`)

(event `DeBugModeUpdate`
  (params (DeBugModeActive :type Boolean))
  (bind _mapeditorhud (`self.MapEditorHUD`))
  (`Widget.RemoveFromParent` _mapeditorhud)
  (if DeBugModeActive
    (`UserWidget.AddToViewport` _mapeditorhud 0)))

(fn `UserConstructionScript`)