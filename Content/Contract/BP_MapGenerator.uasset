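; Generates branching contract maps of typed nodes (enemies, elites, questions, campfires) for display.
; GenerateMap spawns a BP_MapGrid, walks one path per row along the map length, then tallies node types alongside contract info from the game instance.
; Path nodes link back to their predecessor, with types rolled through cascading percentage checks.
; Helpers build a basic map from length and column count, and copy story maps into display data.
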(fn `Convert Story Map Into Display Map`
  (params (StoryMap :type "/Game/Contract/MapEditor/StoryMapSave Structure"))
  (returns (DisplayMap :type "/Game/Contract/MapEditor/StoryMapSave Structure"))
  (locals (LocDisplayMap :type "/Game/Contract/MapEditor/StoryMapSave Structure"))
  (bind (_length _numberineachcolumns _2darraygrid _contracttype _contracttypeextrainfo) (break `/Game/Contract/MapEditor/StoryMapSave` StoryMap))
  (setmembers `/Game/Contract/MapEditor/StoryMapSave` :`StructRef` (`local.LocDisplayMap`) :`Length` _length :`NumberInEachColumns` _numberineachcolumns :`2DArrayGrid` _2darraygrid :`ContractType` _contracttype :`ContractTypeExtraInfo` _contracttypeextrainfo)
  (return (`local.LocDisplayMap`)))

(fn `Generate Random Note Type`
  (returns (ReturnValue :type "/Game/Contract/MapStructs/MapNoteTypes Enum"))
  (bind (_elite _campfire _question) (break `/Game/Town/Guild/ProbabilitiesOfTierInMap_Data` (`.ProbabilitieOfTier_34_C9A086E747EB0AD8D14B848BCD11A5E6` (break `/Game/Town/Guild/MapInfo_Data` (`self.MapInfo`)))))
  (return (select `bool` (`/Game/Core/BFL_General.CheckAgainstRandom100` _elite) :`false` (select `bool` (`/Game/Core/BFL_General.CheckAgainstRandom100` _campfire) :`false` (select `bool` (`/Game/Core/BFL_General.CheckAgainstRandom100` _question) :`false` "NewEnumerator0" :`true` "NewEnumerator1" :!type "/Game/Contract/MapStructs/MapNoteTypes Enum") :`true` "NewEnumerator2") :`true` "NewEnumerator3")))

(fn `GenerateBasicMap`
  (params (Length :type Integer) (NumberInColumn :type Integer))
  (returns (GeneratedMap :type "/Game/Contract/MapStructs/MapForDisplay_Data Structure"))
  (locals (LocMapInfo :type "/Game/Town/Guild/MapInfo_Data Structure"))
  (bind _minmaxmapinfo_data (make `/Game/Town/Guild/MinMaxMapInfo_Data` 0))
  (setmembers `/Game/Town/Guild/MapInfo_Data` :`StructRef` (`local.LocMapInfo`) :`mapLength` Length :`PathsInMap` NumberInColumn)
  (setmembers `/Game/Town/Guild/MapInfo_Data` :`StructRef` (`local.LocMapInfo`) :`MinMaxNormalEnemies` (make `/Game/Town/Guild/MinMaxMapInfo_Data` 0 1000) :`MinMaxQuestion` _minmaxmapinfo_data :`MinMaxCampfire` _minmaxmapinfo_data :`MinMaxElits` _minmaxmapinfo_data)
  (bind _generatedmap (`self.GenerateMap` (`local.LocMapInfo`)))
  (return _generatedmap))

(fn `GenerateMap`
  (params (MapInfoToGen :type "/Game/Town/Guild/MapInfo_Data Structure"))
  (returns (GeneratedMap :type "/Game/Contract/MapStructs/MapForDisplay_Data Structure"))
  (locals (LocMapForDisplay :type "/Game/Contract/MapStructs/MapForDisplay_Data Structure") (NumberInColumns :type "Array of Integer"))
  (bind ((`mapLength_18_97A61A884D961775F9EB69A62A7AEC35` _maplength) (`PathsInMap_39_BFC829DA406418556202E2BF692EDCE8` _pathsinmap)) (break `/Game/Town/Guild/MapInfo_Data` (`self.MapInfo`)))
  (bind ((`ContractTypeExtraInfo_30_5FD7F79445A8A9C31C7BF1B4BBF906BE` _contracttypeextrainfo) (`ContractType_26_58802503459D3560F334A99AC3C80FDF` _contracttype)) (break `/Game/Town/Guild/Contract_Data` (`/Game/Core/GI_Persistence.Contract ` (`/Game/Core/BFL_General.GetGameInst`))))
  ;[1 1 1] Sets length + contract type + extra info
  (set `self.MapInfo` MapInfoToGen)
  (setmembers `/Game/Contract/MapStructs/MapForDisplay_Data` :`StructRef` (`local.LocMapForDisplay`) :`Length` _maplength :`Rows` _pathsinmap :`ContractType` _contracttype :`ContractTypeExtraInfo` _contracttypeextrainfo)
  ;[1 1 1] Spawns an sets the MapGrid (is the array)
  (bind _returnvalue (`|SpawnActorFromClass` :`Class` "/Game/Contract/BP_MapGrid.BP_MapGrid_C" :`SpawnTransform` (`KismetMathLibrary.MakeTransform` (-999.0 -999.0 -999.0)) :`CollisionHandlingOverride` "Undefined" :`TransformScaleMethod` "MultiplyWithRoot" :`Instigator` null))
  (set `self.MapGrid` _returnvalue)
  (for _index (range (`.PathsInMap_39_BFC829DA406418556202E2BF692EDCE8` (break `/Game/Town/Guild/MapInfo_Data` (`self.MapInfo`))))
    (`self.GeneratePathInMap` _index))
  (setmembers `/Game/Contract/MapStructs/MapForDisplay_Data` :`StructRef` (`local.LocMapForDisplay`) :`2DGrid` (`/Game/Contract/BP_MapGrid.InternalArray` (`self.MapGrid`)))
  ;[1 1 1] fills the numberOf.. in the List is used to generate mission that arnt boss
  (for _array_element (`/Game/Contract/BP_MapGrid.InternalArray` (`self.MapGrid`))
    (bind (_positionin2darray_x _positionin2darray_y) (break `/Game/Contract/MapStructs/2DArrayPosition_Data` (break `/Game/Contract/MapStructs/MapNote_Data` _array_element)))
    (switch `/Game/Contract/MapStructs/MapNoteTypes` (`.TypeOfNote_29_44166E4E4FC6DD1739E5DA9462B38D2E` (break `/Game/Contract/MapStructs/MapNote_Data` (`/Game/Contract/BP_MapGrid.GetElement2D` (`self.MapGrid`) _positionin2darray_x _positionin2darray_y)))
      (:`NewEnumerator0`
        (`/Engine/EditorBlueprintResources/StandardMacros.IncrementInt` (`.NumberOfNormalEnemies_14_3DC6D06B4ABD1EF29533BEA3B4D9176E` (break `/Game/Contract/MapStructs/MapForDisplay_Data` (`local.LocMapForDisplay`)))))
      (:`NewEnumerator1`
        (`/Engine/EditorBlueprintResources/StandardMacros.IncrementInt` (`.NumberOfQuestion_12_FB8C42584B9BACCB2A7DA787642FE94E` (break `/Game/Contract/MapStructs/MapForDisplay_Data` (`local.LocMapForDisplay`)))))
      (:`NewEnumerator2`
        (`/Engine/EditorBlueprintResources/StandardMacros.IncrementInt` (`.NumberOfCampfires_10_0DE21AFD4BD9034B55109989A15C1F9E` (break `/Game/Contract/MapStructs/MapForDisplay_Data` (`local.LocMapForDisplay`)))))
      (:`NewEnumerator3`
        (`/Engine/EditorBlueprintResources/StandardMacros.IncrementInt` (`.NumberOfElits_9_C557B08A486408B1A106DA84257DBD1A` (break `/Game/Contract/MapStructs/MapForDisplay_Data` (`local.LocMapForDisplay`)))))
      (:`NewEnumerator6`
        (`/Engine/EditorBlueprintResources/StandardMacros.IncrementInt` (`.NumberOfElits_9_C557B08A486408B1A106DA84257DBD1A` (break `/Game/Contract/MapStructs/MapForDisplay_Data` (`local.LocMapForDisplay`)))))))
  (bind _structout (setmembers `/Game/Contract/MapStructs/MapForDisplay_Data` :`StructRef` (`local.LocMapForDisplay`) :`2DGrid` (`/Game/Contract/BP_MapGrid.InternalArray` (`self.MapGrid`))))
  (return _structout))

(fn `GeneratePathInMap`
  (params (StartingIndex :type Integer))
  (locals (LocCurrentIndexX :type Integer) (LocCurrentIndexY :type Integer) (LocLastIndexX :type Integer) (LocLastIndexY :type Integer) (LocPathForNote :type "Array of /Game/Contract/MapStructs/2DArrayPosition_Data Structure") (LocPathFull :type "Array of /Game/Contract/MapStructs/2DArrayPosition_Data Structure"))
  (bind _2darrayposition_data (make `/Game/Contract/MapStructs/2DArrayPosition_Data` (`local.LocLastIndexX`) (`local.LocLastIndexY`)))
  (bind _returnvalue (`KismetMathLibrary.Clamp` (+ (`local.LocCurrentIndexY`) (`KismetMathLibrary.RandomIntegerInRange` -1 1)) 0 (+ (`.PathsInMap_39_BFC829DA406418556202E2BF692EDCE8` (break `/Game/Town/Guild/MapInfo_Data` (`self.MapInfo`))) 1)))
  ;[1 1 1] is used to generate the first note in the path
  (bind _output_get (set `local.LocCurrentIndexX` 0))
  (bind _output_get_2 (set `local.LocCurrentIndexY` (`local.StartingIndex`)))
  (bind _structout (setmembers `/Game/Contract/MapStructs/MapNote_Data` :`StructRef` (`/Game/Contract/BP_MapGrid.GetElement2D` (`self.MapGrid`) _output_get _output_get_2) :`PositionIn2DArray` (make `/Game/Contract/MapStructs/2DArrayPosition_Data` (`local.LocCurrentIndexX`) (`local.LocCurrentIndexY`)) :`TypeOfNote` "NewEnumerator0" :`Locked` false :`IsInAnyPath` true))
  (`/Game/Contract/BP_MapGrid.Add Out Of Grid Notes` (`self.MapGrid`) _structout)
  (for _index (range 1 (`.mapLength_18_97A61A884D961775F9EB69A62A7AEC35` (break `/Game/Town/Guild/MapInfo_Data` (`self.MapInfo`))))
    ;[1 1 1] sets old indexs for setting in connections
    (set `local.LocLastIndexX` (`local.LocCurrentIndexX`))
    (set `local.LocLastIndexY` (`local.LocCurrentIndexY`))
    (bind _output_get_3 (set `local.LocCurrentIndexX` _index))
    (set `local.LocCurrentIndexY` _returnvalue)
    (bind _output_get_4 (set `local.LocPathForNote` (`|MakeArray` _2darrayposition_data)))
    (bind _noteatindex (`/Game/Contract/BP_MapGrid.GetElement2D` (`self.MapGrid`) _output_get_3 _returnvalue))
    (`KismetArrayLibrary.Array_Append` _output_get_4 (`.Connections_38_3AA328AE439A0A46F0F09F9AEAA74CBB` (break `/Game/Contract/MapStructs/MapNote_Data` _noteatindex)))
    (bind _structout_2 (setmembers `/Game/Contract/MapStructs/MapNote_Data` :`StructRef` _noteatindex :`PositionIn2DArray` (make `/Game/Contract/MapStructs/2DArrayPosition_Data` (`local.LocCurrentIndexX`) (`local.LocCurrentIndexY`)) :`TypeOfNote` (`self.Generate Random Note Type`) :`Locked` true :`Connections` (`local.LocPathForNote`) :`IsInAnyPath` true))
    (`/Game/Contract/BP_MapGrid.Add Out Of Grid Notes` (`self.MapGrid`) _structout_2)
    (`KismetArrayLibrary.Array_Add` (`local.LocPathFull`) _2darrayposition_data))
  (for _ (`local.LocPathFull`)
    _))

(fn `UserConstructionScript`)