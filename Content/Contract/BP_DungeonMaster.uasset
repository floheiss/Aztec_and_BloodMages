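; BP_DungeonMaster builds contract combat encounters and calculates their loot.
; SetUpCombat spends a heat budget from party size, difficulty and randomness on shuffled DT_EnemyGen rows, spawns AI units and hands them to the game instance.
; GenerateLoot rolls rank-weighted, partly seeded drops from defeated enemies, plus experience and gold, though the gold result is never stored.
; Helpers buff enemy stats and compute map-node heat; boss and fallback generation are empty stubs.
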(fn ConstructionScript)

(fn SetUpCombat
  (params (NoteType :type MapNoteTypes%20Enum :default "NewEnumerator0") (IsAmbush :type Boolean))
  (bind _out (CallFunction|GetGameInst))
  (bind _contract_ (Variables|/Game/Core/GI_Persistence.GI_Persistence_C|GetContract%20 _out))
  (bind (_difficulty _contracttype) (Utilities|Struct|BreakContract_Data _contract_))
  (bind _enemeis (Combat|GenerateEnemies _difficulty NoteType _contracttype IsAmbush))
  (Default|SetEnemies (CallFunction|GetGameInst) _enemeis)
  (Default|SetControllerMode (CallFunction|GetGameInst) "NewEnumerator1"))

(fn GenerateEnemies
  (params (Diff :type TierList%20Enum :default "NewEnumerator0") (NoteType :type MapNoteTypes%20Enum :default "NewEnumerator0") (ContractType :type Contract_Types%20Enum :default "NewEnumerator0") (IsAmbush :type Boolean))
  (switch Utilities|FlowControl|Switch|SwitchonMapNoteTypes NoteType
    (:NewEnumerator0
      (bind _maxheat (Combat|CalculateHeat Diff IsAmbush))
      (LocalVariables|SetLocHeat _maxheat)
      (Utilities|FlowControl|Sequence
        (:then_0
          (Utilities|FlowControl|ForLoopwithBreak 0 100 :!label _label
            (:LoopBody
              (if (and (> (LocalVariables|GetLocHeat) (LocalVariables|GetLocMinimumHeatToGenEnemies)) (<= (Utilities|Array|Length (LocalVariables|GetLocEnemies)) 5))
                (bind (_enemy _heatusedup) (Combat|GenerateBaseEnemy (LocalVariables|GetLocHeat) IsAmbush))
                (Utilities|Array|Add (LocalVariables|GetLocEnemies) _enemy)
                (LocalVariables|SetLocHeat (- (LocalVariables|GetLocHeat) _heatusedup))
                (Math|Integer|IncrementInt (LocalVariables|GetLocFailSaveCounter))
                (else
                  ;[1 1 1] fail save if something is wrong
                  (if (> (LocalVariables|GetLocFailSaveCounter) 20)
                    (bind _fallsaveenemies (Combat|FalseSaveEnemyGen))
                    (LocalVariables|SetLocEnemies _fallsaveenemies)
                    (goto _label Break)
                    (else
                      (goto _label Break))))))))
        (:then_1
          (return (LocalVariables|GetLocEnemies)))))
    (:NewEnumerator5
      (bind _bossenemies (Combat|GenerateBoss))
      (return _bossenemies))))

(fn GenerateBoss
  (return 0))

(fn BuffEnemy
  (params (Enemy :type PZD%20Unit%20Object%20Reference))
  (LocalVariables|SetLocEnemy Enemy)
  (bind _pull (|GetRandomPull_2))
  (LocalVariables|SetLocPull _pull)
  (Default|SetONEUnitStat Enemy (Math|Float|Truncate (* (Default|GetUnitStat Enemy (LocalVariables|GetLocPull)) (.Value (Utilities|Map|Find (LocalVariables|GetLocAvaliableStatsToNer) (LocalVariables|GetLocPull))))) false (LocalVariables|GetLocPull))
  (if (Math|Random|RandomBoolwithWeight 0.4)
    (bind _pull_2 (|GetRandomPull))
    (LocalVariables|SetLocPull_2 _pull_2)
    (while (Utilities|Enum|Equal(Enum) (LocalVariables|GetLocPull) (LocalVariables|GetLocPull_2))
      (bind _pull_3 (|GetRandomPull_3))
      (LocalVariables|SetLocPull_2 _pull_3))
    (Default|SetONEUnitStat Enemy (Math|Float|Truncate (* (Default|GetUnitStat Enemy (LocalVariables|GetLocPull)) (.Value (Utilities|Map|Find (LocalVariables|GetLocAvaliableStatsToNer) (LocalVariables|GetLocPull_2))))) false (LocalVariables|GetLocPull_2))))

(fn CalculateHeat
  (params (Diff :type TierList%20Enum :default "NewEnumerator0") (IsAmbush :type Boolean))
  ;[1 1 1] min Heat --> 1 merc = 1 heat
  (LocalVariables|SetLocHeat (+ (LocalVariables|GetLocHeat) (Utilities|Array|Length (Variables|/Game/Core/GI_Persistence.GI_Persistence_C|GetMercGroup%20 (CallFunction|GetGameInst))) 1.0))
  ;[1 1 1] adds heat for diff --> diff * 0.7 = diffHeat
  (LocalVariables|SetLocHeat (+ (LocalVariables|GetLocHeat) (* 0.7 (Math|Conversions|ToFloat(Byte) Diff))))
  ;[1 1 1] adds random heat --> (0.2*diff) to (0.4*diff+1)
  (LocalVariables|SetLocHeat (+ (LocalVariables|GetLocHeat) (Math|Random|RandomFloatinRange (* 0.4 (Math|Conversions|ToFloat(Byte) Diff)) (* 0.7 (+ (Math|Conversions|ToFloat(Byte) Diff) 1.0)))))
  (Development|PrintText (Utilities|Text|FormatText "The max heat: {h}" (LocalVariables|GetLocHeat)) true true "(R=0.000000,G=1.000000,B=0.065609,A=1.000000)" 2e+01)
  (return (LocalVariables|GetLocHeat)))

(fn GenerateBaseEnemy
  (params (ReaminingHeat :type Float%20%28double-precision%29) (IsAmbush :type Boolean))
  (bind _outrownames (DataTable|GetDataTableRowNames "/Game/Chars/DTsUnit/DT_EnemyGen.DT_EnemyGen"))
  (bind _output_get (LocalVariables|SetLocTableRows _outrownames))
  (Utilities|Array|Shuffle _output_get)
  (for _array_element (LocalVariables|GetLocTableRows)
    (bind _returnvalue (Utilities|GetDataTableRow "/Game/Chars/DTsUnit/DT_EnemyGen.DT_EnemyGen" _array_element)
      (:then
        (if (or (not IsAmbush) (== IsAmbush (.AvaliableInAmbush (Utilities|Struct|BreakEnemyGenData _returnvalue))))
          (if (<= (.HeatUsage (Utilities|Struct|BreakEnemyGenData _returnvalue)) ReaminingHeat)
            (bind _returnvalue_2 (Game|SpawnActorfromClass "/Game/Chars/PZD_Unit.PZD_Unit_C" (Math|Transform|MakeTransform "-9999.000000,-99.000000,-999.000000" "0, 0, 0" "1.000000,1.000000,1.000000") "AlwaysSpawn" "MultiplyWithRoot" 0 0))
            (bind _output_get_2 (LocalVariables|SetLocNewEnemy _returnvalue_2))
            (Variables|/Game/Chars/PZD_Unit.PZD_Unit_C|SetClass _output_get_2 (.Class (Utilities|Struct|BreakEnemyGenData _returnvalue)))
            (Variables|/Game/Chars/PZD_Unit.PZD_Unit_C|SetTeam _output_get_2 1)
            (Default|SetUpAI _output_get_2)
            (Default|GetBaseStats (LocalVariables|GetLocNewEnemy))
            (return (LocalVariables|GetLocNewEnemy) (.HeatUsage (Utilities|Struct|BreakEnemyGenData _returnvalue)))))))))

(fn FalseSaveEnemyGen
  (return 0))

(fn GenerateLoot
  (params (Rank :type TierList%20Enum :default "NewEnumerator0") (AllEnemies :type Array%20of%20PZD%20Unit%20Object%20References) (DefeatedEnemies :type Array%20of%20PZD%20Unit%20Object%20References))
  (bind _items (Loot|GenerateDrops Rank DefeatedEnemies))
  (LocalVariables|SetLocItems _items)
  (bind _exp (Loot|CalculateExp Rank AllEnemies))
  (LocalVariables|SetLocExp _exp)
  (Loot|CalculateGold Rank AllEnemies)
  (return (LocalVariables|GetLocItems) (LocalVariables|GetLocGold) (LocalVariables|GetLocExp)))

(fn GenerateDrops
  (params (Rank :type TierList%20Enum :default "NewEnumerator0") (DefeatedEnemies :type Array%20of%20PZD%20Unit%20Object%20References))
  (if (> (Utilities|Array|Length DefeatedEnemies) 0)
    (for _array_element DefeatedEnemies
      (bind _enemydrops (CallFunction|GetDatafromEnemyDrops (Variables|/Game/Chars/PZD_Unit.PZD_Unit_C|GetClass _array_element)))
      (for _index (range 0 (Loot|CalculateDropNumber Rank))
        (bind _raritytouse (CallFunction|GenerateRarityFormMap (Loot|GenRarityMap Rank)))
        (bind _droppeditem (Loot|GenEnemyDropfromRarity _raritytouse (Utilities|Struct|BreakEnemyDropData _enemydrops)))
        (Utilities|Array|Add (LocalVariables|GetLocItemList) _droppeditem)))
    (return (LocalVariables|GetLocItemList))
    (else
      (return (LocalVariables|GetLocItemList)))))

(fn CalculateExp
  (params (Rank :type TierList%20Enum :default "NewEnumerator0") (AllEnemies :type Array%20of%20PZD%20Unit%20Object%20References))
  (for _array_element AllEnemies
    (bind _enemydrops (CallFunction|GetDatafromEnemyDrops (Variables|/Game/Chars/PZD_Unit.PZD_Unit_C|GetClass _array_element)))
    (LocalVariables|SetLocExp (+ (LocalVariables|GetLocExp) (Math|Float|Truncate (* (Utilities|Struct|BreakEnemyDropData _enemydrops) (+ (Math|Float|MakeLiteralFloat 1.0) (* (Utilities|Select :Index Rank :NewEnumerator0 0 :NewEnumerator1 1 :NewEnumerator2 3 :NewEnumerator3 5 :NewEnumerator5 4 :NewEnumerator6 5 :NewEnumerator4 5) 0.1)))))))
  (return (LocalVariables|GetLocExp)))

(fn CalculateGold
  (params (Rank :type TierList%20Enum :default "NewEnumerator0") (AllEnemies :type Array%20of%20PZD%20Unit%20Object%20References))
  (for _array_element AllEnemies
    (bind _enemydrops (CallFunction|GetDatafromEnemyDrops (Variables|/Game/Chars/PZD_Unit.PZD_Unit_C|GetClass _array_element)))
    (LocalVariables|SetLocGoldDrop (+ (LocalVariables|GetLocGoldDrop) (Math|Integer|Clamp(Integer) (+ (.Gold (Utilities|Struct|BreakEnemyDropData _enemydrops)) (Math|Random|RandomIntegerinRange -5 10)) 0 (+ (.Gold (Utilities|Struct|BreakEnemyDropData _enemydrops)) (Math|Random|RandomIntegerinRange -5 10))))))
  (return (LocalVariables|GetLocGoldDrop)))

(fn GenRarityMap
  (params (Rank :type TierList%20Enum :default "NewEnumerator0"))
  (Utilities|Map|Add (LocalVariables|GetLocRarityMap) "NewEnumerator0" (Utilities|Select :Index Rank :NewEnumerator0 (Math|Float|MakeLiteralFloat 0.6) :NewEnumerator1 (Math|Float|MakeLiteralFloat 0.3) :NewEnumerator2 (Math|Float|MakeLiteralFloat 0.2) :NewEnumerator3 (Math|Float|MakeLiteralFloat 0.1) :NewEnumerator5 0.0 :NewEnumerator6 0.0 :NewEnumerator4 0.0))
  (Utilities|Map|Add (LocalVariables|GetLocRarityMap) "NewEnumerator1" (Utilities|Select :Index Rank :NewEnumerator0 (Math|Float|MakeLiteralFloat 0.25) :NewEnumerator1 (Math|Float|MakeLiteralFloat 0.5) :NewEnumerator2 (Math|Float|MakeLiteralFloat 0.3) :NewEnumerator3 (Math|Float|MakeLiteralFloat 0.2) :NewEnumerator5 0.0 :NewEnumerator6 0.0 :NewEnumerator4 0.0))
  (Utilities|Map|Add (LocalVariables|GetLocRarityMap) "NewEnumerator2" (Utilities|Select :Index Rank :NewEnumerator0 (Math|Float|MakeLiteralFloat 0.15) :NewEnumerator1 (Math|Float|MakeLiteralFloat 0.25) :NewEnumerator2 (Math|Float|MakeLiteralFloat 0.35) :NewEnumerator3 (Math|Float|MakeLiteralFloat 0.4) :NewEnumerator5 0.0 :NewEnumerator6 0.0 :NewEnumerator4 0.0))
  (Utilities|Map|Add (LocalVariables|GetLocRarityMap) "NewEnumerator3" (Utilities|Select :Index Rank :NewEnumerator0 (Math|Float|MakeLiteralFloat 0.05) :NewEnumerator1 (Math|Float|MakeLiteralFloat 0.15) :NewEnumerator2 (Math|Float|MakeLiteralFloat 0.15) :NewEnumerator3 (Math|Float|MakeLiteralFloat 0.25) :NewEnumerator5 0.0 :NewEnumerator6 0.0 :NewEnumerator4 0.0))
  (return (LocalVariables|GetLocRarityMap)))

(fn CalculateDropNumber
  (params (Rank :type TierList%20Enum :default "NewEnumerator0"))
  (return (+ (Math|Integer|SelectInt 1 0 (Class|KismetMathLibrary|RandomBoolwithWeightfromStream (Variables|/Game/Core/GI_Persistence.GI_Persistence_C|GetCurrentSeed (CallFunction|GetGameInst)) (Utilities|Select :Index Rank :NewEnumerator0 0.5 :NewEnumerator1 0.7 :NewEnumerator2 0.9 :NewEnumerator3 1.0 :NewEnumerator5 0.0 :NewEnumerator6 0.0 :NewEnumerator4 0.0))) (Math|Integer|SelectInt 1 0 (Class|KismetMathLibrary|RandomBoolwithWeightfromStream (Variables|/Game/Core/GI_Persistence.GI_Persistence_C|GetCurrentSeed (CallFunction|GetGameInst)) (Utilities|Select :Index Rank :NewEnumerator0 0.5 :NewEnumerator1 0.7 :NewEnumerator2 0.9 :NewEnumerator3 1.0 :NewEnumerator5 0.0 :NewEnumerator6 0.0 :NewEnumerator4 0.0))))))

(fn GenEnemyDropfromRarity
  (params (Tier :type TierList%20Enum :default "NewEnumerator0") (DropTabel :type Map%20of%20ItemList%20Enums%20to%20Bytes :default "NewEnumerator0"))
  (bind _values (Utilities|Map|Values DropTabel))
  (for (_array_element _array_index) _values
    (if (Utilities|Enum|Equal(Enum) _array_element Tier)
      (bind _keys (Utilities|Map|Keys DropTabel))
      (Utilities|Array|Add (LocalVariables|GetLocIndexOfItems) (Utilities|Array|Get(acopy) _keys _array_index))))
  (if (> (Utilities|Array|Length (LocalVariables|GetLocIndexOfItems)) 0)
    ;[1 1 1] drops item of matching Tier
    (return (.OutItem (Utilities|Array|Random (LocalVariables|GetLocIndexOfItems))))
    (else
      ;[1 1 1] Drops a random item for all avaliable when no matching
      (bind _keys_2 (Utilities|Map|Keys DropTabel))
      (return (.OutItem (Utilities|Array|Random _keys_2))))))

(fn GenerateHeatforMapNote
  (params (Difficulty :type TierList%20Enum :default "NewEnumerator0") (CurrentLvL :type Integer))
  (Utilities|FlowControl|Sequence
    (:then_0
      ;[1 1 1] min Heat --> 1 merc = 1 heat
      (LocalVariables|SetLocBaseHeatForNote (+ (LocalVariables|GetLocBaseHeatForNote) (Utilities|Array|Length (Variables|/Game/Core/GI_Persistence.GI_Persistence_C|GetMercGroup%20 (CallFunction|GetGameInst))) 1.0))
      ;[1 1 1] adds heat for diff --> diff * 0.7 = diffHeat
      (LocalVariables|SetLocBaseHeatForNote (+ (LocalVariables|GetLocBaseHeatForNote) (* 0.7 (Math|Conversions|ToFloat(Byte) Difficulty))))
      ;[1 1 1] adds random heat --> (0.2*diff) to (0.4*diff+1)
      (LocalVariables|SetLocBaseHeatForNote (+ (LocalVariables|GetLocBaseHeatForNote) (Math|Random|RandomFloatinRange (* 0.4 (Math|Conversions|ToFloat(Byte) Difficulty)) (* 0.7 (+ (Math|Conversions|ToFloat(Byte) Difficulty) 1.0)))))
      ;[0.15 0.15 0.15 0.5] Adds heat for each lvl
      (LocalVariables|SetLocBaseHeatForNote (+ (LocalVariables|GetLocBaseHeatForNote) 0.0)))
    (:then_1
      (for _index (range 0 2)
        (Utilities|Array|Add (LocalVariables|GetLocHeatArray) (|(BaseHeat+(((Diff+1)*HeatPerDiff)*Index)) (Math|Conversions|ToFloat(Byte) Difficulty) (Math|Conversions|ToFloat(Integer) _index) (LocalVariables|GetLocBaseHeatForNote) (LocalVariables|GetLocHeatPerDiff))))
      (return (LocalVariables|GetLocHeatArray)))))