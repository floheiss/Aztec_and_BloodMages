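; BP_MapGrid stores the Contract map as a grid of MapNote nodes, each with a type, lock state and connections.
; It emulates a 2D array with a flat InternalArray, finding entries by linear search on their stored X/Y position.
; Init fills it with locked placeholders, and helpers read or write cells, rows and columns.
; RemoveNote also prunes links to the removed node from both adjacent X columns.
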(event `self.ReceiveBeginPlay`
  (if (`/Game/Core/GI_Persistence.MapSet` (`/Game/Core/BFL_General.GetGameInst`))
    (`self.ReInit` (`self.InternalArray`))))

(fn `Add Empty Map Note`
  (params (X :type Integer) (Y :type Integer))
  (`KismetArrayLibrary.Array_Add` (`self.InternalArray`) (make `/Game/Contract/MapCore/MapNote_Data` (0.0 0.0 0.0) (make `/Game/Contract/MapCore/2DArrayPosition_Data` X Y) "NewEnumerator9" true)))

(fn `Add Out Of Grid Notes`
  (params (MapNote :type "/Game/Contract/MapCore/MapNote_Data Structure"))
  (returns (IndexOfNote :type Integer))
  (bind ((`PositionIn2DArray_33_7FF6CAD844866154E2D040A134BA7301` _positionin2darray)) (break `/Game/Contract/MapCore/MapNote_Data` (`local.MapNote`)))
  (bind (_noteatindex _noteindex _succ) (`self.GetElement2D` (break `/Game/Contract/MapCore/2DArrayPosition_Data` _positionin2darray) (`.Y_17_EE273A42468549352FD16DBB63F77F96` (break `/Game/Contract/MapCore/2DArrayPosition_Data` _positionin2darray))))
  (if _succ
    (`KismetArrayLibrary.Array_Insert` (`self.InternalArray`) (`local.MapNote`) _noteindex)
    (return _noteindex)
    (else
      (bind _returnvalue (`KismetArrayLibrary.Array_Add` (`self.InternalArray`) (`local.MapNote`)))
      (return _returnvalue))))

(fn `ChangeNoteToEmpty`
  (params (NoteToChange :type "/Game/Contract/MapCore/2DArrayPosition_Data Structure"))
  (bind (_x _y) (break `/Game/Contract/MapCore/2DArrayPosition_Data` NoteToChange))
  (setmembers `/Game/Contract/MapCore/MapNote_Data` :`StructRef` (`|GetArrayItem` (`self.InternalArray`) (`.NoteIndex` (`self.GetElement2D` _x _y))) :`TypeOfNote` "NewEnumerator6"))

(fn `Get All Elements Of Given XIndex`
  (params (XIndex :type Integer))
  (returns (AllNotesOfGivenXIndex :type "Map of Integer to /Game/Contract/MapCore/MapNote_Data Structure"))
  (locals (LocMap :type "Map of Integer to /Game/Contract/MapCore/MapNote_Data Structure"))
  (bind _tile_count_x (`KismetMathLibrary.BreakVector2D` (`self.Tile Count`)))
  (for _array_element (`self.InternalArray`)
    (bind ((`PositionIn2DArray_33_7FF6CAD844866154E2D040A134BA7301` _positionin2darray) (`TypeOfNote_29_44166E4E4FC6DD1739E5DA9462B38D2E` _typeofnote)) (break `/Game/Contract/MapCore/MapNote_Data` _array_element))
    (bind (_x _y) (break `/Game/Contract/MapCore/2DArrayPosition_Data` _positionin2darray))
    (if (and (== _x (`local.XIndex`)) (`|EnumInequality` _typeofnote "NewEnumerator9"))
      (`BlueprintMapLibrary.Map_Add` (`local.LocMap`) _y _array_element)
      (if (== (`BlueprintMapLibrary.Map_Length` (`local.LocMap`)) (`KismetMathLibrary.Round` _tile_count_x))
        (return (`local.LocMap`)))))
  (return (`local.LocMap`)))

(fn `Get All Elements Of Given YIndex`
  (params (YIndex :type Integer))
  (returns (AllNotesOfGivenYIndex :type "Map of Integer to /Game/Contract/MapCore/MapNote_Data Structure"))
  (locals (LocMap :type "Map of Integer to /Game/Contract/MapCore/MapNote_Data Structure"))
  (for _array_element (`self.InternalArray`)
    (bind (_x _y) (break `/Game/Contract/MapCore/2DArrayPosition_Data` (`.PositionIn2DArray_33_7FF6CAD844866154E2D040A134BA7301` (break `/Game/Contract/MapCore/MapNote_Data` _array_element))))
    (if (== _y (`local.YIndex`))
      (`BlueprintMapLibrary.Map_Add` (`local.LocMap`) _x _array_element)))
  (return (`local.LocMap`)))

(fn `GetElement2D`
  (params (XIndex :type Integer) (YIndex :type Integer))
  (returns (NoteAtIndex :type "/Game/Contract/MapCore/MapNote_Data Structure") (NoteIndex :type Integer) (Succ :type Boolean))
  (for (_array_element _array_index) (`self.InternalArray`)
    (bind (_x _y) (break `/Game/Contract/MapCore/2DArrayPosition_Data` (`.PositionIn2DArray_33_7FF6CAD844866154E2D040A134BA7301` (break `/Game/Contract/MapCore/MapNote_Data` _array_element))))
    (bind _returnvalue (and (== _x (`local.XIndex`)) (== _y (`local.YIndex`))))
    (if _returnvalue
      (return _array_element _array_index _returnvalue)))
  (return (struct) 0 false))

(fn `Init`
  (params (Size :type "Vector2D Structure"))
  (locals (yIndex :type Integer) (xIndex :type Integer))
  (bind (_tile_count_x _tile_count_y) (`KismetMathLibrary.BreakVector2D` (`self.Tile Count`)))
  (bind _tile_count_x_2 (`KismetMathLibrary.BreakVector2D` (`self.Tile Count`)))
  (`KismetArrayLibrary.Array_Clear` (`self.InternalArray`))
  (for _index (range (`KismetMathLibrary.Round` _tile_count_x_2))
    (set `local.xIndex` _index)
    (for _index_2 (range (`KismetMathLibrary.Round` _tile_count_y))
      (set `local.yIndex` _index_2)
      (`self.Add Empty Map Note` (`local.xIndex`) (`local.yIndex`)))))

(fn `ReInit`
  (params (InternalArray :type "Array of /Game/Contract/MapCore/MapNote_Data Structure"))
  (set `self.InternalArray` InternalArray))

(fn `RemoveNote`
  (params (X :type Integer) (Y :type Integer))
  (bind (_noteatindex _noteindex _succ) (`self.GetElement2D` X Y))
  (if _succ
    (`KismetArrayLibrary.Array_Remove` (`self.InternalArray`) _noteindex)
    (`|ExecutionSequence`
      (:`then_0`
        (bind _allnotesofgivenxindex (`self.Get All Elements Of Given XIndex` (+ (`local.X`) -1)))
        (bind _values (`BlueprintMapLibrary.Map_Values` _allnotesofgivenxindex))
        (for _array_element _values
          (bind ((`ConnectedTo_42_F389FE754222BF472745CEBCC02B48FF` _connectedto)) (break `/Game/Contract/MapCore/MapNote_Data` _array_element))
          (for (_array_element_2 _array_index) _connectedto
            (bind (_x _y) (break `/Game/Contract/MapCore/2DArrayPosition_Data` _array_element_2))
            (if (and (== _x (`local.X`)) (== _y (`local.Y`)))
              (`KismetArrayLibrary.Array_Remove` _connectedto _array_index)))))
      (:`then_1`
        (bind _allnotesofgivenxindex_2 (`self.Get All Elements Of Given XIndex` (+ (`local.X`) 1)))
        (bind _values_2 (`BlueprintMapLibrary.Map_Values` _allnotesofgivenxindex_2))
        (for _array_element_3 _values_2
          (bind ((`Connections_38_3AA328AE439A0A46F0F09F9AEAA74CBB` _connections)) (break `/Game/Contract/MapCore/MapNote_Data` _array_element_3))
          (for (_array_element_4 _array_index_2) _connections
            (bind (_x_2 _y_2) (break `/Game/Contract/MapCore/2DArrayPosition_Data` _array_element_4))
            (if (and (== _x_2 (`local.X`)) (== _y_2 (`local.Y`)))
              (`KismetArrayLibrary.Array_Remove` _connections _array_index_2))))))))

(fn `Set Elements Of Given XIndex`
  (params (XIndex :type Integer) (NotesToSet :type "Array of /Game/Contract/MapCore/MapNote_Data Structure"))
  (locals (LocMap :type "Map of Integer to /Game/Contract/MapCore/MapNote_Data Structure"))
  (bind _allnotesofgivenyindex (`self.Get All Elements Of Given YIndex` XIndex))
  (bind _output_get (set `local.LocMap` _allnotesofgivenyindex))
  (bind _keys (`BlueprintMapLibrary.Map_Keys` _output_get))
  (for (_array_element _array_index) _keys
    (`self.SetElement2D` (`local.XIndex`) _array_element (`|GetArrayItem` (`local.NotesToSet`) _array_index))))

(fn `Set Elements Of Given YIndex`
  (params (YIndex :type Integer) (NotesToSet :type "Array of /Game/Contract/MapCore/MapNote_Data Structure"))
  (locals (LocMap :type "Map of Integer to /Game/Contract/MapCore/MapNote_Data Structure"))
  (bind _allnotesofgivenyindex (`self.Get All Elements Of Given YIndex` YIndex))
  (bind _output_get (set `local.LocMap` _allnotesofgivenyindex))
  (bind _keys (`BlueprintMapLibrary.Map_Keys` _output_get))
  (for (_array_element _array_index) _keys
    (`self.SetElement2D` _array_element (`local.YIndex`) (`|GetArrayItem` (`local.NotesToSet`) _array_index))))

(fn `SetElement2D`
  (params (XIndex :type Integer) (YIndex :type Integer) (MapNote :type "/Game/Contract/MapCore/MapNote_Data Structure"))
  (`KismetArrayLibrary.Array_Set` (`self.InternalArray`) (`.NoteIndex` (`self.GetElement2D` XIndex YIndex)) MapNote))

(fn `UserConstructionScript`)