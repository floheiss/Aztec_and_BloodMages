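; BP_ContractManager runs contract setup and cleanup, managing the map UI and the party's placement.
; SetUpContract teleports each MercGroup member to a PositionsMap slot keyed by team size and index, then creates W_Map as the displayed HUD.
; GetMapForDisplay generates the dungeon map once via a temporary BP_MapGenerator, caching it on the GameInstance.
; Older MainHUD/MapHUD helpers remain, but their creation code never runs and DisplayMap is empty.
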(event Custom|OnMenuUpdate
  (params (MenuOpen :type MenuList%20Enum :default "NewEnumerator3"))
  (switch Utilities|FlowControl|Switch|SwitchonMenuList MenuOpen
    (:NewEnumerator3
      _)
    (:NewEnumerator1
      _)
    (:NewEnumerator4
      _)
    (:NewEnumerator7
      _)
    (:NewEnumerator8
      _)
    (:NewEnumerator9
      _)
    (:NewEnumerator12
      _)
    (:NewEnumerator13
      _)
    (:NewEnumerator14
      _))
  (HUD|DisplayMap))

(event Custom|SetUpContract
  (Variables|HUD|SetLastDisplayedHUDSet false)
  (Variables|HUD|SetLastDisplayedHUD 0)
  (CallFunction|TeleportParty)
  (Variables|HUD|SetAnyHUDWasDisplayed false)
  (bind _returnvalue (UserInterface|CreateWidget "/Game/DungeonMap/MapV2/HUD/W_Map.W_Map_C"))
  (bind _output_get (Variables|Map|SetNewMap _returnvalue))
  (Default|SetUpMapDisplayFirstTime _output_get)
  (Class|INUniversalController|SetDisplayedHUD(Message) (Game|GetPlayerController 0) (Variables|Map|GetNewMap)))

(event EventBeginPlay)

(fn ConstructionScript)

(fn CleanUpContract
  (Variables|/Game/Core/GI_Persistence.GI_Persistence_C|SetContractSet (CallFunction|GetGameInst) false)
  (bind _maphud (Variables|Map|GetMapHUD)
    (:then
      (Widget|RemovefromParent _maphud))
    (:else
      _))
  (bind _mainhud (Variables|HUD|GetMainHUD)
    (:then
      (Widget|RemovefromParent _mainhud))
    (:else
      _))
  (bind _lastdisplayedhud (Variables|HUD|GetLastDisplayedHUD)
    (:then
      (Widget|RemovefromParent _lastdisplayedhud))
    (:else
      _))
  (Variables|HUD|SetAnyHUDWasDisplayed false)
  (Variables|HUD|SetLastDisplayedHUDSet false)
  (Variables|HUD|SetLastDisplayedHUD 0)
  (Utilities|Struct|SetmembersinMapForDisplay_Data (Variables|/Game/Core/GI_Persistence.GI_Persistence_C|GetDungeonMap (CallFunction|GetGameInst)) "(X_16_7E4C91A8417F4C9EF0C141A64BED15BE=-1,Y_17_EE273A42468549352FD16DBB63F77F96=-1)"))

(fn GetMapforDisplay
  (if (Variables|/Game/Core/GI_Persistence.GI_Persistence_C|GetMapSet (CallFunction|GetGameInst))
    _
    (else
      (bind _returnvalue (Game|SpawnActorfromClass "/Game/Contract/BP_MapGenerator.BP_MapGenerator_C" (Math|Transform|MakeTransform "-1999.000000,-1999.000000,-1999.000000" "0, 0, 0" "1.000000,1.000000,1.000000") "Undefined" "MultiplyWithRoot" 0 0))
      (bind _generatedmap (Default|GenerateMap _returnvalue (.MapInfo (Utilities|Struct|BreakContract_Data (Variables|/Game/Core/GI_Persistence.GI_Persistence_C|GetContract%20 (CallFunction|GetGameInst))))))
      (Default|SetDungeonMap (CallFunction|GetGameInst) _generatedmap)
      (Actor|DestroyActor _returnvalue)))
  (return (Variables|/Game/Core/GI_Persistence.GI_Persistence_C|GetDungeonMap (CallFunction|GetGameInst))))

(fn ClearLastOpenHUD
  (if (Widget|IsVisible (Variables|HUD|GetLastDisplayedHUD))
    (Widget|RemovefromParent (Variables|HUD|GetLastDisplayedHUD))
    (Variables|HUD|SetLastDisplayedHUDSet false))
  (return))

(fn SetLastDisplayedHUD
  (params (LastDisplayedHUD :type User%20Widget%20Object%20Reference))
  (Variables|HUD|SetLastDisplayedHUD LastDisplayedHUD)
  (Variables|HUD|SetLastDisplayedHUDSet true)
  (Variables|HUD|SetLastDisplayCompleted false)
  (Variables|HUD|SetAnyHUDWasDisplayed true))

(fn SetLastActiveNote
  (params (Note :type 2D%20Array%20Position%20Data%20Structure)))

(fn DisplayLastDisplayHUD
  (UserInterface|Viewport|AddtoViewport (Variables|HUD|GetLastDisplayedHUD) 0)
  (HUD|RemoveMap)
  (HUD|ReApplyMainHud))

(fn ReApplyMainHud
  (Widget|RemovefromParent (Variables|HUD|GetMainHUD))
  (UserInterface|Viewport|AddtoViewport (Variables|HUD|GetMainHUD) 0))

(fn DisplayMap)

(fn RemoveMap
  (if (Variables|HUD|GetLastDisplayedHUDSet)
    (if (Widget|IsVisible (Variables|Map|GetMapHUD))
      (Widget|RemovefromParent (Variables|Map|GetMapHUD)))))

(fn TeleportParty
  (for (_array_element _array_index) (Variables|/Game/Core/GI_Persistence.GI_Persistence_C|GetMercGroup%20 (CallFunction|GetGameInst))
    (if (.ReturnValue (Utilities|Map|Find (LocalVariables|GetPositionsMap) (Math|Float|Truncate (|((TeamSize*10)+(UnitNumber*1)) (Math|Conversions|ToFloat(Integer) (Utilities|Array|Length (Variables|/Game/Core/GI_Persistence.GI_Persistence_C|GetMercGroup%20 (CallFunction|GetGameInst)))) (Math|Conversions|ToFloat(Integer) _array_index)))))
      (LocalVariables|SetLocCurrentVector (.Value (Utilities|Map|Find (LocalVariables|GetPositionsMap) (Math|Float|Truncate (|((TeamSize*10)+(UnitNumber*1)) (Math|Conversions|ToFloat(Integer) (Utilities|Array|Length (Variables|/Game/Core/GI_Persistence.GI_Persistence_C|GetMercGroup%20 (CallFunction|GetGameInst)))) (Math|Conversions|ToFloat(Integer) _array_index))))))
      (else
        (Development|PrintText (Utilities|Text|FormatText "ERROR NO POSITION FOUND FOR UNIT {U}" (Math|Float|Truncate (|((TeamSize*10)+(UnitNumber*1)) (Math|Conversions|ToFloat(Integer) (Utilities|Array|Length (Variables|/Game/Core/GI_Persistence.GI_Persistence_C|GetMercGroup%20 (CallFunction|GetGameInst)))) (Math|Conversions|ToFloat(Integer) _array_index)))))
        (LocalVariables|SetLocCurrentVector (LocalVariables|GetLocErrorVector))))
    (Transformation|SetActorLocation _array_element (LocalVariables|GetLocCurrentVector) false true)))