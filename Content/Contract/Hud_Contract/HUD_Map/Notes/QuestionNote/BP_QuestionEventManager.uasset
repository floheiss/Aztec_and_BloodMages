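; BP_QuestionEventManager resolves the outcome of question-note events on the contract map.
; It caches the BP_ContractManager at BeginPlay, and HandleQuestionEvent switches on the reward action.
; Gold gain or loss goes through ManageGoldEvents to the game instance's party gold, while no-action and no-effect outcomes only print text.
; It then sets LastDisplayCompleted on the contract manager and switches the menu through the game instance.
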(event `self.ReceiveBeginPlay`
  (bind _returnvalue (`GameplayStatics.GetActorOfClass` "/Game/Contract/BP_ContractManager.BP_ContractManager_C"))
  (set `self.ContractManager` _returnvalue))

(fn `HandleQuestionEvent`
  (params (RewardAction :type "/Game/Contract/MapNotes/Notes/EventStuffAndThings/EventOptionReward Enum" :default "NewEnumerator0") (RewardExtraInfo :type Integer))
  (switch `/Game/Contract/MapNotes/Notes/EventStuffAndThings/EventOptionReward` RewardAction
    (:`NewEnumerator0`
      (`self.ManageGoldEvents` (`local.RewardAction`) (`local.RewardExtraInfo`) :!label _label))
    (:`NewEnumerator1`
      (goto _label))
    (:`NewEnumerator2`
      (`KismetSystemLibrary.PrintText` "Nothing happend" :!label _label_2))
    (:`NewEnumerator3`
      (goto _label_2)))
  (set `/Game/Contract/BP_ContractManager.LastDisplayCompleted` true (`self.ContractManager`))
  (`/Game/Core/GI_Persistence.SetMenu` (`/Game/Core/BFL_General.GetGameInst`) "NewEnumerator14"))

(fn `ManageGoldEvents`
  (params (ActionTaken :type "/Game/Contract/MapNotes/Notes/EventStuffAndThings/EventOptionReward Enum" :default "NewEnumerator0") (GoldAmount :type Integer))
  (`/Game/Core/GI_Persistence.ManagePartyGold` (`/Game/Core/BFL_General.GetGameInst`) GoldAmount (`|EnumEquality` ActionTaken "NewEnumerator1")))

(fn `UserConstructionScript`)