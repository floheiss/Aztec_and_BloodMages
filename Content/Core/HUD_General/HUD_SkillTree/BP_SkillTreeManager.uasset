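; BP_SkillTreeManager backs the skill tree menu, opening W_SkillTrees and handling attack purchases with party gold and attack selection.
; Selections are capped and locked to one skill tree plus neutral attacks, with conflicts raising a swap widget and SwapSkilltree removing the old tree's picks.
; It tracks the main ability and selection validity, and ConvertToMainSelection rebuilds the Blood Mage's AttackManager loadout, preserving upgrade flags.
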(event `DisplaySkillTree`
  (bind _returnvalue (`|CreateWidget` "/Game/Core/HUD_General/HUD_SkillTree/HUD/W_SkillTrees.W_SkillTrees_C" null self))
  (set `self.SkillTreeHud` _returnvalue)
  (message `/Game/Core/IN_UniversalController.SetDisplayedHUD` (`GameplayStatics.GetPlayerController` 0) (`self.SkillTreeHud`))
  (`/Game/Core/GI_Persistence.SetMenu` (`/Game/Core/BFL_General.GetGameInst`) "NewEnumerator13"))

(fn `AddAttackToSelection`
  (params (Attack :type "/Game/Chars/Attacks/Enums/AttackList Enum" :default "NewEnumerator1"))
  (if (< (`KismetArrayLibrary.Array_Length` (`self.SelectedAttacks`)) (`self.MaxSelectedAttacks`))
    (if (`self.CheckSkilltree` (`local.Attack`))
      (if (`KismetArrayLibrary.Array_Contains` (`self.SelectedAttacks`) (`local.Attack`))
        (message `/Game/Core/IN_UniversalController.DisplayNotification` (`GameplayStatics.GetPlayerController` 0) "Attack already selected" 10.0)
        (else
          (`KismetArrayLibrary.Array_Add` (`self.SelectedAttacks`) (`local.Attack`))
          (`self.ManageMainAttack` (`local.Attack`))
          (`self.AttackSelectionChanged` (`local.Attack`))))
      (else
        (bind _skilltreedata (`/Game/Chars/Attacks/BFL_Attacks.GetAttackSkillDataFromAttack` (`local.Attack`)))
        (`self.DisplayWidgetSwapSkilltree` (`.SkillTree_25_0468AD3C473FF95CC15D0F9ECF0973AE` (break `/Game/Chars/Attacks/AttackSkillTreeData` _skilltreedata)))))
    (else
      (message `/Game/Core/IN_UniversalController.DisplayNotification` (`GameplayStatics.GetPlayerController` 0) "Max number of attacks selected" 10.0))))

(fn `BuyAttack`
  (params (AttackToBuy :type "/Game/Chars/Attacks/Enums/AttackList Enum" :default "NewEnumerator1"))
  (returns (Succ :type Boolean))
  (locals (LocSkillTreeData :type "/Game/Chars/Attacks/AttackSkillTreeData Structure"))
  (bind _skilltreedata (`/Game/Chars/Attacks/BFL_Attacks.GetAttackSkillDataFromAttack` AttackToBuy))
  (bind _succ (`/Game/Core/GI_Persistence.ManagePartyGold` (`/Game/Core/BFL_General.GetGameInst`) (`.Price_26_0F67AF674B31102D8DDBD9A2DD8B7AF8` (break `/Game/Chars/Attacks/AttackSkillTreeData` _skilltreedata)) true))
  (if _succ
    (`KismetArrayLibrary.Array_Add` (`self.UnlockedAttack`) (`local.AttackToBuy`))
    (`self.BroughtAttack` (`local.AttackToBuy`))
    (return true)
    (else
      (message `/Game/Core/IN_UniversalController.DisplayNotification` (`GameplayStatics.GetPlayerController` 0) "So no Money " 6.0)
      (return false))))

(fn `CheckResetSkilltree`
  (locals (LocCheckFailed :type Boolean))
  (for _array_element (`self.SelectedAttacks`)
    (bind _skilltreedata (`/Game/Chars/Attacks/BFL_Attacks.GetAttackSkillDataFromAttack` _array_element))
    (if (`|EnumInequality` (`.SkillTree_25_0468AD3C473FF95CC15D0F9ECF0973AE` (break `/Game/Chars/Attacks/AttackSkillTreeData` _skilltreedata)) "NewEnumerator5")
      (set `local.LocCheckFailed` true)))
  (if (not (`local.LocCheckFailed`))
    (`KismetSystemLibrary.PrintText` "skilltree was reset :)")
    (set `self.CurrentSkilltree` "NewEnumerator5")))

(fn `CheckSkilltree`
  (params (AttackToCheck :type "/Game/Chars/Attacks/Enums/AttackList Enum" :default "NewEnumerator1"))
  (returns (`Is Valid` :type Boolean))
  (if (`|EnumEquality` (`self.CurrentSkilltree`) "NewEnumerator5")
    ;[1 1 1] if no skilltree selected it is set
    (bind _skilltreedata (`/Game/Chars/Attacks/BFL_Attacks.GetAttackSkillDataFromAttack` (`local.AttackToCheck`)))
    (set `self.CurrentSkilltree` (`.SkillTree_25_0468AD3C473FF95CC15D0F9ECF0973AE` (break `/Game/Chars/Attacks/AttackSkillTreeData` _skilltreedata)))
    (return true)
    (else
      ;[1 1 1] checks if is current if not returns error
      (bind _skilltreedata_2 (`/Game/Chars/Attacks/BFL_Attacks.GetAttackSkillDataFromAttack` (`local.AttackToCheck`)))
      (bind ((`SkillTree_25_0468AD3C473FF95CC15D0F9ECF0973AE` _skilltree)) (break `/Game/Chars/Attacks/AttackSkillTreeData` _skilltreedata_2))
      (if (or (`|EnumEquality` _skilltree (`self.CurrentSkilltree`)) (`|EnumEquality` _skilltree "NewEnumerator5"))
        (return true)
        (else
          (return false))))))

(fn `ConvertToMainSelection`
  (locals (LocAttackManager :type "/Game/Chars/AttackManager/BP_AttackManager Object Reference") (LocBackUpList :type "Map of /Game/Chars/Attacks/Enums/AttackList Enum to Boolean"))
  (bind _output_get (set `local.LocAttackManager` (`/Game/Chars/PZD_Unit.AttackManager` (`/Game/Core/GI_Persistence.GetBloodMage` (`/Game/Core/BFL_General.GetGameInst`)))))
  (bind _avaliableattacks (`/Game/Chars/AttackManager/BP_AttackManager.GetAllAvaliableAttacks` _output_get))
  (set `local.LocBackUpList` _avaliableattacks)
  (`/Game/Chars/AttackManager/BP_AttackManager.ClearAvaliableAttck` (`local.LocAttackManager`))
  (`/Game/Chars/AttackManager/BP_AttackManager.ClearSelectedAttacks` (`local.LocAttackManager`))
  (for _array_element (`self.SelectedAttacks`)
    (`/Game/Chars/AttackManager/BP_AttackManager.AddAvaliableAttacks` (`local.LocAttackManager`) _array_element (`BlueprintMapLibrary.Map_Find` (`local.LocBackUpList`) _array_element) (`|EnumEquality` _array_element (`self.MainAttack`)))))

(fn `DisplayWidgetSwapSkilltree`
  (params (NewSkilltree :type "/Game/Core/GeneralEnums/SkillTreeList Enum" :default "NewEnumerator0"))
  (set `self.WarningUp` true)
  (`/Game/Core/HUD_General/HUD_SkillTree/HUD/W_SkillTrees.DisplaySkillTreeSwapWidget` (`self.SkillTreeHud`) (`local.NewSkilltree`)))

(fn `IsSelectionValid`
  (returns (IsValid :type Boolean))
  (locals (LocValid :type Boolean :default false))
  (return (and (`self.MainAttackSet`) (== (`KismetArrayLibrary.Array_Length` (`self.SelectedAttacks`)) (`self.MaxSelectedAttacks`)))))

(fn `ManageMainAttack`
  (params (Attack :type "/Game/Chars/Attacks/Enums/AttackList Enum" :default "NewEnumerator1") (IsRemoved :type Boolean))
  (bind _skilltreedata (`/Game/Chars/Attacks/BFL_Attacks.GetAttackSkillDataFromAttack` Attack))
  (bind ((`IsMainAbility_21_A4FA16114B301A9E18AD0A8EA32BBEDC` _ismainability) (`SkillTree_25_0468AD3C473FF95CC15D0F9ECF0973AE` _skilltree)) (break `/Game/Chars/Attacks/AttackSkillTreeData` _skilltreedata))
  (if _ismainability
    (if (`local.IsRemoved`)
      (set `self.MainAttack` "NewEnumerator1")
      (set `self.MainAttackSet` false)
      (else
        (set `self.MainAttack` (`local.Attack`))
        (set `self.MainAttackSet` true)
        (set `self.CurrentSkilltree` _skilltree)))))

(fn `RemoveAttackFormSelection`
  (params (Attack :type "/Game/Chars/Attacks/Enums/AttackList Enum" :default "NewEnumerator1"))
  (if (`KismetArrayLibrary.Array_Contains` (`self.SelectedAttacks`) Attack)
    (`KismetArrayLibrary.Array_RemoveItem` (`self.SelectedAttacks`) (`local.Attack`))
    (`self.ManageMainAttack` (`local.Attack`) true)
    (`self.CheckResetSkilltree`)
    (`self.AttackSelectionChanged` (`local.Attack`) true)
    (else
      (message `/Game/Core/IN_UniversalController.DisplayNotification` (`GameplayStatics.GetPlayerController` 0) "Attack not selected, cant be removed" 10.0))))

(fn `SwapSkilltree`
  (params (NewSkilltree :type "/Game/Core/GeneralEnums/SkillTreeList Enum" :default "NewEnumerator0"))
  (for _array_element (`self.SelectedAttacks`)
    (bind _skilltreedata (`/Game/Chars/Attacks/BFL_Attacks.GetAttackSkillDataFromAttack` _array_element))
    (if (`|EnumEquality` (`.SkillTree_25_0468AD3C473FF95CC15D0F9ECF0973AE` (break `/Game/Chars/Attacks/AttackSkillTreeData` _skilltreedata)) (`self.CurrentSkilltree`))
      (`self.RemoveAttackFormSelection` _array_element)))
  (set `self.CurrentSkilltree` (`local.NewSkilltree`)))

(fn `UserConstructionScript`)