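; Manager for the dungeon map that shows the W_Map HUD widget and tracks contract progress between fights.
; DisplayMap creates the widget once, then runs ordered checks where later hits override the menu: map, campfire, unspent level-up, saved loot.
; Combat start is forwarded to BP_DungeonMaster; combat completion increments fight and level counters.
; Reaching the contract's max level only shows a placeholder notification, as ExitContract is empty.
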(event `self.ReceiveBeginPlay`
  (add `self.CombatStart` (`|CreateDelegate` :!event `OnCombatStart`))
  (add `self.CombatDone` (`|CreateDelegate` :!event `OnCombatDone`)))

(fn `CheckEndContract`
  (if (>= (`self.CurrentLvL`) (`.MapMaxLvL_39_53F0F00109DF40889978B82FCFCA8E52` (break `/Game/Town/Guild/Contract_Data` (`/Game/Core/GI_Persistence.GetContract` (`/Game/Core/BFL_General.GetGameInst`)))))
    (message `/Game/Core/IN_UniversalController.DisplayNotification` (`GameplayStatics.GetPlayerController` 0) "Would have ended contract" 3.0)
    (`self.ExitContract`)))

(fn `DisplayLvLUp`
  (params (LvLUpData :type "/Game/Chars/MercLvLManagment/UnitLeveledDisplayUpData Structure"))
  (`/Game/DungeonMap/MapV2/HUD/W_Map.SetLvLUpScreen` (`self.Map`) LvLUpData))

(fn `DisplayMap`
  (`self.Map`
    (:`then`
      _)
    (:`else`
      (bind _returnvalue (`|CreateWidget` "/Game/DungeonMap/MapV2/HUD/W_Map.W_Map_C"))
      (set `self.Map` _returnvalue)))
  (if (`|EnumEquality` (`/Game/Core/GI_Persistence.Controller Mode` (`/Game/Core/BFL_General.GetGameInst`)) "NewEnumerator2")
    (message `/Game/Core/IN_UniversalController.SetDisplayedHUD` (`GameplayStatics.GetPlayerController` 0) (`self.Map`))
    (set `self.MenuToDisplay` "NewEnumerator14")
    (`|ExecutionSequence`
      (:`then_0`
        (`self.CheckForMap`))
      (:`then_1`
        (`self.CheckForCampfire`))
      (:`then_2`
        (`self.CheckForLvL`))
      (:`then_3`
        (`self.CheckForLoot`))
      (:`then_4`
        (`/Game/Core/GI_Persistence.SetMenu` (`/Game/Core/BFL_General.GetGameInst`) (`self.MenuToDisplay`))))
    (else
      (`Widget.RemoveFromParent` (`self.Map`)))))

(fn `DisplayUnit`
  (params (UnitToDisplay :type "/Game/Chars/PZD_Unit Object Reference"))
  (`/Game/Core/GI_Persistence.SetMenu` (`/Game/Core/BFL_General.GetGameInst`) "NewEnumerator10")
  (`/Game/DungeonMap/MapV2/HUD/W_Map.SetMercDisplay` (`self.Map`) (`local.UnitToDisplay`)))

(fn `ExitContract`)

(fn `IncremtentAfterCombat`
  (params (NoteType :type "/Game/DungeonMap/MapV2/NoteType Enum" :default "NewEnumerator0"))
  (`|ExecutionSequence`
    (:`then_0`
      (`/Engine/EditorBlueprintResources/StandardMacros.IncrementInt` (`self.FightCounter`)
        (:`  `
          (if (`|EnumInequality` (`local.NoteType`) "NewEnumerator0")
            (`/Engine/EditorBlueprintResources/StandardMacros.IncrementInt` (`self.CurrentLvL`)
              (:`  `
                (`self.LvLIncrement`)))))))
    (:`then_1`
      (`self.FightCounterIncrement`))))

(fn `OnCombatDone`
  (params (NoteType :type "/Game/DungeonMap/MapV2/NoteType Enum" :default "NewEnumerator0") (Heat :type "Float (double-precision)"))
  (`self.IncremtentAfterCombat` NoteType)
  (`self.CheckEndContract`))

(fn `OnCombatStart`
  (params (NoteType :type "/Game/DungeonMap/MapV2/NoteType Enum" :default "NewEnumerator0") (Heat :type "Float (double-precision)"))
  (set `self.CurrNoteType` NoteType)
  (set `self.CurrNoteHeat` Heat)
  (bind _returnvalue (`GameplayStatics.GetActorOfClass` "/Game/Contract/BP_DungeonMaster.BP_DungeonMaster_C"))
  (`/Game/Contract/BP_DungeonMaster.StartCombat` _returnvalue (`self.CurrNoteType`) (`self.CurrNoteHeat`)))

(fn `RemoveMap`
  (message `/Game/Core/IN_UniversalController.RemoveDisplayedHUD` (`GameplayStatics.GetPlayerController` 0)))

(fn `UserConstructionScript`)