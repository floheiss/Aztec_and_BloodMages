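; BP_QuestionEventManager applies the outcome of a question event on the dungeon map.
; HandleQuestionEvent routes gold gain and loss actions to ManageGoldEvents, which adjusts party gold through the game instance, while no-action and no-effect outcomes do nothing.
; Every outcome then clears the displayed HUD message and switches the menu through the game instance.
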(fn `HandleQuestionEvent`
  (params (RewardAction :type "/Game/DungeonMap/MapNotes/HUD/EventStuffAndThings/EventOptionReward Enum" :default "NewEnumerator0") (RewardExtraInfo :type Integer))
  (switch `/Game/DungeonMap/MapNotes/HUD/EventStuffAndThings/EventOptionReward` RewardAction
    (:`NewEnumerator0`
      (`self.ManageGoldEvents` (`local.RewardAction`) (`local.RewardExtraInfo`) :!label _label))
    (:`NewEnumerator1`
      (goto _label))
    (:`NewEnumerator2`
      _)
    (:`NewEnumerator3`
      _))
  (message `/Game/Core/UniversalController_Interface.RemoveDisplayedHUD` (`GameplayStatics.GetPlayerController` 0))
  (`/Game/Core/GI_Persistence.UpdateMenu` (`/Game/Generel_Actor/BFL_General.GetGameInst`) "NewEnumerator3"))

(fn `ManageGoldEvents`
  (params (ActionTaken :type "/Game/DungeonMap/MapNotes/HUD/EventStuffAndThings/EventOptionReward Enum" :default "NewEnumerator0") (GoldAmount :type Integer))
  (`/Game/Core/GI_Persistence.ManagePartyGold` (`/Game/Generel_Actor/BFL_General.GetGameInst`) GoldAmount (`|EnumEquality` ActionTaken "NewEnumerator1")))

(fn `UserConstructionScript`)