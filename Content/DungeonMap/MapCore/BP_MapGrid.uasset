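; BP_MapGrid holds the dungeon map as a 2D grid of MapNoteData, stored in one flat array.
; On BeginPlay, Init fills the TileCount X-by-Y grid with empty, locked notes that record their own coordinates.
; Element lookups scan the array linearly for matching positions, while row and column getters return maps keyed by the other axis.
; Setters overwrite entries through these lookups, and AddOutOfGridNotes appends extra notes to the same array.
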(event `self.ReceiveBeginPlay`
  (`self.Init` (`self.Tile Count`)))

(fn `AddOutOfGridNotes`
  (params (MapNote :type "/Game/DungeonMap/MapCore/MapNote_Data Structure"))
  (returns (IndexOfNote :type Integer))
  (bind _returnvalue (`KismetArrayLibrary.Array_Add` (`self.InternalArray`) MapNote))
  (return _returnvalue))

(fn `Get All Elements Of Given XIndex`
  (params (XIndex :type Integer))
  (returns (AllNotesOfGivenXIndex :type "Map of Integer to /Game/DungeonMap/MapCore/MapNote_Data Structure"))
  (locals (LocMap :type "Map of Integer to /Game/DungeonMap/MapCore/MapNote_Data Structure"))
  (bind _tile_count_x (`KismetMathLibrary.BreakVector2D` (`self.Tile Count`)))
  (bind _tile_count_x_2 (`KismetMathLibrary.BreakVector2D` (`self.Tile Count`)))
  (bind _tile_count_x_3 (`KismetMathLibrary.BreakVector2D` (`self.Tile Count`)))
  (for _array_element (`self.InternalArray`)
    (bind (_x _y) (break `/Game/DungeonMap/MapCore/2DArrayPosition_Data` (`.PositionIn2DArray_33_7FF6CAD844866154E2D040A134BA7301` (break `/Game/DungeonMap/MapCore/MapNote_Data` _array_element))))
    (if (== _x (`local.XIndex`))
      (`BlueprintMapLibrary.Map_Add` (`local.LocMap`) _y _array_element)
      (if (== (`BlueprintMapLibrary.Map_Length` (`local.LocMap`)) (`KismetMathLibrary.Round` _tile_count_x_2))
        (`KismetSystemLibrary.PrintText` (`|FormatText` "MapLength: {MapL}, The XLength: {XL}" (`BlueprintMapLibrary.Map_Length` (`local.LocMap`)) _tile_count_x))
        (return (`local.LocMap`)))))
  (`KismetSystemLibrary.PrintText` (`|FormatText` "MapLength: {MapL}, The XLength: {XL}" (`BlueprintMapLibrary.Map_Length` (`local.LocMap`)) _tile_count_x_3))
  (return (`local.LocMap`)))

(fn `Get All Elements Of Given YIndex`
  (params (YIndex :type Integer))
  (returns (AllNotesOfGivenYIndex :type "Map of Integer to /Game/DungeonMap/MapCore/MapNote_Data Structure"))
  (locals (LocMap :type "Map of Integer to /Game/DungeonMap/MapCore/MapNote_Data Structure"))
  (bind (_tile_count_x _tile_count_y) (`KismetMathLibrary.BreakVector2D` (`self.Tile Count`)))
  (bind _tile_count_x_2 (`KismetMathLibrary.BreakVector2D` (`self.Tile Count`)))
  (bind (_tile_count_x_3 _tile_count_y_2) (`KismetMathLibrary.BreakVector2D` (`self.Tile Count`)))
  (for _array_element (`self.InternalArray`)
    (bind (_x _y) (break `/Game/DungeonMap/MapCore/2DArrayPosition_Data` (`.PositionIn2DArray_33_7FF6CAD844866154E2D040A134BA7301` (break `/Game/DungeonMap/MapCore/MapNote_Data` _array_element))))
    (if (== _y (`local.YIndex`))
      (`BlueprintMapLibrary.Map_Add` (`local.LocMap`) _x _array_element)
      (if (== (`BlueprintMapLibrary.Map_Length` (`local.LocMap`)) (`KismetMathLibrary.Round` _tile_count_y))
        (`KismetSystemLibrary.PrintText` (`|FormatText` "Early Exit MapLength: {MapL}, The XLength: {XL}" (`BlueprintMapLibrary.Map_Length` (`local.LocMap`)) _tile_count_x_2))
        (return (`local.LocMap`)))))
  (`KismetSystemLibrary.PrintText` (`|FormatText` "MapLength: {MapL}, The YLength: {XL}" (`BlueprintMapLibrary.Map_Length` (`local.LocMap`)) _tile_count_y_2))
  (return (`local.LocMap`)))

(fn `GetElement2D`
  (params (XIndex :type Integer) (YIndex :type Integer))
  (returns (NoteAtIndex :type "/Game/DungeonMap/MapCore/MapNote_Data Structure") (NoteIndex :type Integer))
  (for (_array_element _array_index) (`self.InternalArray`)
    (bind (_x _y) (break `/Game/DungeonMap/MapCore/2DArrayPosition_Data` (`.PositionIn2DArray_33_7FF6CAD844866154E2D040A134BA7301` (break `/Game/DungeonMap/MapCore/MapNote_Data` _array_element))))
    (if (and (== _x (`local.XIndex`)) (== _y (`local.YIndex`)))
      (return _array_element _array_index)))
  (`KismetSystemLibrary.PrintText` (`|FormatText` "There is no note at: {X}, {Y}" (`local.XIndex`) (`local.YIndex`))))

(fn `Init`
  (params (Size :type "Vector2D Structure"))
  (locals (yIndex :type Integer) (xIndex :type Integer))
  (bind (_tile_count_x _tile_count_y) (`KismetMathLibrary.BreakVector2D` (`self.Tile Count`)))
  (bind _tile_count_x_2 (`KismetMathLibrary.BreakVector2D` (`self.Tile Count`)))
  (bind (_tile_count_x_3 _tile_count_y_2) (`KismetMathLibrary.BreakVector2D` (`self.Tile Count`)))
  (`KismetArrayLibrary.Array_Clear` (`self.InternalArray`))
  (`|ExecutionSequence`
    (:`then_0`
      ;[1 1 1] debug
      (`KismetSystemLibrary.PrintText` (`|FormatText` "Requested X: {X},Requested Y: {y}" _tile_count_x_3 _tile_count_y_2)))
    (:`then_1`
      (for _index (range (`KismetMathLibrary.Round` _tile_count_x_2))
        (set `local.xIndex` _index)
        (for _index_2 (range (`KismetMathLibrary.Round` _tile_count_y))
          (set `local.yIndex` _index_2)
          (`self.SetEmptyMapNote` (`local.xIndex`) (`local.yIndex`)))))))

(fn `ReInit`
  (params (InternalArray :type "Array of /Game/DungeonMap/MapCore/MapNote_Data Structure"))
  (set `self.InternalArray` InternalArray))

(fn `Set Elements Of Given XIndex`
  (params (XIndex :type Integer) (NotesToSet :type "Array of /Game/DungeonMap/MapCore/MapNote_Data Structure"))
  (locals (LocMap :type "Map of Integer to /Game/DungeonMap/MapCore/MapNote_Data Structure"))
  (bind _allnotesofgivenyindex (`self.Get All Elements Of Given YIndex` XIndex))
  (bind _output_get (set `local.LocMap` _allnotesofgivenyindex))
  (bind _keys (`BlueprintMapLibrary.Map_Keys` _output_get))
  (for (_array_element _array_index) _keys
    (`self.SetElement2D` (`local.XIndex`) _array_element (`|GetArrayItem` (`local.NotesToSet`) _array_index))))

(fn `Set Elements Of Given YIndex`
  (params (YIndex :type Integer) (NotesToSet :type "Array of /Game/DungeonMap/MapCore/MapNote_Data Structure"))
  (locals (LocMap :type "Map of Integer to /Game/DungeonMap/MapCore/MapNote_Data Structure"))
  (bind _allnotesofgivenyindex (`self.Get All Elements Of Given YIndex` YIndex))
  (bind _output_get (set `local.LocMap` _allnotesofgivenyindex))
  (bind _keys (`BlueprintMapLibrary.Map_Keys` _output_get))
  (for (_array_element _array_index) _keys
    (`self.SetElement2D` _array_element (`local.YIndex`) (`|GetArrayItem` (`local.NotesToSet`) _array_index))))

(fn `SetElement2D`
  (params (XIndex :type Integer) (YIndex :type Integer) (MapNote :type "/Game/DungeonMap/MapCore/MapNote_Data Structure"))
  (bind (_noteatindex _noteindex) (`self.GetElement2D` XIndex YIndex))
  (`KismetArrayLibrary.Array_Set` (`self.InternalArray`) _noteindex MapNote))

(fn `SetEmptyMapNote`
  (params (X :type Integer) (Y :type Integer))
  (`KismetArrayLibrary.Array_Add` (`self.InternalArray`) (make `/Game/DungeonMap/MapCore/MapNote_Data` (0.0 0.0 0.0) (make `/Game/DungeonMap/MapCore/2DArrayPosition_Data` X Y) "NewEnumerator9" true)))

(fn `UserConstructionScript`)