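; BP_MapGenerator procedurally builds the branching dungeon contract map of enemy, elite, question and campfire nodes.
; GenerateMap randomizes column sizes, fills a BP_MapGrid (reused from or registered on the C_DungeonMap controller) and returns display data.
; Each node gets a probability-rolled type, jittered coordinates and weighted random links to the previous column.
; Single-node helpers add the start, exit and contract-dependent boss, linking them to all preceding nodes.
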(fn ConstructionScript)

(fn GenerateMap
  (params (MapInfoToGen :type Map%20Info%20Data%20Structure))
  (bind _out (CallFunction|GetGameInst))
  (bind _locmapfordisplay (LocalVariables|GetLocMapForDisplay))
  (bind (_maplength _rowsinmap) (Utilities|Struct|BreakMapInfo_Data MapInfoToGen))
  (bind _contracttype (Utilities|Struct|BreakMapForDisplay_Data _locmapfordisplay))
  (bind _contract_ (Variables|/Game/Core/GI_Persistence.GI_Persistence_C|GetContract%20 _out))
  (bind (_contracttypeextrainfo _contracttype_2) (Utilities|Struct|BreakContract_Data _contract_))
  (bind _returnvalue (Utilities|Enum|Equal(Enum) _contracttype "NewEnumerator0"))
  (Variables|Default|SetMapInfo MapInfoToGen)
  ;[1 1 1] Sets length + contract type + extra info
  (Utilities|Struct|SetmembersinMapForDisplay_Data (LocalVariables|GetLocMapForDisplay) (Utilities|Struct|BreakMapInfo_Data MapInfoToGen) _contracttype_2 _contracttypeextrainfo)
  ;[1 1 1] Spawns an sets the MapGrid (is the array)
  (bind _asc_dungeon_map (Utilities|Casting|CastToC_DungeonMap (Game|GetPlayerController 0)))
  (if (Variables|/Game/DungeonMap/MapCore/C_DungeonMap.C_DungeonMap_C|GetIsMapGridSet _asc_dungeon_map)
    (Variables|Default|SetMapGrid (Variables|/Game/DungeonMap/MapCore/C_DungeonMap.C_DungeonMap_C|GetMapGrid _asc_dungeon_map))
    (else
      (bind _returnvalue_2 (Game|SpawnActorfromClass "/Game/DungeonMap/MapCore/BP_MapGrid.BP_MapGrid_C" (Math|Transform|MakeTransform "-999.000000,-999.000000,-999.000000" "0, 0, 0" "1.000000,1.000000,1.000000") "Undefined" "MultiplyWithRoot" 0 0 (Math|Vector2D|MakeVector2D (Math|Conversions|ToFloat(Integer) (+ _rowsinmap 1)) (Math|Conversions|ToFloat(Integer) _maplength)) 0))
      (Variables|Default|SetMapGrid _returnvalue_2)))
  (Utilities|FlowControl|Sequence
    (:then_0
      ;[1 1 1] sets the first as the spawn note
      (Utilities|Array|Add (LocalVariables|GetNumberInColumns) 1)
      ;[1 1 1] this is used to make the map column sizes(For the length of the map a random number is selected as size)
      (for _index (range 1 (Utilities|Struct|BreakMapInfo_Data MapInfoToGen))
        (Utilities|Array|Add (LocalVariables|GetNumberInColumns) (Math|Integer|Clamp(Integer) (+ (Utilities|Struct|BreakMapInfo_Data MapInfoToGen) (Math|Random|RandomIntegerinRange -1 1)) 1 8)))
      (Utilities|Struct|SetmembersinMapForDisplay_Data (LocalVariables|GetLocMapForDisplay) (LocalVariables|GetNumberInColumns)))
    (:then_1
      ;[1 1 1] Spawns the rows
      (for (_array_element _array_index) (LocalVariables|GetNumberInColumns)
        (if (!= _array_index 0)
          (Default|SetElementsOfGivenYIndex (Variables|Default|GetMapGrid) _array_index (CallFunction|GenerateMapRow _array_index _array_element (Variables|Default|GetMapGrid)))
          (else
            (Default|AddOutOfGridNotes (Variables|Default|GetMapGrid) (CallFunction|GenerateSingleNote 0 "NewEnumerator6" (Variables|Default|GetMapGrid)))))))
    (:then_2
      ;[1 1 1] fills the numberOf.. in the List is used to generate mission that arnt boss
      (for _array_element_2 (Variables|/Game/DungeonMap/MapCore/BP_MapGrid.BP_MapGrid_C|GetInternalArray (Variables|Default|GetMapGrid))
        (switch Utilities|FlowControl|Switch|SwitchonMapNoteTypes (Utilities|Struct|BreakMapNote_Data (.NoteAtIndex (Default|GetElement2D (Variables|Default|GetMapGrid) (.x (Utilities|Struct|BreakMapNote_Data _array_element_2)) (.y (Utilities|Struct|BreakMapNote_Data _array_element_2)))))
          (:NewEnumerator0
            (Math|Integer|IncrementInt (Utilities|Struct|BreakMapForDisplay_Data (LocalVariables|GetLocMapForDisplay))))
          (:NewEnumerator1
            (Math|Integer|IncrementInt (Utilities|Struct|BreakMapForDisplay_Data (LocalVariables|GetLocMapForDisplay))))
          (:NewEnumerator2
            (Math|Integer|IncrementInt (Utilities|Struct|BreakMapForDisplay_Data (LocalVariables|GetLocMapForDisplay))))
          (:NewEnumerator3
            (Math|Integer|IncrementInt (Utilities|Struct|BreakMapForDisplay_Data (LocalVariables|GetLocMapForDisplay))))
          (:NewEnumerator6
            (Math|Integer|IncrementInt (Utilities|Struct|BreakMapForDisplay_Data (LocalVariables|GetLocMapForDisplay))))))
      ;[1 1 1] Addes boss note
      (if _returnvalue
        (Default|AddOutOfGridNotes (Variables|Default|GetMapGrid) (CallFunction|GenerateSingleNote (Utilities|Array|Length (Utilities|Struct|BreakMapForDisplay_Data (LocalVariables|GetLocMapForDisplay))) "NewEnumerator5" (Variables|Default|GetMapGrid))))
      ;[1 1 1] addes the exit (always)
      (Default|AddOutOfGridNotes (Variables|Default|GetMapGrid) (CallFunction|GenerateSingleNote (+ (Utilities|Array|Length (Utilities|Struct|BreakMapForDisplay_Data (LocalVariables|GetLocMapForDisplay))) (select _returnvalue 1 0)) "NewEnumerator4" (Variables|Default|GetMapGrid)))
      (Utilities|Struct|SetmembersinMapForDisplay_Data (LocalVariables|GetLocMapForDisplay) (Variables|/Game/DungeonMap/MapCore/BP_MapGrid.BP_MapGrid_C|GetInternalArray (Variables|Default|GetMapGrid)))
      (bind _asc_dungeon_map_2 (Utilities|Casting|CastToC_DungeonMap (Game|GetPlayerController 0)))
      (if (not (Variables|/Game/DungeonMap/MapCore/C_DungeonMap.C_DungeonMap_C|GetIsMapGridSet _asc_dungeon_map_2))
        (Default|SetMapGrid _asc_dungeon_map_2 (Variables|Default|GetMapGrid))
        (return (LocalVariables|GetLocMapForDisplay))))))

(fn GenerateMapRow
  (params (CurrentRow :type Integer) (NumberToGenerate :type Integer) (MapGrid :type BP%20Map%20Grid%20Object%20Reference))
  (bind _returnvalue (== NumberToGenerate 1))
  (for _index (range 0 NumberToGenerate)
    (Utilities|Array|Add (LocalVariables|GetLocMapNotes) (Utilities|Struct|MakeMapNote_Data (Utilities|Struct|Make2DArrayPosition_Data _index CurrentRow) (CallFunction|GenerateRandomNoteType))))
  (CallFunction|GenerateCordinates (LocalVariables|GetLocMapNotes) CurrentRow _returnvalue)
  (CallFunction|GenerateConnections (LocalVariables|GetLocMapNotes) CurrentRow _returnvalue MapGrid)
  (return (LocalVariables|GetLocMapNotes)))

(fn GenerateCordinates
  (params (MapNotes :type Array%20of%20Map%20Note%20Data%20Structures) (CurrentRow :type Integer) (isSingleNote :type Boolean))
  (bind _returnvalue (Math|Random|RandomIntegerinRange -50 50))
  (bind _returnvalue_2 (Math|Random|RandomIntegerinRange -50 50))
  (bind _returnvalue_3 (Math|Conversions|ToFloat(Integer) _returnvalue_2))
  (bind _returnvalue_4 (Math|Conversions|ToFloat(Integer) _returnvalue))
  (LocalVariables|SetXCord (select isSingleNote (/ (LocalVariables|GetMaxHeightOfMapGen) 2) (Math|Float|Truncate (|({AF7754BA-4493-71D2-D8C8-E1BE473AC31A}/NumberInColumn) (Math|Conversions|ToFloat(Integer) (Utilities|Array|Length MapNotes))))))
  (LocalVariables|SetYCord (Math|Float|Truncate (|(700*Row) (Math|Conversions|ToFloat(Integer) CurrentRow))))
  (if (not isSingleNote)
    (for _index (range 0 (- (Utilities|Array|Length MapNotes) 1))
      (Utilities|Struct|SetmembersinMapNote_Data (Utilities|Array|Get(acopy) MapNotes _index) (Math|Vector|MakeVector (|(({706B84D1-4BEE-7CC0-9EEE-78817B529F96}*Index)+RandomPuill) (Math|Conversions|ToFloat(Integer) _index) _returnvalue_3) (|({688362AA-4621-01D6-640E-78ADCACAD910}+RandomPuill) _returnvalue_3) 1e+01)))
    (else
      (return (Math|Vector|MakeVector (|(({706B84D1-4BEE-7CC0-9EEE-78817B529F96}*Index)+RandomPuill) 1.0 _returnvalue_4) (|({688362AA-4621-01D6-640E-78ADCACAD910}+RandomPuill) _returnvalue_4) 1e+01)))))

(fn GenerateRandomNoteType
  (bind _mapinfo (Variables|Default|GetMapInfo))
  (bind _probabilitieoftier (Utilities|Struct|BreakMapInfo_Data _mapinfo))
  (bind (_elite _campfire _question) (Utilities|Struct|BreakProbabilitiesOfTierInMap_Data _probabilitieoftier))
  (return (select (CallFunction|CheckAgainstRandom100 _elite) "NewEnumerator3" (select (CallFunction|CheckAgainstRandom100 _campfire) "NewEnumerator2" (select (CallFunction|CheckAgainstRandom100 _question) "NewEnumerator1" "NewEnumerator0")))))

(fn GenerateConnections
  (params (MapNotes :type Array%20of%20Map%20Note%20Data%20Structures) (CurrentRow :type Integer) (IsSingleNote :type Boolean) (MapGrid :type BP%20Map%20Grid%20Object%20Reference))
  (bind _2darrayposition_data (Utilities|Struct|Make2DArrayPosition_Data 0 0))
  (bind _array (Utilities|Array|MakeArray _2darrayposition_data))
  (if (not IsSingleNote)
    (Utilities|FlowControl|Sequence
      (:then_0
        (for _index (range 0 (- (Utilities|Array|Length MapNotes) 1))
          (Utilities|FlowControl|Sequence
            (:then_0
              (LocalVariables|SetLocCurrIndex _index)
              (if (not (== CurrentRow 1))
                (bind _allnotesofgivenyindex (Default|GetAllElementsOfGivenYIndex MapGrid (- CurrentRow 1)))
                (LocalVariables|SetXBefor _allnotesofgivenyindex)
                (Utilities|Array|Add (LocalVariables|GetConnectionsArray) (Utilities|Struct|BreakMapNote_Data (select false (.Value (Utilities|Map|Find (LocalVariables|GetXBefor) (LocalVariables|GetLocCurrIndex))) (.Value (Utilities|Map|Find (LocalVariables|GetXBefor) (- (LocalVariables|GetLocCurrIndex) 1))))))
                (if (Math|Random|RandomBoolwithWeight (LocalVariables|GetMoreConnectionsChance))
                  (Utilities|Array|AddUnique (LocalVariables|GetConnectionsArray) (CallFunction|FindConnections (LocalVariables|GetXBefor) (LocalVariables|GetLocCurrIndex) false)))
                (if (Math|Random|RandomBoolwithWeight (LocalVariables|GetMoreConnectionsChance))
                  (Utilities|Array|AddUnique (LocalVariables|GetConnectionsArray) (CallFunction|FindConnections (LocalVariables|GetXBefor) (LocalVariables|GetLocCurrIndex) true)))
                (else
                  ;[1 1 1] Handels the first row
                  (bind _structout (Utilities|Struct|SetmembersinMapNote_Data (Utilities|Array|Get(acopy) MapNotes (LocalVariables|GetLocCurrIndex)) _array))
                  (CallFunction|SetConnectedto _structout _array MapGrid))))
            (:then_1
              ;[1 1 1] is used for all but first row
              (if (not (== CurrentRow 1))
                (bind _structout_2 (Utilities|Struct|SetmembersinMapNote_Data (Utilities|Array|Get(acopy) MapNotes (LocalVariables|GetLocCurrIndex)) (LocalVariables|GetConnectionsArray)))
                (CallFunction|SetConnectedto _structout_2 (LocalVariables|GetConnectionsArray) MapGrid)))
            (:then_2
              (Utilities|Array|Clear (LocalVariables|GetConnectionsArray)))))))
    (else
      (bind _allnotesofgivenyindex_2 (Default|GetAllElementsOfGivenYIndex MapGrid (- CurrentRow 1)))
      (bind _output_get (LocalVariables|SetXBefor _allnotesofgivenyindex_2))
      (bind _values (Utilities|Map|Values _output_get))
      (for _array_element _values
        (Utilities|Array|Add (LocalVariables|GetConnectionsArray) (Utilities|Struct|BreakMapNote_Data (.NoteAtIndex (Default|GetElement2D MapGrid (.x (Utilities|Struct|BreakMapNote_Data _array_element)) (.y (Utilities|Struct|BreakMapNote_Data _array_element)))))))
      (bind _structout_3 (Utilities|Struct|SetmembersinMapNote_Data (Utilities|Array|Get(acopy) MapNotes) (LocalVariables|GetConnectionsArray)))
      (Default|SetElement2D MapGrid (.x (Utilities|Struct|BreakMapNote_Data _structout_3)) (.y (Utilities|Struct|BreakMapNote_Data _structout_3)) _structout_3)
      (CallFunction|SetConnectedto (Utilities|Array|Get(acopy) MapNotes) (LocalVariables|GetConnectionsArray) MapGrid))))

(fn FindConnections
  (params (XBefor :type Map%20of%20Integers%20to%20Structs) (Index :type Integer) (Weighted :type Boolean))
  (return (Utilities|Struct|BreakMapNote_Data (select false (.Value (Utilities|Map|Find XBefor (+ Index (select Weighted -1 1)))) (select false (.Value (Utilities|Map|Find XBefor (+ Index (select Weighted 1 -1)))) (select false (.Value (Utilities|Map|Find XBefor (+ Index (select Weighted -2 2)))) (.Value (Utilities|Map|Find XBefor (+ Index (select Weighted 2 -2))))))))))

(fn SetConnectedto
  (params (NoteThat%20Conneted :type Map%20Note%20Data%20Structure%20%28by%20ref%29) (ConnectionsOfNote :type Array%20of%202D%20Array%20Position%20Data%20Structures) (MapGrid :type BP%20Map%20Grid%20Object%20Reference)))

(fn GenerateSingleNote
  (params (XIndex :type Integer) (NoteType :type MapNoteTypes%20Enum :default "NewEnumerator0") (MapGrid :type BP%20Map%20Grid%20Object%20Reference))
  (bind _structout (Utilities|Struct|SetmembersinMapNote_Data (LocalVariables|GetLocMapNote) (Utilities|Struct|Make2DArrayPosition_Data (Utilities|CorrectXIndex) 0) NoteType true))
  (bind _cordsforsingle (CallFunction|GenerateCordinates (Utilities|Array|MakeArray _structout) (Utilities|CorrectXIndex) true))
  (Utilities|Struct|SetmembersinMapNote_Data (LocalVariables|GetLocMapNote) _cordsforsingle)
  (CallFunction|GenerateConnections (Utilities|Array|MakeArray (LocalVariables|GetLocMapNote)) (Utilities|CorrectXIndex) true MapGrid)
  (return (LocalVariables|GetLocMapNote)))

(fn GenerateSingleNotewithY
  (params (XIndex :type Integer) (YCord :type Integer) (NoteType :type MapNoteTypes%20Enum :default "NewEnumerator0") (MapGrid :type BP%20Map%20Grid%20Object%20Reference))
  (bind _structout (Utilities|Struct|SetmembersinMapNote_Data (LocalVariables|GetLocMapNote) (Utilities|Struct|Make2DArrayPosition_Data (Utilities|CorrectXIndex) YCord) NoteType true))
  (bind _cordsforsingle (CallFunction|GenerateCordinates (Utilities|Array|MakeArray _structout) (Utilities|CorrectXIndex) true))
  (Utilities|Struct|SetmembersinMapNote_Data (LocalVariables|GetLocMapNote) _cordsforsingle)
  (CallFunction|GenerateConnections (Utilities|Array|MakeArray (LocalVariables|GetLocMapNote)) (Utilities|CorrectXIndex) true MapGrid)
  (return (LocalVariables|GetLocMapNote)))

(fn ConvertStoryMapIntoDisplayMap
  (params (StoryMap :type Story%20Map%20Save%20Structure))
  (bind (_length _numberineachcolumns _2darraygrid _contracttype _contracttypeextrainfo) (Utilities|Struct|BreakStoryMapSave StoryMap))
  (Utilities|Struct|SetmembersinStoryMapSave (LocalVariables|GetLocDisplayMap) _length _numberineachcolumns _2darraygrid _contracttype _contracttypeextrainfo)
  (return (LocalVariables|GetLocDisplayMap)))

(fn GenerateBasicMap
  (params (Length :type Integer) (NumberInColumn :type Integer))
  (bind _minmaxmapinfo_data (Utilities|Struct|MakeMinMaxMapInfo_Data))
  (Utilities|Struct|SetmembersinMapInfo_Data (LocalVariables|GetLocMapInfo) Length NumberInColumn)
  (Utilities|Struct|SetmembersinMapInfo_Data (LocalVariables|GetLocMapInfo) (Utilities|Struct|MakeMinMaxMapInfo_Data 0 1000) _minmaxmapinfo_data _minmaxmapinfo_data _minmaxmapinfo_data)
  (bind _generatedmap (CallFunction|GenerateMap (LocalVariables|GetLocMapInfo)))
  (return _generatedmap))