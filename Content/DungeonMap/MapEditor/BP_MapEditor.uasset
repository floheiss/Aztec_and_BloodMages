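; BP_MapEditor is an actor that sets up the dungeon map editor UI.
; On BeginPlay it takes the MapGrid from the C_DungeonMap player controller, then creates a W_TABS_MapEditor widget bound to itself and adds it to the viewport.
; It also binds to the game instance's debug mode update, so later toggles show or hide the editor HUD.
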(event `self.ReceiveBeginPlay`
  (bind _asc_dungeon_map (cast `/Game/DungeonMap/MapCore/C_DungeonMap` (`GameplayStatics.GetPlayerController` 0)))
  (set `self.MapGrid` (`/Game/DungeonMap/MapCore/C_DungeonMap.MapGrid` _asc_dungeon_map))
  (bind _returnvalue (`|CreateWidget` "/Game/DungeonMap/MapEditor/HUD_MapEditor/W_TABS_MapEditor.W_TABS_MapEditor_C" null self))
  (`UserWidget.AddToViewport` _returnvalue 0)
  (set `self.MapEditorHUD` _returnvalue)
  (add `/Game/Core/GI_Persistence.DeBugModeUpdate` (`/Game/Generel_Actor/BFL_General.GetGameInst`) (delegate `DeBugModeUpdate`)))

(event `DeBugModeUpdate`
  (params (DeBugModeActive :type Boolean))
  (bind _mapeditorhud (`self.MapEditorHUD`))
  (`Widget.RemoveFromParent` _mapeditorhud)
  (if DeBugModeActive
    (`UserWidget.AddToViewport` _mapeditorhud 0)))

(fn `UserConstructionScript`)