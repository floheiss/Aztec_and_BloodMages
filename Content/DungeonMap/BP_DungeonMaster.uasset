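; Dungeon master Blueprint that builds combat enemy waves and stores them on the game instance through SetUpCombat.
; Mercenary party strength and size drive random wave count and size limits.
; Enemies are picked from DT_EnemyAbaliable by combat situation, with Bandit as fallback, and spawned at far-off coordinates.
; Boss generation is an empty stub, casting handles only Bandit, and random stat buff/nerf helpers are never called here.
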(fn `BuffEnemy`
  (params (Enemy :type "/Game/Chars/PZD_Unit Object Reference"))
  (locals (LocAvaliableStatsToNer :type "Map of /Game/Chars/Utilities/UnitStatToChange Enum to Float (double-precision)") (LocEnemy :type "/Game/Chars/PZD_Unit Object Reference") (LocPull :type "/Game/Chars/Utilities/UnitStatToChange Enum" :default "NewEnumerator0") (LocPull_2 :type "/Game/Chars/Utilities/UnitStatToChange Enum" :default "NewEnumerator0"))
  (set `local.LocEnemy` Enemy)
  (bind _keys (`BlueprintMapLibrary.Map_Keys` (`local.LocAvaliableStatsToNer`)))
  (set `local.LocPull` (`KismetArrayLibrary.Array_Random` _keys))
  (`/Game/Chars/PZD_Unit.SetONEUnitStat` (`local.Enemy`) (`KismetMathLibrary.FTrunc` (* (`/Game/Chars/PZD_Unit.GetUnitStat` (`local.Enemy`) (`local.LocPull`)) (`BlueprintMapLibrary.Map_Find` (`local.LocAvaliableStatsToNer`) (`local.LocPull`)))) false (`local.LocPull`))
  (if (`KismetMathLibrary.RandomBoolWithWeight` 0.4)
    (bind _keys_2 (`BlueprintMapLibrary.Map_Keys` (`local.LocAvaliableStatsToNer`)))
    (set `local.LocPull_2` (`KismetArrayLibrary.Array_Random` _keys_2))
    (while (`|EnumEquality` (`local.LocPull`) (`local.LocPull_2`))
      (bind _keys_3 (`BlueprintMapLibrary.Map_Keys` (`local.LocAvaliableStatsToNer`)))
      (set `local.LocPull_2` (`KismetArrayLibrary.Array_Random` _keys_3)))
    (`/Game/Chars/PZD_Unit.SetONEUnitStat` (`local.Enemy`) (`KismetMathLibrary.FTrunc` (* (`/Game/Chars/PZD_Unit.GetUnitStat` (`local.Enemy`) (`local.LocPull`)) (`BlueprintMapLibrary.Map_Find` (`local.LocAvaliableStatsToNer`) (`local.LocPull_2`)))) false (`local.LocPull_2`))))

(fn `CastEnemyToClass`
  (params (ActorToCast :type "Actor Object Reference") (ClassToCastTo :type "/Game/Chars/Utilities/ClassList Enum" :default "NewEnumerator0"))
  (returns (CastActor :type "/Game/Chars/PZD_Unit Object Reference"))
  (locals (LocCastActor :type "/Game/Chars/PZD_Unit Object Reference"))
  (switch `/Game/Chars/Utilities/ClassList` ClassToCastTo
    (:`NewEnumerator11`
      (bind _asu_bandit (cast `/Game/Chars/SubClasses/Enemies/Bandit/U_Bandit` (`local.ActorToCast`)))
      (set `local.LocCastActor` _asu_bandit)
      (return (`local.LocCastActor`)))))

(fn `GenerateBoss`
  (returns (NewParam :type "Map of Integer to /Game/DungeonMap/CombatWaveData Structure"))
  (return))

(fn `GenerateEnemies`
  (params (Diff :type "/Game/Core/GeneralEnums/TierList Enum" :default "NewEnumerator0") (NoteType :type "/Game/DungeonMap/MapCore/MapNoteTypes Enum" :default "NewEnumerator0") (ContractType :type "/Game/Town/Guild/Contract_Types Enum" :default "NewEnumerator0") (CombatSituation :type "/Game/Combat/CombatSituations Enum" :default "NewEnumerator6"))
  (returns (Enemeis :type "Map of Integer to /Game/DungeonMap/CombatWaveData Structure"))
  (locals (LocWaveMap :type "Map of Integer to /Game/DungeonMap/CombatWaveData Structure") (LocMaxNumberEnemiesInWave :type Integer) (LocMaxNumberOfWaves :type Integer))
  (set `self.MercPartyStrength` (`/Game/Core/GI_Persistence.PartyOverallStrength` (`/Game/Core/BFL_General.GetGameInst`)))
  (bind _output_get (set `self.MercPartySize` (`KismetArrayLibrary.Array_Length` (`/Game/Core/GI_Persistence.MercGroup ` (`/Game/Core/BFL_General.GetGameInst`)))))
  (set `local.LocMaxNumberEnemiesInWave` (`KismetMathLibrary.Clamp` (+ _output_get (select `/Game/Core/GeneralEnums/TierList` (`self.MercPartyStrength`) :`NewEnumerator0` 1 :`NewEnumerator1` 1 :`NewEnumerator2` 1 :`NewEnumerator3` 2 :`NewEnumerator5` 2 :`NewEnumerator6` 2)) 2 6))
  (set `local.LocMaxNumberOfWaves` (select `/Game/Core/GeneralEnums/TierList` (`self.MercPartyStrength`) :`NewEnumerator0` 2 :`NewEnumerator1` 2 :`NewEnumerator2` 2 :`NewEnumerator3` 3 :`NewEnumerator5` 3 :`NewEnumerator6` 5))
  (if (`|EnumInequality` (`local.NoteType`) "NewEnumerator5")
    (for _index (range (+ (`KismetMathLibrary.RandomIntegerInRange` 1 (`local.LocMaxNumberOfWaves`)) 1))
      (bind _newwave (`self.GenerateWave` (`self.MercPartyStrength`) (`local.ContractType`) (`local.LocMaxNumberEnemiesInWave`) (`local.CombatSituation`)))
      (`BlueprintMapLibrary.Map_Add` (`local.LocWaveMap`) _index _newwave))
    (return (`local.LocWaveMap`))
    (else
      (`self.GenerateBoss`)
      (return (`local.LocWaveMap`)))))

(fn `GenerateRandomEnemy`
  (params (Diff :type "/Game/Core/GeneralEnums/TierList Enum" :default "NewEnumerator0") (ContractType :type "/Game/Town/Guild/Contract_Types Enum" :default "NewEnumerator0") (WaveIsBigger :type Boolean) (CombatSituation :type "/Game/Combat/CombatSituations Enum" :default "NewEnumerator0"))
  (returns (EnemyForWave :type "/Game/Chars/PZD_Unit Object Reference"))
  (locals (LocEnemy :type "/Game/Chars/PZD_Unit Object Reference"))
  (bind (_classesforspawning _classesforcasting) (`self.Get Avaliable Enemies Form Situation` CombatSituation))
  (bind _returnvalue (`KismetMathLibrary.RandomIntegerInRange` 0 (- (`KismetArrayLibrary.Array_Length` _classesforcasting) 1)))
  (set `local.LocEnemy` (`self.SpawnEnemyOfClass` (`|GetArrayItem` _classesforspawning _returnvalue) (`|GetArrayItem` _classesforcasting _returnvalue)))
  (if (`local.WaveIsBigger`)
    (return (`local.LocEnemy`))))

(fn `GenerateWave`
  (params (Diff :type "/Game/Core/GeneralEnums/TierList Enum" :default "NewEnumerator0") (ContractType :type "/Game/Town/Guild/Contract_Types Enum" :default "NewEnumerator0") (MaxNumberInWave :type Integer) (CombatSituation :type "/Game/Combat/CombatSituations Enum" :default "NewEnumerator0"))
  (returns (NewWave :type "/Game/DungeonMap/CombatWaveData Structure"))
  (locals (LocEnemyArray :type "Array of /Game/Chars/PZD_Unit Object Reference") (LocNumberInWave :type Integer :default 0) (WaveIsBigger :type Boolean))
  (bind _output_get (set `local.LocNumberInWave` (`KismetMathLibrary.Clamp` (`KismetMathLibrary.RandomIntegerInRange` (- (`self.MercPartySize`) 1) (`local.MaxNumberInWave`)) 1 (`local.MaxNumberInWave`))))
  (bind _output_get_2 (set `local.WaveIsBigger` (>= _output_get (`self.MercPartySize`))))
  (if _output_get_2
    (for _ (range (+ (`local.MaxNumberInWave`) 1))
      (bind _enemyforwave (`self.GenerateRandomEnemy` (`local.Diff`) (`local.ContractType`) (`local.WaveIsBigger`) (`local.CombatSituation`)))
      (`KismetArrayLibrary.Array_Add` (`local.LocEnemyArray`) _enemyforwave))
    (return (make `/Game/DungeonMap/CombatWaveData` (`local.LocEnemyArray`)))))

(fn `Get Avaliable Enemies Form Situation`
  (params (CombatSituation :type "/Game/Combat/CombatSituations Enum" :default "NewEnumerator0"))
  (returns (ClassesForSpawning :type "Array of Actor Class Reference") (ClassesForCasting :type "Array of /Game/Chars/Utilities/ClassList Enum"))
  (locals (LocEnemyArray :type "Array of Actor Class Reference") (LocEnemyClass :type "Array of /Game/Chars/Utilities/ClassList Enum"))
  (bind _outrownames (`DataTableFunctionLibrary.GetDataTableRowNames` "/Game/Chars/EnemyManagment/DT_EnemyAbaliable.DT_EnemyAbaliable"))
  (for _array_element _outrownames
    (bind _returnvalue (`|GetDataTableRow` "/Game/Chars/EnemyManagment/DT_EnemyAbaliable.DT_EnemyAbaliable" _array_element)
      (:`then`
        (bind (_class _classforcasting _combatsituationavaliable) (break `/Game/Chars/EnemyManagment/EnemyAvaliableData` _returnvalue))
        (if (`KismetArrayLibrary.Array_Contains` _combatsituationavaliable (`local.CombatSituation`))
          (`KismetArrayLibrary.Array_Add` (`local.LocEnemyArray`) _class)
          (`KismetArrayLibrary.Array_Add` (`local.LocEnemyClass`) _classforcasting)))))
  (if (> (`KismetArrayLibrary.Array_Length` (`local.LocEnemyArray`)) 0)
    (return (`local.LocEnemyArray`) (`local.LocEnemyClass`))
    (else
      (`KismetArrayLibrary.Array_Add` (`local.LocEnemyArray`) "/Game/Chars/SubClasses/Enemies/Bandit/U_Bandit.U_Bandit_C")
      (`KismetArrayLibrary.Array_Add` (`local.LocEnemyClass`) "NewEnumerator11")
      (return (`local.LocEnemyArray`) (`local.LocEnemyClass`)))))

(fn `NerfEnemy`
  (params (Enemy :type "/Game/Chars/PZD_Unit Object Reference"))
  (locals (LocAvaliableStatsToNer :type "Map of /Game/Chars/Utilities/UnitStatToChange Enum to Float (double-precision)") (LocEnemy :type "/Game/Chars/PZD_Unit Object Reference") (LocPull :type "/Game/Chars/Utilities/UnitStatToChange Enum" :default "NewEnumerator0") (LocPull_2 :type "/Game/Chars/Utilities/UnitStatToChange Enum" :default "NewEnumerator0"))
  (set `local.LocEnemy` Enemy)
  (bind _keys (`BlueprintMapLibrary.Map_Keys` (`local.LocAvaliableStatsToNer`)))
  (set `local.LocPull` (`KismetArrayLibrary.Array_Random` _keys))
  (`/Game/Chars/PZD_Unit.SetONEUnitStat` (`local.Enemy`) (`KismetMathLibrary.FTrunc` (* (`/Game/Chars/PZD_Unit.GetUnitStat` (`local.Enemy`) (`local.LocPull`)) (`BlueprintMapLibrary.Map_Find` (`local.LocAvaliableStatsToNer`) (`local.LocPull`)))) true (`local.LocPull`))
  (if (`KismetMathLibrary.RandomBoolWithWeight` 0.4)
    (bind _keys_2 (`BlueprintMapLibrary.Map_Keys` (`local.LocAvaliableStatsToNer`)))
    (set `local.LocPull_2` (`KismetArrayLibrary.Array_Random` _keys_2))
    (while (`|EnumEquality` (`local.LocPull`) (`local.LocPull_2`))
      (bind _keys_3 (`BlueprintMapLibrary.Map_Keys` (`local.LocAvaliableStatsToNer`)))
      (set `local.LocPull_2` (`KismetArrayLibrary.Array_Random` _keys_3)))
    (`/Game/Chars/PZD_Unit.SetONEUnitStat` (`local.Enemy`) (`KismetMathLibrary.FTrunc` (* (`/Game/Chars/PZD_Unit.GetUnitStat` (`local.Enemy`) (`local.LocPull`)) (`BlueprintMapLibrary.Map_Find` (`local.LocAvaliableStatsToNer`) (`local.LocPull_2`)))) true (`local.LocPull_2`))))

(fn `SetUpCombat`
  (params (Diff :type "/Game/Core/GeneralEnums/TierList Enum" :default "NewEnumerator0") (NoteType :type "/Game/DungeonMap/MapCore/MapNoteTypes Enum" :default "NewEnumerator0") (ContractType :type "/Game/Town/Guild/Contract_Types Enum" :default "NewEnumerator0") (CombatSituation :type "/Game/Combat/CombatSituations Enum" :default "NewEnumerator6"))
  (bind _enemeis (`self.GenerateEnemies` Diff NoteType ContractType CombatSituation))
  (`/Game/Core/GI_Persistence.SetCombatWaves` (`/Game/Core/BFL_General.GetGameInst`) _enemeis))

(fn `SpawnEnemyOfClass`
  (params (ClassToSpawn :type "Actor Class Reference") (ClassToCast :type "/Game/Chars/Utilities/ClassList Enum" :default "NewEnumerator0"))
  (returns (ActorOfGivenClass :type "/Game/Chars/PZD_Unit Object Reference"))
  (bind _returnvalue (`|SpawnActorFromClass` ClassToSpawn (`KismetMathLibrary.MakeTransform` (`KismetMathLibrary.MakeVector` -999.0 -999.0 (`KismetMathLibrary.RandomFloatInRange` -999.0 -9999.0))) "AlwaysSpawn" "MultiplyWithRoot" null null))
  (bind _castactor (`self.CastEnemyToClass` _returnvalue (`local.ClassToCast`)))
  (message `/Game/Chars/Utilities/IN_Unit.GetBaseStats` _castactor)
  (return _castactor))

(fn `UserConstructionScript`)