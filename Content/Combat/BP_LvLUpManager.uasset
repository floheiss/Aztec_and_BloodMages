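; BP_LvLUpManager queues mercenary level-ups and feeds them to the contract level-up menu.
; On BeginPlay it binds to level-up events on each merc's LvLManager in the game instance's MercGroup, and hooks merc additions for newcomers.
; When that menu opens, it passes the oldest queued entry to BP_MapManager for display, or switches to ContractViewMap if none remain.
; Helper functions read or remove the front entry.
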(event `self.ReceiveBeginPlay`
  (add `/Game/Core/GI_Persistence.MercWasAdded` (`/Game/Core/BFL_General.GetGameInst`) (`|CreateDelegate` :!event `OnUnitSpawned`))
  (for _array_element (`/Game/Core/GI_Persistence.MercGroup ` (`/Game/Core/BFL_General.GetGameInst`))
    (add `/Game/Chars/MercLvLManagment/BP_LVLManager.UnitLevelUp` (`/Game/Chars/PZD_Unit.LvLManager` _array_element) (`|CreateDelegate` :!event `OnUnitLvLUp`))))

(event `OnUnitSpawned`
  (params (NewMerc :type "/Game/Chars/PZD_Unit Object Reference"))
  ; handles unit lvl up
  (add `/Game/Chars/MercLvLManagment/BP_LVLManager.UnitLevelUp` (`/Game/Chars/PZD_Unit.LvLManager` NewMerc) (`|CreateDelegate` :!event `OnUnitLvLUp`)))

(event `OnUnitLvLUp`
  (params (UnitLeveledUp :type "/Game/Chars/MercLvLManagment/UnitLeveledDisplayUpData Structure"))
  ; handles unit lvl up
  (`KismetArrayLibrary.Array_Add` (`self.UnSpendLvLUpArray`) UnitLeveledUp)
  (set `self.ThereAreUnSpendLvL` true))

(event `OnMenuUpdate`
  (params (MenuOpen :type "/Game/Core/GeneralEnums/MenuList Enum" :default "NewEnumerator3"))
  (switch `/Game/Core/GeneralEnums/MenuList` MenuOpen
    (:`NewEnumerator16`
      (if (> (`KismetArrayLibrary.Array_Length` (`self.UnSpendLvLUpArray`)) 0)
        (bind _returnvalue (`GameplayStatics.GetActorOfClass` "/Game/DungeonMap/MapV2/BP_MapManager.BP_MapManager_C"))
        (`/Game/DungeonMap/MapV2/BP_MapManager.DisplayLvLUp` _returnvalue (`|GetArrayItem` (`self.UnSpendLvLUpArray`)))
        (`KismetArrayLibrary.Array_Remove` (`self.UnSpendLvLUpArray`))
        (set `self.ThereAreUnSpendLvL` (> (`KismetArrayLibrary.Array_Length` (`self.UnSpendLvLUpArray`)) 0))
        (else
          (`/Game/Core/GI_Persistence.SetMenu` (`/Game/Core/BFL_General.GetGameInst`) "NewEnumerator14"))))))

(fn `GetOneUnSpendLvL`
  (returns (UnSpendLvL :type "/Game/Chars/MercLvLManagment/UnitLeveledDisplayUpData Structure"))
  (locals (LocReturnLvL :type "/Game/Chars/MercLvLManagment/UnitLeveledDisplayUpData Structure"))
  (set `local.LocReturnLvL` (`|GetArrayItem` (`self.UnSpendLvLUpArray`)))
  (return (`local.LocReturnLvL`)))

(fn `RemoveUnSpendLvL`
  (`KismetArrayLibrary.Array_Remove` (`self.UnSpendLvLUpArray`))
  (set `self.ThereAreUnSpendLvL` (> (`KismetArrayLibrary.Array_Length` (`self.UnSpendLvLUpArray`)) 0)))

(fn `UserConstructionScript`)